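; Base Blueprint for projectile spells, using a box collision and a SpellMovement component whose speed and gravity scale are set from variables in the construction script.
; On BeginPlay the box ignores its owner while moving.
; On hit it calls OnProjectileCollision, an empty hook apparently meant for child spells to override, then spawns collision FX and sound at the impact point and destroys itself.
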(event `self.ReceiveBeginPlay`
  (`PrimitiveComponent.IgnoreActorWhenMoving` (`self.BoxCollision`) (`self.GetOwner`) true))

(event `self.BoxCollision.OnComponentHit`
  (params (HitComponent :type "PrimitiveComponent Object Reference") (OtherActor :type "Actor Object Reference") (OtherComp :type "PrimitiveComponent Object Reference") (NormalImpulse :type "Vector Structure") (Hit :type "HitResult Structure (by ref)"))
  (bind (_bblockinghit _binitialoverlap _time _distance _location) (`GameplayStatics.BreakHitResult` Hit))
  (`self.OnProjectileCollision` OtherActor Hit)
  ; Depending on if this behaviour is the same for all projectile spells
  (`NiagaraFunctionLibrary.SpawnSystemAtLocation` (`self.OnCollisionFX`) _location)
  (`GameplayStatics.PlaySoundAtLocation` (`self.OnCollisionSound`) _location (struct) 1.0 1.0 0.0 null null null null)
  (`KismetSystemLibrary.PrintString` "Destroyed")
  (`self.K2_DestroyActor`))

(fn `OnProjectileCollision`
  (params (OtherActor :type "Actor Object Reference") (Hit :type "HitResult Structure")))

(fn `UserConstructionScript`
  (bind _spellmovement (`self.SpellMovement`))
  (`parent.UserConstructionScript`)
  (bind _output_get (set `ProjectileMovementComponent.MaxSpeed` (`self.MovementSpeed`) _spellmovement))
  (set `ProjectileMovementComponent.InitialSpeed` _output_get _spellmovement)
  (set `ProjectileMovementComponent.ProjectileGravityScale` (`self.GravityScale`) _spellmovement))