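; Base spell Blueprint that spawns an object, a destroyable going by the asset's name, in front of the spell actor.
; On BeginPlay it spawns the SpawnedObject class using the transform from GetSpawnTransform.
; That function offsets the actor's location along its forward vector by SpawningDistance and keeps the actor's rotation and scale.
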(event `self.ReceiveBeginPlay`
  (bind _transform (`self.GetSpawnTransform`))
  (`|SpawnActorFromClass` (`self.SpawnedObject`) _transform "Undefined" "MultiplyWithRoot" null null))

(fn `GetSpawnTransform`
  (returns (Transform :type "Transform Structure"))
  (bind (_returnvalue_location _returnvalue_rotation _returnvalue_scale) (`KismetMathLibrary.BreakTransform` (`self.GetTransform`)))
  (return (`KismetMathLibrary.MakeTransform` (+ (* (`self.GetActorForwardVector`) (`self.SpawningDistance`)) _returnvalue_location) _returnvalue_rotation _returnvalue_scale)))

(fn `UserConstructionScript`
  (`parent.UserConstructionScript`))