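; BP_Dash is a spell actor that launches its owning character forward in a dash.
; On BeginPlay it takes the forward vector of SpellOwner's root component, scales it by a fixed distance and DashForce, and passes it to LaunchCharacter, adding to current velocity rather than overriding it.
; The actor then destroys itself immediately, so spawning it is the whole cast.
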(event `self.ReceiveBeginPlay`
  (bind _spellowner (`self.SpellOwner`))
  (bind _rootcomponent (`Actor.RootComponent` _spellowner))
  (bind _returnvalue (`SceneComponent.K2_GetComponentLocation` _rootcomponent))
  (`Character.LaunchCharacter` _spellowner (* (- (+ _returnvalue (* (`KismetMathLibrary.GetForwardVector` (`SceneComponent.K2_GetComponentRotation` _rootcomponent)) 100.0)) _returnvalue) (`self.DashForce`)) false false)
  (`self.K2_DestroyActor`))

(fn `UserConstructionScript`
  (`parent.UserConstructionScript`))