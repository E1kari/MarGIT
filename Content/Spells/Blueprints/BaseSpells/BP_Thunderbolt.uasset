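; Thunderbolt spell Blueprint that deals area damage when its projectile collides.
; The construction script sizes the DamageSphere component to DamageRadius.
; On projectile collision, every actor overlapping that sphere receives DamageAmount through the HSIOnTakeDamage interface message, regardless of which actor was hit.
; BeginPlay runs the parent logic and prints a debug string.
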(event `self.ReceiveBeginPlay`
  (`parent.ReceiveBeginPlay`)
  (`KismetSystemLibrary.PrintString` "ThunderBolt"))

(fn `OnProjectileCollision`
  (params (OtherActor :type "Actor Object Reference") (Hit :type "HitResult Structure"))
  (for _array_element (`PrimitiveComponent.GetOverlappingActors` (`self.DamageSphere`) null)
    (message `/Game/Blueprints/Interfaces/BPI_HealthSystemInterface.HSI_OnTakeDamage` _array_element (`self.DamageAmount`))))

(fn `UserConstructionScript`
  (`parent.UserConstructionScript`)
  (`SphereComponent.SetSphereRadius` (`self.DamageSphere`) (`self.DamageRadius`) true))