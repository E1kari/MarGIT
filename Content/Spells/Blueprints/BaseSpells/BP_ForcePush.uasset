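; BP_ForcePush is a Force Push spell Blueprint, still a stub with debug prints in place of any push effect.
; The construction script runs the parent's, then shapes BoxCollision into a thin slab from the Size variable, mapped to the Y and Z extents.
; BeginPlay calls its parent, while it, box overlap and OnProjectileCollision each only print a message.
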(event `self.ReceiveBeginPlay`
  (`parent.ReceiveBeginPlay`)
  (`KismetSystemLibrary.PrintString` "ForcePush"))

(event `self.BoxCollision.OnComponentBeginOverlap`
  (params (OverlappedComponent :type "PrimitiveComponent Object Reference") (OtherActor :type "Actor Object Reference") (OtherComp :type "PrimitiveComponent Object Reference") (OtherBodyIndex :type Integer) (bFromSweep :type Boolean) (SweepResult :type "HitResult Structure (by ref)"))
  (`KismetSystemLibrary.PrintString` "Overlap"))

(fn `OnProjectileCollision`
  (params (OtherActor :type "Actor Object Reference") (Hit :type "HitResult Structure"))
  (`KismetSystemLibrary.PrintString` "Collision"))

(fn `UserConstructionScript`
  (bind (_size_x _size_y) (`KismetMathLibrary.BreakVector2D` (`self.Size`)))
  (`parent.UserConstructionScript`)
  (`BoxComponent.SetBoxExtent` (`self.BoxCollision`) (`KismetMathLibrary.MakeVector` 1.0 _size_x _size_y) true))