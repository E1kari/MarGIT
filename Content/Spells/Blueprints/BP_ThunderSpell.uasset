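; BP_ThunderSpell is a thunder spell projectile that deals area damage on its first overlap.
; On BeginPlay it launches along its forward vector at Speed through ProjectileMovement.
; On overlap it expands its collision sphere to DamageRadius and sends Damage through BPI_HealthSystemInterface to overlapping actors that implement it, excluding BP_BaseSpell.
; It then prints a debug message and destroys itself.
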(event `self.ReceiveBeginPlay`
  (set `MovementComponent.Velocity` (* (`self.GetActorForwardVector`) (`self.Speed`)) (`self.ProjectileMovement`)))

(event `self.Collision.OnComponentBeginOverlap`
  (params (OverlappedComponent :type "PrimitiveComponent Object Reference") (OtherActor :type "Actor Object Reference") (OtherComp :type "PrimitiveComponent Object Reference") (OtherBodyIndex :type Integer) (bFromSweep :type Boolean) (SweepResult :type "HitResult Structure (by ref)"))
  (bind _collision (`self.Collision`))
  (`SphereComponent.SetSphereRadius` _collision (`self.DamageRadius`) true)
  (for _array_element (`PrimitiveComponent.GetOverlappingActors` _collision null)
    (if (== _array_element "/Game/Spells/Blueprints/BP_BaseSpell.BP_BaseSpell")
      _
      (elif (`KismetSystemLibrary.DoesImplementInterface` _array_element "/Game/Blueprints/BPI_HealthSystemInterface.BPI_HealthSystemInterface_C")
        (message `/Game/Blueprints/BPI_HealthSystemInterface.OnTakeDamage` _array_element (`self.Damage`)))))
  (`KismetSystemLibrary.PrintString` "Spell destroyed")
  (`self.K2_DestroyActor`))

(fn `UserConstructionScript`
  (`parent.UserConstructionScript`))