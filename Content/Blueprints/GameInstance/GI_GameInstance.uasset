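; Game instance that registers hub portals with each other and records debug statistics on rune and spell usage.
; Two events gather all temple-hub or newer hub portal actors and pass the full list to each portal.
; Counter functions tally predicted runes with their confidence, via per-rune debug objects, and spell casts by name in a map.
; On shutdown, both tallies are saved to a timestamped text file.
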(event `AddAllPortals`
  (bind _outactors (`GameplayStatics.GetAllActorsOfClass` "/Game/Blueprints/Environment/Portals/BP_Portal_TempleHub.BP_Portal_TempleHub_C"))
  (bind _output_get (set `self.AllTempleHubPortals` _outactors))
  (for _array_element _output_get
    (`/Game/Blueprints/Environment/Portals/BP_Portal_Base.AddAllTempleHubPortals` _array_element _output_get)))

(event `AddAllPortalsNew`
  (bind _outactors (`GameplayStatics.GetAllActorsOfClass` "/Game/Blueprints/Environment/Portals/NewTry/BP_Portal_Hub.BP_Portal_Hub_C"))
  (bind _output_get (set `self.AllTempleHubPortalsNew` _outactors))
  (for _array_element _output_get
    (`/Game/Blueprints/Environment/Portals/NewTry/BP_Portal.AddAllHubPortals` _array_element _output_get)))

(event `self.ReceiveShutdown`
  (bind (_year _month _day _hour _minute _second) (`KismetMathLibrary.BreakDateTime` (`KismetMathLibrary.Now`)))
  (`RuneFunctionLibrary.SaveDebugStatsToText` (`self.RuneCounter`) (`self.SpellCounter`) (`KismetStringLibrary.Concat_StrStr` "RuneAndSpellUsage_" (`KismetStringLibrary.Concat_StrStr` (`KismetStringLibrary.Conv_IntToString` _year) "-" (`KismetStringLibrary.Conv_IntToString` _month) "-" (`KismetStringLibrary.Conv_IntToString` _day) "_" (`KismetStringLibrary.Conv_IntToString` _hour) "-" (`KismetStringLibrary.Conv_IntToString` _minute) "-" (`KismetStringLibrary.Conv_IntToString` _second)) ".txt")))

(fn `AddToRuneCounter`
  (params (PredictionResult :type "PredictionResult Structure"))
  (locals (`RuneAlreadyExists?` :type Boolean))
  (bind (_predictedlabel _predictedindex _confidence) (break `PredictionResult` PredictionResult))
  (for _array_element (`self.RuneCounter`)
    (if (`KismetStringLibrary.EqualEqual_StrStr` (`DebugRuneCount.RuneName` _array_element) _predictedlabel)
      (set `local.RuneAlreadyExists?` true)
      (`DebugRuneCount.IncrementCount` _array_element _confidence)
      (break)))
  (if (not (`local.RuneAlreadyExists?`))
    (bind _returnvalue (`DebugRuneCount.CreateDebugRuneCountObject` PredictionResult))
    (`KismetArrayLibrary.Array_Add` (`self.RuneCounter`) _returnvalue)))

(fn `AddToSpellCounter`
  (params (SpellName :type String))
  (bind (_value _returnvalue) (`BlueprintMapLibrary.Map_Find` (`self.SpellCounter`) SpellName))
  (if (not _returnvalue)
    (`BlueprintMapLibrary.Map_Add` (`self.SpellCounter`) SpellName 1)
    (else
      (`BlueprintMapLibrary.Map_Add` (`self.SpellCounter`) SpellName (+ _value 1)))))