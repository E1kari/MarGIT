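; BP_Enemy_Base is the base enemy Character, handling health, damage, death, knockback and movement speed by state.
; Damage is reported to AI perception, lowers health and updates a debug gizmo widget; at zero, IsAlive turns false.
; The IsAlive RepNotify triggers death, swapping the mesh material and notifying AIC_Enemy_Base, which also receives the behavior tree on init.
; Debug events toggle gizmo and hitbox visibility, while several ETI getters are empty stubs.
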(event `/Game/Blueprints/Interfaces/BPI_DebugGizmos.DG_ShowEnemyStatus`
  (bind _debuggizmo (`self.DebugGizmo`))
  (`SceneComponent.SetVisibility` _debuggizmo (not (`SceneComponent.bVisible` _debuggizmo)) false))

(event `self.ReceiveAnyDamage`
  (params (Damage :type "Float (single-precision)") (DamageType :type "DamageType Object Reference") (InstigatedBy :type "Controller Object Reference") (DamageCauser :type "Actor Object Reference"))
  (`self.OnTakeDamage` Damage DamageType InstigatedBy DamageCauser))

(event `/Game/Blueprints/Interfaces/BPI_EffectTargetInterface.ETI_OnKnockback`
  (params (ImpulseForce :type "Vector Structure"))
  (`self.LaunchCharacter` ImpulseForce))

(event `/Game/Blueprints/Interfaces/BPI_DebugGizmos.DG_ShowHitbox`
  (bind _output_get (set `self.ShowHitbox?` (not (`self.ShowHitbox?`))))
  (if _output_get
    (`SceneComponent.SetHiddenInGame` (`self.CapsuleComponent`) false false)
    (else
      (`SceneComponent.SetHiddenInGame` (`self.CapsuleComponent`) true false))))

(fn `EAI_SetMovementSpeed`
  (params (MovementState :type "/Game/Blueprints/Enumeration/E_MovementState Enum" :default "NewEnumerator0"))
  (returns (MovementSpeed :type "Float (double-precision)"))
  (bind _output_get (set `CharacterMovementComponent.MaxWalkSpeed` (`BlueprintMapLibrary.Map_Find` (`self.MovementSpeed`) MovementState) (`self.CharacterMovement`)))
  (return _output_get))

(fn `ETI_GetGravityScale`
  (returns (GravityScale :type "Float (double-precision)"))
  (return 0.0))

(fn `ETI_GetMovementSpeed`
  (returns (MovementSpeed :type "Float (double-precision)"))
  (return 0.0))

(fn `ETI_GetPlayerController`
  (returns (PlayerController :type "PlayerController Object Reference"))
  (return null))

(fn `OnEnemyDeath`
  (`PrimitiveComponent.SetMaterial` (`self.Mesh`) 0 "/Game/StarterContent/Characters/Mannequins/Materials/Instances/Manny/MI_Manny_01.MI_Manny_01")
  (bind _asaic_enemy_base (cast `/Game/Blueprints/Enemy/AI/AIC_Enemy_Base` (`AIBlueprintHelperLibrary.GetAIController` self))
    (:`then`
      (`/Game/Blueprints/Enemy/AI/AIC_Enemy_Base.OnEnemyDeath` _asaic_enemy_base)
      (`KismetSystemLibrary.PrintString` "Emeny Died"))
    (:`CastFailed`
      (`KismetSystemLibrary.PrintString` "Failed"))))

(fn `OnInit`
  (set `self.CurrentHealth` (`self.MaxHealth`))
  (bind _asaic_enemy_base (cast `/Game/Blueprints/Enemy/AI/AIC_Enemy_Base` (`AIBlueprintHelperLibrary.GetAIController` self))
    (:`then`
      (set `/Game/Blueprints/Enemy/AI/AIC_Enemy_Base.BehaviorTree` (`self.Behavior Tree`) _asaic_enemy_base))
    (:`CastFailed`
      (`KismetSystemLibrary.PrintString` "Failed"))))

(fn `OnRep_IsAlive`
  (`self.OnEnemyDeath`))

(fn `OnTakeDamage`
  (params (DamageAmount :type "Float (double-precision)") (DamageType :type "DamageType Object Reference") (InstigatedBy :type "Controller Object Reference") (DamageCauser :type "Actor Object Reference"))
  ; Report damage to perception ai
  (`/Engine/EditorBlueprintResources/StandardMacros.IsValid` InstigatedBy
    (:`Is Valid`
      (`AISense_Damage.ReportDamageEvent` self InstigatedBy DamageAmount (`self.K2_GetActorLocation` (`Controller.K2_GetPawn` InstigatedBy))))
    (:`Is Not Valid`
      (`KismetSystemLibrary.PrintString` "No valid instigator")))
  ; reduce health
  (set `self.CurrentHealth` (- (`self.CurrentHealth`) DamageAmount))
  ; Set Debug Gizmo Health
  (bind _aswb_enemy_gizmos (cast `/Game/Blueprints/Enemy/Gizmos/WB_EnemyGizmos` (`WidgetComponent.GetWidget` (`self.DebugGizmo`))))
  (`/Game/Blueprints/Enemy/Gizmos/WB_EnemyGizmos.SetHealthPercent` _aswb_enemy_gizmos (/ (`self.CurrentHealth`) (`self.MaxHealth`)))
  ; check if dead
  (if (<= (`self.CurrentHealth`) 0.0)
    (`/Engine/EditorBlueprintResources/StandardMacros.DoOnce` false
      (:`Completed`
        (set `self.IsAlive` false)))))

(fn `SetDebugGizmoState`
  (params (State :type "/Game/Blueprints/Enumeration/E_AIStates Enum" :default "NewEnumerator1"))
  (bind _aswb_enemy_gizmos (cast `/Game/Blueprints/Enemy/Gizmos/WB_EnemyGizmos` (`WidgetComponent.GetWidget` (`self.DebugGizmo`))))
  (`/Game/Blueprints/Enemy/Gizmos/WB_EnemyGizmos.SetState` _aswb_enemy_gizmos State))

(fn `UserConstructionScript`)