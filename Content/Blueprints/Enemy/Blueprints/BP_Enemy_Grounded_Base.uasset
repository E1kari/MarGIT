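; Base Blueprint for grounded enemy characters, handling health, damage, death and AI-driven movement speed.
; AnyDamage subtracts from health and reports a damage event at the instigating pawn's location for AI perception.
; Depleted health clears IsAlive, whose RepNotify runs the death handler to swap the mesh material and print debug text.
; An EAI function sets walk speed from a movement-state map, while ETI getters are empty stubs.
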(event `self.ReceiveAnyDamage`
  (params (Damage :type "Float (single-precision)") (DamageType :type "DamageType Object Reference") (InstigatedBy :type "Controller Object Reference") (DamageCauser :type "Actor Object Reference"))
  (`self.OnTakeDamage` Damage DamageType)
  (`AISense_Damage.ReportDamageEvent` self InstigatedBy Damage (`self.K2_GetActorLocation` (`Controller.K2_GetPawn` InstigatedBy))))

(fn `EAI_SetMovementSpeed`
  (params (MovementState :type "/Game/Blueprints/Enumeration/E_MovementState Enum" :default "NewEnumerator0"))
  (returns (MovementSpeed :type "Float (double-precision)"))
  (bind _output_get (set `CharacterMovementComponent.MaxWalkSpeed` (`BlueprintMapLibrary.Map_Find` (`self.MovementSpeed`) MovementState) (`self.CharacterMovement`)))
  (return _output_get))

(fn `ETI_GetGravityScale`
  (returns (GravityScale :type "Float (double-precision)"))
  (return 0.0))

(fn `ETI_GetMovementSpeed`
  (returns (MovementSpeed :type "Float (double-precision)"))
  (return 0.0))

(fn `ETI_GetPlayerController`
  (returns (PlayerController :type "PlayerController Object Reference"))
  (return null))

(fn `OnEnemyDeath`
  (`PrimitiveComponent.SetMaterial` (`self.Mesh`) 0 "/Game/Characters/Mannequins/Materials/Instances/Manny/MI_Manny_01.MI_Manny_01")
  (`KismetSystemLibrary.PrintString` "Emeny Died"))

(fn `OnRep_IsAlive`
  (`self.OnEnemyDeath`))

(fn `OnTakeDamage`
  (params (DamageAmount :type "Float (double-precision)") (DamageType :type "DamageType Object Reference"))
  (`KismetSystemLibrary.PrintString` (`KismetStringLibrary.Conv_DoubleToString` DamageAmount))
  (bind _output_get (set `self.CurrentHealth` (- (`self.CurrentHealth`) DamageAmount)))
  (if (<= _output_get 0.0)
    (`/Engine/EditorBlueprintResources/StandardMacros.DoOnce` false
      (:`Completed`
        (set `self.IsAlive` false)))))

(fn `UserConstructionScript`
  (set `self.CurrentHealth` (`self.MaxHealth`)))