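; Rune-drawing spellcasting component that recognises mouse-drawn runes with an ONNX model and turns them into spells.
; Each stroke spawns an inference actor with trail FX and time dilation, while recording mouse points scaled to 64x64.
; On release, the points render to a canvas target whose grayscale data feeds inference.
; Recognised labels form a sorted, unique "+"-joined SpellsMap key, with spawning and FX routed through server RPC events.
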(event `self.ReceiveBeginPlay`
  (bind _returnvalue (`CanvasRenderTarget2D.CreateCanvasRenderTarget2D` "/Game/RuneAI/Blueprints/BP_RuneDrawCanvas.BP_RuneDrawCanvas_C" 64 64))
  (set `self.RuneCanvas` _returnvalue))

(event `RPC_RS_Server_SpawnONNXActor`
  (params (Position :type "Transform Structure"))
  ; Spawn ONNX Actor
  (`self.RPC_SpawnONNXActor` Position))

(event `RPC_SpawnONNXActor`
  (params (Position :type "Transform Structure"))
  ; Spawn ONNX Actor
  (bind _returnvalue (`|SpawnActorFromClass` "/Game/RuneAI/Blueprints/BP_ONNXInferenceActor.BP_ONNXInferenceActor_C" Position "AlwaysSpawn" "MultiplyWithRoot" null null))
  (bind _output_get (set `self.ONNXModel` _returnvalue))
  (`KismetArrayLibrary.Array_Add` (`self.AllONNXModels`) _output_get)
  (`/Game/RuneAI/Blueprints/BP_ONNXInferenceActor.RPC_OIA_Server_StartTimeDelation` _output_get))

(event `RPC_RS_Server_UpdateFXPosition`
  (params (Position :type "Vector Structure"))
  ; Update Rune FX Position
  (`self.RPC_UpdateFXPosition` Position))

(event `RPC_RS_Server_RuneNotRecognized`
  ; FX Rune (Not) Recognized Calls
  (`self.RPC_RuneNotRecognized`))

(event `RPC_RS_Server_RuneRecognized`
  ; FX Rune (Not) Recognized Calls
  (`self.RPC_RuneRecognized`))

(event `RPC_RuneNotRecognized`
  ; FX Rune (Not) Recognized Calls
  (`/Game/RuneAI/Blueprints/BP_ONNXInferenceActor.RuneNotRecognized` (`self.ONNXModel`)))

(event `RPC_RuneRecognized`
  ; FX Rune (Not) Recognized Calls
  (`/Game/RuneAI/Blueprints/BP_ONNXInferenceActor.RuneRecognized` (`self.ONNXModel`)))

(event `RPC_UpdateFXPosition`
  (params (Position :type "Vector Structure"))
  ; Update Rune FX Position
  (`/Game/RuneAI/Blueprints/BP_ONNXInferenceActor.UpdateRuneTrailTXPosition` (`self.ONNXModel`) Position))

(event `RPC_RS_Server_DestroyONNXActors`
  ; Destroy all drawn runes
  (`self.RPC_DestroyONNXActors`))

(event `RPC_RS_Server_CastSpell`
  (params (SpellBluePrint :type "/Game/Spells_And_Effects/Spells/BaseSpells/BP_BaseSpell Class Reference") (SpellOwner :type "Character Object Reference"))
  ; Cast Spell
  (bind _asbp_third_person_character (cast `/Game/ThirdPerson/Blueprints/BP_ThirdPersonCharacter` (`self.GetOwner`)))
  (bind _rotation (`/Game/ThirdPerson/Blueprints/BP_ThirdPersonCharacter.GetCameraRotation` _asbp_third_person_character))
  (`|SpawnActorFromClass` SpellBluePrint (`KismetMathLibrary.MakeTransform` (`SceneComponent.K2_GetComponentLocation` (`/Game/ThirdPerson/Blueprints/BP_ThirdPersonCharacter.SpellCastPoint` _asbp_third_person_character)) _rotation) "Undefined" "MultiplyWithRoot" null SpellOwner null))

(event `RPC_DestroyONNXActors`
  (bind _allonnxmodels (`self.AllONNXModels`))
  ; Destroy all drawn runes
  (for _array_element _allonnxmodels
    (`Actor.K2_DestroyActor` _array_element))
  (`KismetArrayLibrary.Array_Clear` _allonnxmodels))

(fn `ClearRunePredictionResultsArray`
  (`KismetArrayLibrary.Array_Clear` (`self.RunePredictionResultArray`)))

(fn `GetDeprojectScreenToWorld`
  (returns (Pos :type "Vector Structure"))
  (bind _returnvalue (`GameplayStatics.GetPlayerController` 0))
  (bind (_locationx _locationy) (`PlayerController.GetMousePosition` _returnvalue))
  (bind (_worldposition _worlddirection) (`GameplayStatics.DeprojectScreenToWorld` _returnvalue (`KismetMathLibrary.MakeVector2D` _locationx _locationy)))
  (return (+ _worldposition (* _worlddirection 200.0))))

(fn `RS_CastSpell`
  (params (SpellOwner :type "Character Object Reference"))
  (locals (RunesNames :type "Array of String") (SpellName :type String))
  (bind _runesnames (`local.RunesNames`))
  (bind _runesnames_2 (`local.RunesNames`))
  (bind _returnvalue (`KismetArrayLibrary.Array_Length` _runesnames))
  (bind (_value _returnvalue_2) (`BlueprintMapLibrary.Map_Find` (`self.SpellsMap`) (`local.SpellName`)))
  (`KismetArrayLibrary.Array_Clear` (`local.RunesNames`))
  (for _array_element (`self.RunePredictionResultArray`)
    (`KismetArrayLibrary.Array_AddUnique` (`local.RunesNames`) (`.PredictedLabel` (break `PredictionResult` _array_element))))
  (`KismetArrayLibrary.SortStringArray` _runesnames)
  (if (> _returnvalue 0)
    (set `local.SpellName` (`|GetArrayItem` _runesnames))
    (if (> _returnvalue 1)
      (for _index (range 1 (+ (`KismetArrayLibrary.Array_LastIndex` _runesnames_2) 1))
        (set `local.SpellName` (`KismetStringLibrary.Concat_StrStr` (`local.SpellName`) "+" (`|GetArrayItem` _runesnames_2 _index)))))
    (if _returnvalue_2
      (`self.RPC_RS_Server_CastSpell` _value SpellOwner)
      (else
        (`KismetSystemLibrary.PrintString` "Spell not Found")))
    (`self.RPC_RS_Server_DestroyONNXActors`)))

(fn `RS_OnOngoingDrawing`
  (bind (_returnvalue_x _returnvalue_y) (`KismetMathLibrary.BreakVector2D` (`WidgetLayoutLibrary.GetViewportSize`)))
  (bind (_locationx _locationy) (`PlayerController.GetMousePosition` (`GameplayStatics.GetPlayerController` 0)))
  (`KismetArrayLibrary.Array_Add` (`self.RuneDrawingPoints`) (`KismetMathLibrary.MakeVector2D` (* (/ _locationx _returnvalue_x) 64.0) (* (/ _locationy _returnvalue_y) 64.0)))
  (bind _pos (`self.GetDeprojectScreenToWorld`))
  (`self.RPC_RS_Server_UpdateFXPosition` _pos))

(fn `RS_OnStartDrawing`
  (`KismetArrayLibrary.Array_Clear` (`self.RuneDrawingPoints`))
  (bind _pos (`self.GetDeprojectScreenToWorld`))
  (`self.RPC_RS_Server_SpawnONNXActor` (`KismetMathLibrary.Conv_VectorToTransform` _pos)))

(fn `RS_OnStopDrawing`
  (bind _runecanvas (`self.RuneCanvas`))
  (bind _onnxmodel (`self.ONNXModel`))
  (bind _asbp_rune_draw_canvas (cast `/Game/RuneAI/Blueprints/BP_RuneDrawCanvas` _runecanvas)
    (:`then`
      (set `/Game/RuneAI/Blueprints/BP_RuneDrawCanvas.RunePoints` (`self.RuneDrawingPoints`) _asbp_rune_draw_canvas)
      (`CanvasRenderTarget2D.UpdateResource` _runecanvas)
      (bind _outdata (`RuneFunctionLibrary.GetCanvasGrayscaleData` _runecanvas))
      (if (`KismetSystemLibrary.IsValid` _onnxmodel)
        (bind _returnvalue (`ONNXInferenceActor.RunInferenceBP` _onnxmodel _outdata))
        (if (`KismetStringLibrary.EqualEqual_StrStr` (`.PredictedLabel` (break `PredictionResult` _returnvalue)) "Unknown")
          (`self.RPC_RS_Server_RuneNotRecognized`)
          (else
            (`KismetArrayLibrary.Array_Add` (`self.RunePredictionResultArray`) _returnvalue)
            (`self.RPC_RS_Server_RuneRecognized`)))
        (`/Game/RuneAI/Blueprints/BP_ONNXInferenceActor.RPC_OIA_Server_StopTimeDelation` (`self.ONNXModel`))
        (else
          (`KismetSystemLibrary.PrintString` "Not Valid"))))
    (:`CastFailed`
      (`KismetSystemLibrary.PrintString` "Cast Failed"))))

(fn `SetLocalMousePos64x64`
  (returns (NewParam :type "Vector2D Structure"))
  (bind (_returnvalue_x _returnvalue_y) (`KismetMathLibrary.BreakVector2D` (`WidgetLayoutLibrary.GetViewportSize`)))
  (bind (_locationx _locationy) (`PlayerController.GetMousePosition` (`GameplayStatics.GetPlayerController` 0)))
  (return (`KismetMathLibrary.MakeVector2D` (* (/ _locationx _returnvalue_x) 64.0) (* (/ _locationy _returnvalue_y) 64.0))))