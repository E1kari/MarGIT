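; Actor component that gives its owner a health pool and handles its death.
; BeginPlay fills current health to the maximum, and HSOnTakeDamage subtracts the damage amount from it.
; When health reaches zero or below, HSOnActorDeath sends a death message to the owner through BPI_HealthSystemInterface, if the owner implements it.
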(event `self.ReceiveBeginPlay`
  (set `self.CurrentHealthPoints` (`self.MaxHealthPoints`)))

(fn `HS_OnActorDeath`
  (bind _returnvalue (`self.GetOwner`))
  (if (`KismetSystemLibrary.DoesImplementInterface` _returnvalue "/Game/Blueprints/Interfaces/BPI_HealthSystemInterface.BPI_HealthSystemInterface_C")
    (message `/Game/Blueprints/Interfaces/BPI_HealthSystemInterface.HSI_OnDeath` _returnvalue)))

(fn `HS_OnTakeDamage`
  (params (DamageAmount :type "Float (double-precision)"))
  (bind _output_get (set `self.CurrentHealthPoints` (- (`self.CurrentHealthPoints`) DamageAmount)))
  (if (<= _output_get 0.0)
    (`self.HS_OnActorDeath`)))