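; BPC_EffectManager is a component that holds active effect objects and lets them react to ticks and incoming damage.
; EMAddEffect constructs each given effect class and notifies it on application, while EMRemoveEffect notifies and drops one.
; Tick forwards DeltaSeconds to every active effect.
; EMCallGetHit passes damage through the effects in order, subtracting what each returns and returning the remainder.
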(event `self.ReceiveTick`
  (params (DeltaSeconds :type "Float (single-precision)"))
  (if (> (`self.ActiveEffectsCount`) 0)
    (for _array_element (`self.ActiveEffects`)
      (`/Game/Spells_And_Effects/Effects/BP_Effect_Base.OnUpdateFunction` _array_element DeltaSeconds))))

(fn `EM_AddEffect`
  (params (Effects :type "Array of /Game/Spells_And_Effects/Effects/BP_Effect_Base Class Reference") (EffectOwner :type "/Game/Blueprints/Interfaces/BPI_EffectTargetInterface Interface"))
  (bind _activeeffects (`self.ActiveEffects`))
  (bind _activeeffects_2 (`self.ActiveEffects`))
  (for _array_element Effects
    (bind _returnvalue (`|GenericCreateObject` _array_element))
    (bind _returnvalue_2 (`KismetArrayLibrary.Array_AddUnique` _activeeffects _returnvalue))
    (if (== _returnvalue_2 (`KismetArrayLibrary.Array_LastIndex` _activeeffects))
      (`/Game/Spells_And_Effects/Effects/BP_Effect_Base.OnEffectApplied` (`|GetArrayItem` _activeeffects_2 (`KismetArrayLibrary.Array_LastIndex` _activeeffects_2)) EffectOwner self)
      (`/Engine/EditorBlueprintResources/StandardMacros.IncrementInt` (`self.ActiveEffectsCount`)
        (:`  `
          (`KismetSystemLibrary.PrintString` "Effect added"))))))

(fn `EM_CallGetHit`
  (params (DamageAmount :type "Float (double-precision)"))
  (returns (RestDamageAmount :type "Float (double-precision)"))
  (locals (RestDamageCounter :type "Float (double-precision)"))
  (bind _output_get (set `local.RestDamageCounter` DamageAmount))
  (for _array_element (`self.ActiveEffects`)
    (bind _restdamageamount (`/Game/Spells_And_Effects/Effects/BP_Effect_Base.OnGetHit` _array_element _output_get))
    (set `local.RestDamageCounter` (- (`local.RestDamageCounter`) _restdamageamount)))
  (return (`local.RestDamageCounter`)))

(fn `EM_RemoveEffect`
  (params (Effect :type "/Game/Spells_And_Effects/Effects/BP_Effect_Base Object Reference"))
  (`/Game/Spells_And_Effects/Effects/BP_Effect_Base.OnEffectRemoved` Effect)
  (`KismetArrayLibrary.Array_RemoveItem` (`self.ActiveEffects`) Effect)
  (`/Engine/EditorBlueprintResources/StandardMacros.DecrementInt` (`self.ActiveEffectsCount`)))