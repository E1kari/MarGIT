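; BP_Effect_SlowDown is a spell effect that reduces the movement speed of its owner while applied.
; On apply, it caches the owner's current speed through ETI getter calls, then sets it reduced by the SlowDownPercentage fraction.
; On removal, it writes the cached speed back, overriding any speed changes made in the meantime.
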(fn `OnEffectApplied`
  (bind _effectowner (`self.EffectOwner`))
  (bind _movementspeed (`/Game/Blueprints/Interfaces/BPI_EffectTargetInterface.ETI_GetMovementSpeed` _effectowner))
  (bind _output_get (set `self.BaseMovementSpeed` _movementspeed))
  (`/Game/Blueprints/Interfaces/BPI_EffectTargetInterface.ETI_SetMovementSpeed` _effectowner (* _output_get (- 1.0 (`self.SlowDownPercentage`)))))

(fn `OnEffectRemoved`
  (`/Game/Blueprints/Interfaces/BPI_EffectTargetInterface.ETI_SetMovementSpeed` (`self.EffectOwner`) (`self.BaseMovementSpeed`)))