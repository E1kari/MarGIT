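; Spell effect that lets its owner fly by adjusting gravity and adding flight input controls.
; On apply, it adds the fly input mapping context, caches the default gravity scale and sets separate up and down flying gravity scales through the effect owner's interface.
; On removal it reverses both changes, and it can optionally remove itself through the effect manager when the owner gets hit.
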(fn `OnEffectApplied`
  (bind _playercontroller (`/Game/Blueprints/Interfaces/BPI_EffectTargetInterface.ETI_GetPlayerController` (`self.EffectOwner`)))
  (`EnhancedInputSubsystemInterface.AddMappingContext` (pcsubsystem `EnhancedInputLocalPlayerSubsystem` _playercontroller) "/Game/Inputs/InputMappingContext/IMC_SpellEffectFly.IMC_SpellEffectFly" 1 (struct))
  (bind _gravityscale (`/Game/Blueprints/Interfaces/BPI_EffectTargetInterface.ETI_GetGravityScale` (`self.EffectOwner`)))
  (set `self.DefaultGravityScale` _gravityscale)
  (`/Game/Blueprints/Interfaces/BPI_EffectTargetInterface.ETI_SetFlyingGravityScale` (`self.EffectOwner`) (`self.FlyingUpGravityScale`) (`self.FlyingDownGravityScale`)))

(fn `OnEffectRemoved`
  (bind _playercontroller (`/Game/Blueprints/Interfaces/BPI_EffectTargetInterface.ETI_GetPlayerController` (`self.EffectOwner`)))
  (`EnhancedInputSubsystemInterface.RemoveMappingContext` (pcsubsystem `EnhancedInputLocalPlayerSubsystem` _playercontroller) "/Game/Inputs/InputMappingContext/IMC_SpellEffectFly.IMC_SpellEffectFly" (struct))
  (`/Game/Blueprints/Interfaces/BPI_EffectTargetInterface.ETI_SetGravityScale` (`self.EffectOwner`) (`self.DefaultGravityScale`)))

(fn `OnGetHit`
  (params (DamageAmount :type "Float (double-precision)"))
  (returns (RestDamageAmount :type "Float (double-precision)"))
  (if (`self.RemoveOnHit`)
    (`/Game/Blueprints/Components/BPC_EffectManager.EM_RemoveEffect` (`self.EffectManager`) self)
    (return 0.0)
    (else
      (return 0.0))))