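; BP_Effect_GravityReversal is a spell effect that changes its owner's gravity while active, presumably reversing it as the name suggests.
; On apply, it caches the owner's gravity scale as DefaultGravity through ETI-prefixed calls, then sends NewGravity to the owner.
; On removal, it runs the parent logic and restores the cached value.
; The apply override does not call its parent.
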(fn `OnEffectApplied`
  (bind _gravityscale (`/Game/Blueprints/Interfaces/BPI_EffectTargetInterface.ETI_GetGravityScale` (`self.EffectOwner`)))
  (set `self.DefaultGravity` _gravityscale)
  (`/Game/Blueprints/Interfaces/BPI_EffectTargetInterface.ETI_OnGravityChange` (`self.EffectOwner`) (`self.NewGravity`)))

(fn `OnEffectRemoved`
  (`parent.OnEffectRemoved`)
  (`/Game/Blueprints/Interfaces/BPI_EffectTargetInterface.ETI_OnGravityChange` (`self.EffectOwner`) (`self.DefaultGravity`)))