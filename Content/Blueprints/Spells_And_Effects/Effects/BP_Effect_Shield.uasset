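; A shield effect that absorbs incoming damage from a pool of shield points held by the effect.
; Initialization fills the pool to its maximum, and each hit drains it, returning the damage amount or, when depleted, the points that remained before that hit.
; Depletion removes the effect through its effect manager.
; On removal, the effect's owner casts an explosion spell.
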(fn `OnEffectRemoved`
  (`/Game/Blueprints/Interfaces/BPI_EffectTargetInterface.ETI_CastSpell` (`self.EffectOwner`) (`self.ExplosionSpell`)))

(fn `OnGetHit`
  (params (DamageAmount :type "Float (double-precision)"))
  (returns (RestDamageAmount :type "Float (double-precision)"))
  (locals (StartingPoints :type "Float (double-precision)"))
  (bind _currentshieldpoints (`self.CurrentShieldPoints`))
  (set `local.StartingPoints` _currentshieldpoints)
  (bind _output_get (set `self.CurrentShieldPoints` (- _currentshieldpoints DamageAmount)))
  (if (> _output_get 0.0)
    (return DamageAmount)
    (else
      (`/Game/Blueprints/Components/BPC_EffectManager.EM_RemoveEffect` (`self.EffectManager`) self)
      (return (`local.StartingPoints`)))))

(fn `OnInit`
  (params (EffectOwner :type "/Game/Blueprints/Interfaces/BPI_EffectTargetInterface Interface") (EffectManager :type "/Game/Blueprints/Components/BPC_EffectManager Object Reference"))
  (`parent.OnInit` EffectOwner EffectManager)
  (set `self.CurrentShieldPoints` (`self.MaxShieldPoints`)))