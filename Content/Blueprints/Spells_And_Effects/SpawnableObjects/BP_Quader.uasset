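; BP_Quader is a spawnable spell object with a scalable mesh that reacts to damage.
; Damage caused by a BP_Spell_PullProjectile destroys it immediately, while all other damage is forwarded to OnTakeDamage.
; Its construction script runs the parent's, then applies the Scale variable to the mesh in world space.
; The ETI getters are stubbed, reporting zero gravity scale and movement speed and no player controller.
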(event `self.ReceiveAnyDamage`
  (params (Damage :type "Float (single-precision)") (DamageType :type "DamageType Object Reference") (InstigatedBy :type "Controller Object Reference") (DamageCauser :type "Actor Object Reference"))
  (if (`GameplayStatics.ObjectIsA` DamageCauser "/Game/Blueprints/Spells_And_Effects/Spells/Spells/BP_Spell_PullProjectile.BP_Spell_PullProjectile_C")
    (`self.K2_DestroyActor`)
    (else
      (`self.OnTakeDamage` Damage DamageType))))

(fn `ETI_GetGravityScale`
  (returns (GravityScale :type "Float (double-precision)"))
  (return 0.0))

(fn `ETI_GetMovementSpeed`
  (returns (MovementSpeed :type "Float (double-precision)"))
  (return 0.0))

(fn `ETI_GetPlayerController`
  (returns (PlayerController :type "PlayerController Object Reference"))
  (return null))

(fn `UserConstructionScript`
  (`parent.UserConstructionScript`)
  (`SceneComponent.SetWorldScale3D` (`self.Mesh`) (`self.Scale`)))