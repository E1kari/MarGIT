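; BP_LightningSphere is a chain lightning effect that damages its main target on spawn, losing damage with each jump cycle.
; After a timer, it rolls a jump chance for every other Character overlapping its collision sphere.
; Successful rolls spawn new spheres carrying the incremented cycle, so chains branch and can revisit earlier targets.
; The sphere destroys itself after jumping, but only while within the cycle limit.
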(event `self.ReceiveBeginPlay`
  (`GameplayStatics.ApplyDamage` (`self.MainTarget`) (- (`self.BaseDamage`) (* (* (`self.BaseDamage`) (`self.DamageReduction`)) (`self.CurrentJumpCycle`))) null self (`self.Damage Type Class`))
  (`KismetSystemLibrary.K2_SetTimer` null "OnLightningJump" (`self.JumpTimer`)))

(fn `OnLightningJump`
  (if (<= (`self.CurrentJumpCycle`) (`self.MaxJumpCycles`))
    (`/Engine/EditorBlueprintResources/StandardMacros.IncrementInt` (`self.CurrentJumpCycle`)
      (:`  `
        (for _array_element (`PrimitiveComponent.GetOverlappingActors` (`self.SphereCollision`) "/Script/Engine.Character")
          (if (!= (`self.MainTarget`) _array_element)
            (if (<= (`KismetMathLibrary.RandomFloatInRange` 0.0 1.0) (`self.JumpChance`))
              (`|SpawnActorFromClass` "BP_LightningSphere_C" (`KismetMathLibrary.Conv_VectorToTransform` (`self.K2_GetActorLocation` _array_element)) "Undefined" "MultiplyWithRoot" null _array_element (`self.CurrentJumpCycle`) null))))
        (`self.K2_DestroyActor`)))))

(fn `UserConstructionScript`
  (`parent.UserConstructionScript`)
  (`SphereComponent.SetSphereRadius` (`self.SphereCollision`) (`self.SphereRadius`) true))