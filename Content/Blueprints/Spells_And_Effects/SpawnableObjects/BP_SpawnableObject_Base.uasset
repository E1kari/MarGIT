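; Base actor for spawnable objects in the spells and effects system, providing simple health and destruction.
; The construction script sets current health to max health.
; Incoming AnyDamage, gated by a CanTakeDamage flag, reduces health through OnTakeDamage, which calls OnDeath at zero or below to destroy the actor.
; A DGShowHitbox event toggles a ShowHitbox flag.
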(event `self.ReceiveAnyDamage`
  (params (Damage :type "Float (single-precision)") (DamageType :type "DamageType Object Reference") (InstigatedBy :type "Controller Object Reference") (DamageCauser :type "Actor Object Reference"))
  (if (`self.CanTakeDamage`)
    (`self.OnTakeDamage` Damage DamageType)))

(event `/Game/Blueprints/Interfaces/BPI_DebugGizmos.DG_ShowHitbox`
  (set `self.ShowHitbox?` (not (`self.ShowHitbox?`))))

(fn `OnDeath`
  (`self.K2_DestroyActor`))

(fn `OnTakeDamage`
  (params (DamageAmount :type "Float (double-precision)") (DamageType :type "DamageType Object Reference"))
  (bind _output_get (set `self.CurrentHealth` (- (`self.CurrentHealth`) DamageAmount)))
  (if (<= _output_get 0.0)
    (`self.OnDeath`)))

(fn `UserConstructionScript`
  (set `self.CurrentHealth` (`self.MaxHealth`)))