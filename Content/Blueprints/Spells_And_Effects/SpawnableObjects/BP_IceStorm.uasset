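; BP_IceStorm is a spawnable Ice Storm spell actor that exists for a set Duration, then destroys itself on a timer.
; The Construction Script sizes the DamageCollision sphere from DamageRadius and raises the Niagara effect by the same amount.
; ShowHitbox controls the sphere's in-game visibility, extending the parent's DGShowHitbox event.
; No damage logic runs in this graph; the authority-gated effect add and remove chains are unconnected.
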(event `self.ReceiveBeginPlay`
  (`KismetSystemLibrary.K2_SetTimerDelegate` (delegate `DestroyIceStorm`) (`self.Duration`)))

(event `DestroyIceStorm`
  (`self.K2_DestroyActor`))

(event `/Game/Blueprints/Interfaces/BPI_DebugGizmos.DG_ShowHitbox`
  (`parent.DG_ShowHitbox`)
  (if (`self.ShowHitbox?`)
    (`SceneComponent.SetHiddenInGame` (`self.DamageCollision`) false false)
    (else
      (`SceneComponent.SetHiddenInGame` (`self.DamageCollision`) true false))))

(fn `UserConstructionScript`
  (bind _damageradius (`self.DamageRadius`))
  (`parent.UserConstructionScript`)
  (`SphereComponent.SetSphereRadius` (`self.DamageCollision`) _damageradius true)
  (`SceneComponent.K2_SetRelativeLocation` (`self.Niagara`) (`KismetMathLibrary.MakeVector` 0.0 0.0 _damageradius) false false)
  (if (`self.ShowHitbox?`)
    (`SceneComponent.SetHiddenInGame` (`self.DamageCollision`) false false)))