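; BP_BaseSpell is a base spell actor with a box collision hitbox.
; On BeginPlay it destroys itself wherever it lacks authority, so it persists only on the authoritative side.
; A ShowHitbox flag reveals the box and its children at construction, and the DGShowHitbox event flips that flag at runtime to show or hide the box alone.
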(event `self.ReceiveBeginPlay`
  (if (not (`self.HasAuthority`))
    (`self.K2_DestroyActor`)))

(event `/Game/Blueprints/Interfaces/BPI_DebugGizmos.DG_ShowHitbox`
  (bind _output_get (set `self.ShowHitbox?` (not (`self.ShowHitbox?`))))
  (if _output_get
    (`SceneComponent.SetHiddenInGame` (`self.BoxCollision`) false false)
    (else
      (`SceneComponent.SetHiddenInGame` (`self.BoxCollision`) true false))))

(fn `UserConstructionScript`
  (if (`self.ShowHitbox?`)
    (`SceneComponent.SetHiddenInGame` (`self.BoxCollision`) false true)))