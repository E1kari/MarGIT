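; BP_Spell_ProjectileAoE is a child spell projectile that explodes for area damage.
; On collision it applies full radial damage at its collision box, crediting the spell owner's controller as instigator.
; It then spawns a BP_MasterField actor at its transform and destroys itself.
; Reaching maximum distance runs the same collision logic, so the spell detonates even without hitting anything.
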(fn `OnMaxDistanceReached`
  (`self.OnProjectileCollision` null))

(fn `OnProjectileCollision`
  (params (OtherActor :type "Actor Object Reference") (Hit :type "HitResult Structure"))
  (`GameplayStatics.ApplyRadialDamage` :`BaseDamage` (`self.DamageAmount`) :`Origin` (`SceneComponent.K2_GetComponentLocation` (`self.BoxCollision`)) :`DamageRadius` (`self.DamageRadius`) :`DamageTypeClass` (`self.Damage Type Class`) :`DamageCauser` self :`InstigatedByController` (`Pawn.GetController` (`self.SpellOwner`)) :`bDoFullDamage` true)
  (`|SpawnActorFromClass` "/Game/Destructables/BP_MasterField.BP_MasterField_C" (`self.GetTransform`) "Undefined" "MultiplyWithRoot" null null)
  (`self.K2_DestroyActor`))

(fn `UserConstructionScript`
  (`parent.UserConstructionScript`))