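; Spell projectile that pulls nearby actors toward its end point and deals radial damage there.
; On collision or at max distance, it sends a knockback impulse toward itself to actors overlapping the pull sphere, applies damage, then destroys itself.
; Construction sizes the pull and damage spheres from their radius variables.
; The hitbox debug event toggles the damage sphere but leaves the pull sphere visible in both branches.
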(event `/Game/Blueprints/Interfaces/BPI_DebugGizmos.DG_ShowHitbox`
  (`parent.DG_ShowHitbox`)
  (if (`self.ShowHitbox?`)
    (`SceneComponent.SetHiddenInGame` (`self.DamageRadiusSphere`) false false)
    (`SceneComponent.SetHiddenInGame` (`self.PullRadiusSphere`) false false)
    (else
      (`SceneComponent.SetHiddenInGame` (`self.DamageRadiusSphere`) true false)
      (`SceneComponent.SetHiddenInGame` (`self.PullRadiusSphere`) false false))))

(fn `OnMaxDistanceReached`
  (`self.OnProjectileCollision` null))

(fn `OnProjectileCollision`
  (params (OtherActor :type "Actor Object Reference") (Hit :type "HitResult Structure"))
  (for _array_element (`PrimitiveComponent.GetOverlappingActors` (`self.PullRadiusSphere`) null)
    (message `/Game/Blueprints/Interfaces/BPI_EffectTargetInterface.ETI_OnKnockback` _array_element (* (`KismetMathLibrary.GetDirectionUnitVector` (`self.K2_GetActorLocation` _array_element) (`SceneComponent.K2_GetComponentLocation` (`self.BoxCollision`))) (`self.ImpulseStrenght`))))
  (`GameplayStatics.ApplyRadialDamage` :`BaseDamage` (`self.Base Damage`) :`Origin` (`SceneComponent.K2_GetComponentLocation` (`self.BoxCollision`)) :`DamageRadius` (`self.DamageRadius`) :`DamageTypeClass` (`self.DamageType`) :`DamageCauser` self :`InstigatedByController` (`Pawn.GetController` (`self.SpellOwner`)) :`bDoFullDamage` (`self.DoFullDamage`))
  (`self.K2_DestroyActor`))

(fn `UserConstructionScript`
  (`parent.UserConstructionScript`)
  (`SphereComponent.SetSphereRadius` (`self.PullRadiusSphere`) (`self.PullRadius`) true)
  (`SphereComponent.SetSphereRadius` (`self.DamageRadiusSphere`) (`self.DamageRadius`) true))