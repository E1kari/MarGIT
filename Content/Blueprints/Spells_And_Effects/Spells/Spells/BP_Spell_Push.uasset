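; BP_Spell_Push is a one-shot spell that knocks back characters in a box in front of it, then destroys itself.
; On BeginPlay it shifts the box, sized by BoxScale at construction, forward by its X extent and gathers overlapping Characters.
; A visibility trace from the Arrow filters out blocked targets.
; Each remaining target gets a knockback message pointing away from SpellOwner, scaled by PushForce.
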(event `self.ReceiveBeginPlay`
  (bind _boxcollision (`self.BoxCollision`))
  (bind _boxscale_x (`KismetMathLibrary.BreakVector` (`self.BoxScale`)))
  (`parent.ReceiveBeginPlay`)
  (`SceneComponent.K2_SetWorldLocation` _boxcollision (+ (`SceneComponent.K2_GetComponentLocation` _boxcollision) (* (`SceneComponent.GetForwardVector` _boxcollision) _boxscale_x)) false true)
  (for _array_element (`PrimitiveComponent.GetOverlappingActors` (`self.BoxCollision`) "/Script/Engine.Character")
    (bind _returnvalue (`self.K2_GetActorLocation` _array_element))
    (bind _outhit (`KismetSystemLibrary.LineTraceSingle` (`SceneComponent.K2_GetComponentLocation` (`self.Arrow`)) _returnvalue "TraceTypeQuery1"))
    (if (== _array_element (`.HitActor` (`GameplayStatics.BreakHitResult` _outhit)))
      (message `/Game/Blueprints/Interfaces/BPI_EffectTargetInterface.ETI_OnKnockback` _array_element (* (`KismetMathLibrary.GetDirectionUnitVector` (`self.K2_GetActorLocation` (`self.SpellOwner`)) _returnvalue) (`self.PushForce`)))))
  (`self.K2_DestroyActor`))

(fn `UserConstructionScript`
  (bind _boxscale (`self.BoxScale`))
  (`parent.UserConstructionScript`)
  (`BoxComponent.SetBoxExtent` (`self.BoxCollision`) _boxscale true)
  (`SceneComponent.K2_AddLocalOffset` (`self.Arrow`) (`KismetMathLibrary.MakeVector` (* (.x _boxscale) -1.0)) false false))