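; BP_Spell_BlackHole is a raycast-targeted spell that spawns a black hole at the aimed point.
; Its hit and no-hit handlers pass the impact location or the ray endpoint, respectively, to a server RPC.
; The RPC spawns BP_BlackHole there, handing over the spell owner as owner and instigator along with the hitbox display setting.
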(event `RPC_Server_SpawnBlackHole`
  (params (Position :type "Vector Structure"))
  (bind _spellowner (`self.SpellOwner`))
  (`|SpawnActorFromClass` "/Game/Blueprints/Spells_And_Effects/SpawnableObjects/BP_BlackHole.BP_BlackHole_C" (`KismetMathLibrary.Conv_VectorToTransform` Position) "Undefined" "MultiplyWithRoot" null _spellowner (`self.ShowHitbox?`) _spellowner))

(fn `OnNoRaycastHit`
  (params (RaycastEndpoint :type "Vector Structure"))
  (`self.RPC_Server_SpawnBlackHole` RaycastEndpoint))

(fn `OnRaycastHit`
  (params (HitResult :type "HitResult Structure"))
  (`self.RPC_Server_SpawnBlackHole` (`.Location` (`GameplayStatics.BreakHitResult` HitResult))))

(fn `UserConstructionScript`
  (`parent.UserConstructionScript`))