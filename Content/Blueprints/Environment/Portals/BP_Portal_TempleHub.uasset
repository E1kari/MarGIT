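; BP_Portal_TempleHub is a temple hub portal that streams in its linked level and pairs with that section's portal.
; When the third-person character enters the preload volume, it starts a non-blocking level load, then searches for the BP_Portal_TempleSections whose OwnLevel matches.
; If found, it registers itself there with its index in AllTempleHubPortals.
; The unload logic, guarded against just-teleported players, is disconnected.
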(event `self.PreloadVolume.OnComponentBeginOverlap`
  (params (OverlappedComponent :type "PrimitiveComponent Object Reference") (OtherActor :type "Actor Object Reference") (OtherComp :type "PrimitiveComponent Object Reference") (OtherBodyIndex :type Integer) (bFromSweep :type Boolean) (SweepResult :type "HitResult Structure (by ref)"))
  (bind _linkedportal (`self.LinkedPortal`))
  (if (`GameplayStatics.ObjectIsA` OtherActor "/Game/Blueprints/Player/Blueprints/BP_ThirdPersonCharacter.BP_ThirdPersonCharacter_C")
    (`GameplayStatics.LoadStreamLevelBySoftObjectPtr` (`self.LinkedLevel`) true)
    (bind _outactors (`GameplayStatics.GetAllActorsOfClass` "/Game/Blueprints/Environment/Portals/BP_Portal_TempleSections.BP_Portal_TempleSections_C"))
    (for _array_element _outactors
      (if (== (`/Game/Blueprints/Environment/Portals/BP_Portal_Base.OwnLevel` _array_element) (`self.LinkedLevel`))
        (set `self.LinkedPortal` _array_element)))
    (`/Engine/EditorBlueprintResources/StandardMacros.IsValid` _linkedportal
      (:`Is Valid`
        (bind _asbp_portal_temple_sections (cast `/Game/Blueprints/Environment/Portals/BP_Portal_TempleSections` _linkedportal))
        (`/Game/Blueprints/Environment/Portals/BP_Portal_TempleSections.AddLinkedPortal` _asbp_portal_temple_sections (`KismetArrayLibrary.Array_Find` (`self.AllTempleHubPortals`) self) self)))))

(fn `UserConstructionScript`
  (`parent.UserConstructionScript`))