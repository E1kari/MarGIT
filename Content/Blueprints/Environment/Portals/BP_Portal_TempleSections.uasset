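; Portal Blueprint for temple sections that streams in its linked level and resolves its destination portal.
; When the third-person character overlaps PreloadVolume, it loads LinkedLevel visibly without blocking.
; If LinkedPortal is invalid, it has GI_GameInstance run AddAllPortals, then looks up the partner in AllTempleHubPortals by LinkedPortalIndex.
; AddLinkedPortal can also set the index and reference directly.
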(event `AddLinkedPortal`
  (params (LinkedPortalIndex :type Integer) (LinkedPortalRef :type "/Game/Blueprints/Environment/Portals/BP_Portal_Base Object Reference"))
  (set `self.Linked Portal Index` LinkedPortalIndex)
  (set `self.LinkedPortal` LinkedPortalRef))

(event `self.PreloadVolume.OnComponentBeginOverlap`
  (params (OverlappedComponent :type "PrimitiveComponent Object Reference") (OtherActor :type "Actor Object Reference") (OtherComp :type "PrimitiveComponent Object Reference") (OtherBodyIndex :type Integer) (bFromSweep :type Boolean) (SweepResult :type "HitResult Structure (by ref)"))
  (if (`GameplayStatics.ObjectIsA` OtherActor "/Game/Blueprints/Player/Blueprints/BP_ThirdPersonCharacter.BP_ThirdPersonCharacter_C")
    (`GameplayStatics.LoadStreamLevelBySoftObjectPtr` (`self.LinkedLevel`) true)
    (`/Engine/EditorBlueprintResources/StandardMacros.IsValid` (`self.LinkedPortal`)
      (:`Is Not Valid`
        (bind _asgi_game_instance (cast `/Game/GameInstance/GI_GameInstance` (`GameplayStatics.GetGameInstance`)))
        (`/Game/GameInstance/GI_GameInstance.AddAllPortals` _asgi_game_instance)
        (set `self.LinkedPortal` (`|GetArrayItem` (`/Game/GameInstance/GI_GameInstance.AllTempleHubPortals` _asgi_game_instance) (`self.Linked Portal Index`)))))))

(fn `UserConstructionScript`
  (`parent.UserConstructionScript`))