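; BP_Portal_Hub is the hub-side portal that streams in its linked sublevel and pairs with the portal there.
; On the load event it starts a non-blocking level load, then searches BP_Portal_Sublevel actors for one whose OwnLevel matches.
; It registers itself with that portal using its index in AllHubPortals, then sets the linked portal's render target.
; AddLinkedPortal here simply stores the given reference, ignoring the index.
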(event `self.OnLoadOtherLevel`
  (`GameplayStatics.LoadStreamLevelBySoftObjectPtr` (`self.LinkedSubLevel`) true)
  (bind _outactors (`GameplayStatics.GetAllActorsOfClass` "/Game/Blueprints/Environment/Portals/NewTry/BP_Portal_Sublevel.BP_Portal_Sublevel_C"))
  (for _array_element _outactors
    (if (== (`/Game/Blueprints/Environment/Portals/NewTry/BP_Portal.OwnLevel` _array_element) (`self.LinkedSubLevel`))
      (set `self.LinkedPortal` _array_element)))
  (bind _linkedportal (`self.LinkedPortal`)
    (:`then`
      (`self.AddLinkedPortal` _linkedportal (`KismetArrayLibrary.Array_Find` (`self.AllHubPortals`) self) self)
      (`self.SetLinkedPortalRenderTarget`))
    (:`else`)))

(fn `AddLinkedPortal`
  (params (Index :type Integer) (LinkedPortalRef :type "/Game/Blueprints/Environment/Portals/NewTry/BP_Portal Object Reference"))
  (set `self.LinkedPortal` LinkedPortalRef))

(fn `UserConstructionScript`
  (`parent.UserConstructionScript`))