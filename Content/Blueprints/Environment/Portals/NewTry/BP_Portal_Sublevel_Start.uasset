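; Start-side sublevel portal, a child portal Blueprint that streams in its linked sublevel and pairs itself with a temple hub portal.
; On the load event it streams the level without blocking, then sets the linked portal render target.
; If no link is valid, it refreshes the GameInstance portal list, takes the hub portal at the stored index and links both ways.
; AddLinkedPortal stores that hub index in the GameInstance and sets the link.
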(event `self.OnLoadOtherLevel`
  (`GameplayStatics.LoadStreamLevelBySoftObjectPtr` (`self.LinkedSubLevel`) true)
  (`self.LinkedPortal`
    (:`then`
      (`self.SetLinkedPortalRenderTarget`))
    (:`else`
      (bind _asgi_game_instance (cast `/Game/Blueprints/GameInstance/GI_GameInstance` (`GameplayStatics.GetGameInstance`)))
      (`/Game/Blueprints/GameInstance/GI_GameInstance.AddAllPortalsNew` _asgi_game_instance)
      (bind _output_get (set `self.LinkedPortal` (`|GetArrayItem` (`/Game/Blueprints/GameInstance/GI_GameInstance.AllTempleHubPortalsNew` _asgi_game_instance) (`/Game/Blueprints/GameInstance/GI_GameInstance.PortalHubIndex` _asgi_game_instance))))
      (`self.AddLinkedPortal` _output_get 0 self)
      (`self.SetLinkedPortalRenderTarget`))))

(fn `AddLinkedPortal`
  (params (Index :type Integer) (LinkedPortalRef :type "/Game/Blueprints/Environment/Portals/NewTry/BP_Portal Object Reference"))
  (bind _asgi_game_instance (cast `/Game/Blueprints/GameInstance/GI_GameInstance` (`GameplayStatics.GetGameInstance`)))
  (set `/Game/Blueprints/GameInstance/GI_GameInstance.PortalHubIndex` Index _asgi_game_instance)
  (set `self.LinkedPortal` LinkedPortalRef))

(fn `UserConstructionScript`
  (`parent.UserConstructionScript`))