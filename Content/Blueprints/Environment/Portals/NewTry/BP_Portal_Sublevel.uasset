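; Portal actor that streams in its linked sublevel and pairs itself with a portal from the temple hub list.
; On the load event it starts a non-blocking load, then sets the linked portal's render target if the link is already valid.
; Otherwise it refreshes the GameInstance's hub portal list, takes the entry at its linked index and registers itself on that portal at index 0.
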(event `self.OnLoadOtherLevel`
  (`GameplayStatics.LoadStreamLevelBySoftObjectPtr` (`self.LinkedSubLevel`) true)
  (`self.LinkedPortal`
    (:`then`
      (`self.SetLinkedPortalRenderTarget`))
    (:`else`
      (bind _asgi_game_instance (cast `/Game/GameInstance/GI_GameInstance` (`GameplayStatics.GetGameInstance`)))
      (`/Game/GameInstance/GI_GameInstance.AddAllPortalsNew` _asgi_game_instance)
      (bind _output_get (set `self.LinkedPortal` (`|GetArrayItem` (`/Game/GameInstance/GI_GameInstance.AllTempleHubPortalsNew` _asgi_game_instance) (`self.LinkedPortalIndex`))))
      (`self.AddLinkedPortal` _output_get 0 self))))

(fn `AddLinkedPortal`
  (params (Index :type Integer) (LinkedPortalRef :type "/Game/Blueprints/Environment/Portals/NewTry/BP_Portal Object Reference"))
  (set `self.LinkedPortalIndex` Index)
  (set `self.LinkedPortal` LinkedPortalRef))

(fn `UserConstructionScript`
  (`parent.UserConstructionScript`))