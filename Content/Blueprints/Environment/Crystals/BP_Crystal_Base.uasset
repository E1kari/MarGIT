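; BP_Crystal_Base is a base crystal actor that toggles between active and inactive whenever it takes damage.
; The construction script seeds IsActive from StartAsActive, and each toggle calls OnActivate or OnDeactivate, empty hooks that child classes can override.
; A RepNotify on IsActive swaps the CylinderBody material to show the current state.
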(event `self.ReceiveAnyDamage`
  (params (Damage :type "Float (single-precision)") (DamageType :type "DamageType Object Reference") (InstigatedBy :type "Controller Object Reference") (DamageCauser :type "Actor Object Reference"))
  (bind _output_get (set `self.IsActive` (not (`self.IsActive`))))
  (if _output_get
    (`self.OnActivate`)
    (else
      (`self.OnDeactivate`))))

(fn `OnActivate`)

(fn `OnDeactivate`)

(fn `OnRep_IsActive`
  (if (`self.IsActive`)
    (`PrimitiveComponent.SetMaterial` (`self.CylinderBody`) 0 (`self.Material_Active`))
    (else
      (`PrimitiveComponent.SetMaterial` (`self.CylinderBody`) 0 (`self.Material_Deactive`)))))

(fn `UserConstructionScript`
  (set `self.IsActive` (`self.StartAsActive`)))