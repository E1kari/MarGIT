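; Looping moving platform that travels along a referenced spline, wrapping around on circular paths or ping-ponging on open ones.
; BeginPlay sets the timeline play rate and calls StartOnBegin, while EIonActivate and EIonDeactivate play and stop the movement.
; Timeline updates map MoveTrack to distance along the spline to set the actor's world location without sweep.
; On finish, the timeline restarts for circular paths, otherwise a toggled flag alternates forward and reverse playback.
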(event `self.ReceiveBeginPlay`
  (`self.SetPlayRate` (`self.MovementTimeline`))
  (`self.StartOnBegin`))

(event `/Game/Blueprints/Interfaces/BPI_EnvironmentInterface.EI_OnActivate`
  (bind _spline (`/Game/Blueprints/Environment/SplinePath/BP_SplinePath.Spline` (`self.SplineReference`)))
  (bind (_direction _movetrack) (`Timeline|MovementTimeline` :!label _label)
    (:`Update`
      (`self.K2_SetActorLocation` (`SplineComponent.GetLocationAtDistanceAlongSpline` _spline (`KismetMathLibrary.Lerp` 0.0 (`SplineComponent.GetSplineLength` _spline) _movetrack) "World")))
    (:`Finished`
      (if (`self.SplinePathIsCircle`)
        (goto _label :!via `PlayFromStart`)
        (else
          (set `self.StartedAtStart` (not (`self.StartedAtStart`)))
          (if (not (`self.StartedAtStart`))
            (goto _label :!via `PlayFromStart`)
            (else
              (goto _label :!via `ReverseFromEnd`))))))))

(event `/Game/Blueprints/Interfaces/BPI_EnvironmentInterface.EI_OnDeactivate`
  (goto _label :!via `Stop`))

(fn `UserConstructionScript`
  (`parent.UserConstructionScript`)
  (set `self.StartedAtStart` false))