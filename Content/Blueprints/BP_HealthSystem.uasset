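; Health system that an owning actor uses to track health points and a Resistance buffer, with health set to maximum on BeginPlay.
; AddToResistance grows the buffer, and TakeDamage drains it first, passing any overflow to health.
; When overflow drops health to zero or below, ActorDeath sends OnDeathMessage to the owner through BPI_HealthSystemInterface, leaving Resistance negative.
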(event `self.ReceiveBeginPlay`
  (set `self.CurrentHealthPoints` (`self.MaxHealthPoints`)))

(fn `ActorDeath`
  (bind _returnvalue (`self.GetOwner`))
  (if (`KismetSystemLibrary.DoesImplementInterface` _returnvalue "/Game/Blueprints/BPI_HealthSystemInterface.BPI_HealthSystemInterface_C")
    (message `/Game/Blueprints/BPI_HealthSystemInterface.OnDeath` _returnvalue)))

(fn `AddToResistance`
  (params (AddValue :type "Float (double-precision)"))
  (set `self.Resistance` (+ AddValue (`self.Resistance`))))

(fn `TakeDamage`
  (params (DamageAmount :type "Float (double-precision)"))
  (bind _output_get (set `self.Resistance` (- (`self.Resistance`) DamageAmount)))
  (if (< _output_get 0.0)
    (bind _output_get_2 (set `self.CurrentHealthPoints` (+ (`self.CurrentHealthPoints`) (`self.Resistance`))))
    (if (> _output_get_2 0.0)
      (set `self.Resistance` 0.0)
      (else
        (`self.ActorDeath`)))))