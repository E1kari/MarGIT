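; Rune-recognition actor, named for ONNX inference, that handles the drawn rune's Niagara trail and slow-motion; no inference logic appears in these graphs.
; On BeginPlay, a server RPC enables time dilation only with fewer than two players, gating the start/stop RPCs that switch global dilation.
; Trail updates activate the effect once and move its spawn point.
; Recognition results deactivate it, with failure also adding downward gravity and setting particle lifetime.
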(event `self.ReceiveBeginPlay`
  (`self.RPC_OIA_Server_GetPlayerCount`))

(event `RPC_OIA_Server_GetPlayerCount`
  (bind _asbp_third_person_game_mode (cast `/Game/ThirdPerson/Blueprints/BP_ThirdPersonGameMode` (`GameplayStatics.GetGameMode`)))
  (bind _returnvalue (`GameModeBase.GetNumPlayers` _asbp_third_person_game_mode))
  (if (< _returnvalue 2)
    (set `self.IsTimeDelationEnabled` true)
    (else
      (set `self.IsTimeDelationEnabled` false))))

(event `RPC_OIA_Server_StartTimeDelation`
  (`self.StartTimeDelation`))

(event `RPC_OIA_Server_StopTimeDelation`
  (`self.StopTimeDelation`))

(fn `RuneNotRecognized`
  (bind _runetrailfx (`self.RuneTrailFX`))
  (`NiagaraComponent.SetNiagaraVariableVec3` _runetrailfx "User.GravityForce" (0.0 0.0 -980.0))
  (`NiagaraComponent.SetNiagaraVariableFloat` _runetrailfx "LifeTime" 1.5)
  (`ActorComponent.Deactivate` _runetrailfx))

(fn `RuneRecognized`
  (`ActorComponent.Deactivate` (`self.RuneTrailFX`)))

(fn `StartTimeDelation`
  (if (`self.IsTimeDelationEnabled`)
    (`GameplayStatics.SetGlobalTimeDilation` (`self.SlowedTimeDelation`))))

(fn `StopTimeDelation`
  (if (`self.IsTimeDelationEnabled`)
    (`GameplayStatics.SetGlobalTimeDilation` (`self.BaseTimeDelation`))))

(fn `UpdateRuneTrailTXPosition`
  (params (NewPos :type "Vector Structure"))
  (bind _runetrailfx (`self.RuneTrailFX`))
  (if (not (`self.IsFXActive`))
    (set `self.IsFXActive` true)
    (`ActorComponent.Activate` _runetrailfx false))
  (`NiagaraComponent.SetNiagaraVariableVec3` _runetrailfx "User.SpawnPos" NewPos))

(fn `UserConstructionScript`)