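; Push spell actor that delivers a one-shot knockback to everything inside a box in front of it.
; Construction sizes the box from BoxScale; BeginPlay shifts it forward by its X extent and gathers the overlapping actors.
; Each receives a knockback interface message along the direction away from SpellOwner, scaled by PushForce, then the spell destroys itself.
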(event `self.ReceiveBeginPlay`
  (bind _boxcollision (`self.BoxCollision`))
  (bind _boxscale_x (`KismetMathLibrary.BreakVector` (`self.BoxScale`)))
  (`parent.ReceiveBeginPlay`)
  (`SceneComponent.K2_SetWorldLocation` _boxcollision (+ (`SceneComponent.K2_GetComponentLocation` _boxcollision) (* (`SceneComponent.GetForwardVector` _boxcollision) _boxscale_x)) false true)
  (for _array_element (`PrimitiveComponent.GetOverlappingActors` (`self.BoxCollision`) null)
    (message `/Game/Blueprints/Interfaces/BPI_EffectTargetInterface.ETI_OnKnockback` _array_element (* (`KismetMathLibrary.GetDirectionUnitVector` (`self.K2_GetActorLocation` (`self.SpellOwner`)) (`self.K2_GetActorLocation` _array_element)) (`self.PushForce`))))
  (`self.K2_DestroyActor`))

(fn `UserConstructionScript`
  (`parent.UserConstructionScript`)
  (`BoxComponent.SetBoxExtent` (`self.BoxCollision`) (`self.BoxScale`) true))