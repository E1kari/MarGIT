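; BP_Spell_GravityPull is a projectile spell that pulls nearby actors toward its position when it collides or reaches maximum distance.
; On either event it resizes PullRadiusSphere to Radius, updating overlaps, and gathers every overlapping actor.
; Each receives a knockback message with an impulse aimed at the projectile's collision box, scaled by impulse strength, before the spell destroys itself.
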(fn `OnMaxDistanceReached`
  (`self.OnProjectileCollision` null))

(fn `OnProjectileCollision`
  (params (OtherActor :type "Actor Object Reference") (Hit :type "HitResult Structure"))
  (`SphereComponent.SetSphereRadius` (`self.PullRadiusSphere`) (`self.Radius`) true)
  (for _array_element (`PrimitiveComponent.GetOverlappingActors` (`self.PullRadiusSphere`) null)
    (message `/Game/Blueprints/Interfaces/BPI_EffectTargetInterface.ETI_OnKnockback` _array_element (* (`KismetMathLibrary.GetDirectionUnitVector` (`self.K2_GetActorLocation` _array_element) (`SceneComponent.K2_GetComponentLocation` (`self.BoxCollision`))) (`self.ImpulseStrenght`))))
  (`self.K2_DestroyActor`))

(fn `UserConstructionScript`
  (`parent.UserConstructionScript`))