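; Black hole spell that places a BP_BlackHole actor in the world at the point the spell's raycast targets.
; Both raycast outcomes feed SpawnBlackHole, using the impact location on a hit or the ray's endpoint on a miss, so either result spawns one.
; The spawned actor receives the spell's owner, and this Blueprint holds no other active logic.
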(fn `OnNoRaycastHit`
  (params (RaycastEndpoint :type "Vector Structure"))
  (`self.SpawnBlackHole` RaycastEndpoint))

(fn `OnRaycastHit`
  (params (HitResult :type "HitResult Structure"))
  (`self.SpawnBlackHole` (`.Location` (`GameplayStatics.BreakHitResult` HitResult))))

(fn `SpawnBlackHole`
  (params (SpawnPosition :type "Vector Structure"))
  (`|SpawnActorFromClass` "/Game/Spells_And_Effects/SpawnableObjects/BP_BlackHole.BP_BlackHole_C" (`KismetMathLibrary.Conv_VectorToTransform` SpawnPosition) "Undefined" "MultiplyWithRoot" null (`self.SpellOwner`) null))

(fn `UserConstructionScript`
  (`parent.UserConstructionScript`))