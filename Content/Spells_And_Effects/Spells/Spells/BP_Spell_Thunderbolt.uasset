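; BP_Spell_Thunderbolt is a Thunderbolt spell projectile with an area damage sphere, currently in a debug state.
; The construction script sizes DamageSphere from DamageRadius, and BeginPlay prints the spell name after calling the parent.
; On projectile collision it prints the count and names of actors overlapping the sphere, then destroys itself.
; The damage message call is unconnected, so this graph applies no damage.
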(event `self.ReceiveBeginPlay`
  (`parent.ReceiveBeginPlay`)
  (`KismetSystemLibrary.PrintString` "ThunderBolt"))

(fn `OnProjectileCollision`
  (params (OtherActor :type "Actor Object Reference") (Hit :type "HitResult Structure"))
  (bind _overlappingactors (`PrimitiveComponent.GetOverlappingActors` (`self.DamageSphere`) null))
  (`KismetSystemLibrary.PrintString` (`KismetStringLibrary.Conv_IntToString` (`KismetArrayLibrary.Array_Length` _overlappingactors)))
  (for _array_element _overlappingactors
    (`KismetSystemLibrary.PrintString` (`KismetSystemLibrary.GetDisplayName` _array_element)))
  (`self.K2_DestroyActor`))

(fn `UserConstructionScript`
  (`parent.UserConstructionScript`)
  (`SphereComponent.SetSphereRadius` (`self.DamageSphere`) (`self.DamageRadius`) true))