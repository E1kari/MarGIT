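; BP_Spell_AreaDenial is a spell that places thorns in the world or applies an effect to what it hits.
; Its OnRaycastHit function branches on the hit component's mobility, ignoring invalid components.
; Static geometry gets a BP_Thorns actor spawned at the impact location.
; Non-static hits, if CanApplyAsEffect is true, send SpellEffect to the hit actor through the ETIOnAddEffectMessage call.
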(fn `OnRaycastHit`
  (params (HitResult :type "HitResult Structure"))
  (bind (_bblockinghit _binitialoverlap _time _distance _location _impactpoint _normal _impactnormal _physmat _hitactor _hitcomponent) (`GameplayStatics.BreakHitResult` HitResult))
  (if (`KismetSystemLibrary.IsValid` _hitcomponent)
    (if (`|EnumEquality` (`SceneComponent.Mobility` _hitcomponent) "Static")
      (`|SpawnActorFromClass` "/Game/Spells_And_Effects/SpawnableObjects/BP_Thorns.BP_Thorns_C" (`KismetMathLibrary.Conv_VectorToTransform` _location) "Undefined" "MultiplyWithRoot" null null)
      (elif (`self.CanApplyAsEffect`)
        (message `/Game/Blueprints/Interfaces/BPI_EffectTargetInterface.ETI_OnAddEffect` _hitactor (`self.SpellEffect`))))))

(fn `UserConstructionScript`
  (`parent.UserConstructionScript`))