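; Base projectile spell that flies from where it spawns and destroys itself on reaching its maximum travel distance.
; Construction copies speed and gravity settings into the SpellMovement component.
; On the authority, BeginPlay makes the collision box ignore the spell owner and records the start position, which Tick uses for the distance check.
; Authority-side box hits go to OnProjectileCollision, an empty hook here.
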(event `self.ReceiveBeginPlay`
  (if (`self.HasAuthority`)
    (`parent.ReceiveBeginPlay`)
    (`PrimitiveComponent.IgnoreActorWhenMoving` (`self.BoxCollision`) (`self.SpellOwner`) true)
    (set `self.StartPosition` (`SceneComponent.K2_GetComponentLocation` (`self.BoxCollision`)))))

(event `self.BoxCollision.OnComponentHit`
  (params (HitComponent :type "PrimitiveComponent Object Reference") (OtherActor :type "Actor Object Reference") (OtherComp :type "PrimitiveComponent Object Reference") (NormalImpulse :type "Vector Structure") (Hit :type "HitResult Structure (by ref)"))
  (if (`self.HasAuthority`)
    (`self.OnProjectileCollision` OtherActor Hit)))

(event `self.ReceiveTick`
  (params (DeltaSeconds :type "Float (single-precision)"))
  (if (>= (`KismetMathLibrary.Vector_Distance` (`self.StartPosition`) (`SceneComponent.K2_GetComponentLocation` (`self.BoxCollision`))) (`self.MaxTravelDistance`))
    (`self.K2_DestroyActor`)))

(fn `OnProjectileCollision`
  (params (OtherActor :type "Actor Object Reference") (Hit :type "HitResult Structure")))

(fn `UserConstructionScript`
  (bind _spellmovement (`self.SpellMovement`))
  (`parent.UserConstructionScript`)
  (bind _output_get (set `ProjectileMovementComponent.MaxSpeed` (`self.MovementSpeed`) _spellmovement))
  (set `ProjectileMovementComponent.InitialSpeed` _output_get _spellmovement)
  (set `ProjectileMovementComponent.ProjectileGravityScale` (`self.GravityScale`) _spellmovement))