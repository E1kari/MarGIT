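; Base Blueprint for raycast spells, which hit by a single line trace instead of a travelling projectile.
; On BeginPlay it traces on the Visibility channel from BoxCollision along its forward vector for MaxDistance.
; The result goes to OnRaycastHit, an empty function for child spells to override, which is called whether or not the trace hits anything.
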(event `self.ReceiveBeginPlay`
  (bind _boxcollision (`self.BoxCollision`))
  (bind _returnvalue (`SceneComponent.K2_GetComponentLocation` _boxcollision))
  (bind _outhit (`KismetSystemLibrary.LineTraceSingle` _returnvalue (+ _returnvalue (* (`KismetMathLibrary.GetForwardVector` (`SceneComponent.K2_GetComponentRotation` _boxcollision)) (`self.MaxDistance`))) "TraceTypeQuery1"))
  (`self.OnRaycastHit` _outhit))

(fn `OnRaycastHit`
  (params (HitResult :type "HitResult Structure")))

(fn `UserConstructionScript`
  (`parent.UserConstructionScript`))