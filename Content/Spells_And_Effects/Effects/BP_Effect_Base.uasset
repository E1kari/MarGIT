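; Base Blueprint for timed effects that an effect manager applies to an owner.
; OnInit stores the owner and manager, then sets the remaining duration from the effect's duration.
; While ticking is enabled, the update function counts that time down and asks the manager to remove the effect at zero.
; Applied and removed hooks are empty and the hit hook returns zero, with debug prints on init and expiry.
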(fn `OnEffectApplied`)

(fn `OnEffectRemoved`)

(fn `OnGetHit`
  (params (DamageAmount :type "Float (double-precision)"))
  (returns (RestDamageAmount :type "Float (double-precision)"))
  (return 0.0))

(fn `OnInit`
  (params (EffectOwner :type "/Game/Blueprints/Interfaces/BPI_EffectTargetInterface Interface") (EffectManager :type "/Game/Blueprints/Components/BPC_EffectManager Object Reference"))
  (set `self.EffectOwner` EffectOwner)
  (set `self.EffectManager` EffectManager)
  (bind _output_get (set `self.RemainingDuration` (`self.EffectDuration`)))
  (`KismetSystemLibrary.PrintString` null "Init")
  (`KismetSystemLibrary.PrintString` null (`KismetStringLibrary.Conv_DoubleToString` _output_get)))

(fn `OnTick`
  (params (DeltaTime :type "Float (double-precision)"))
  (bind _output_get (set `self.RemainingDuration` (- (`self.RemainingDuration`) DeltaTime)))
  (if (<= _output_get 0.0)
    (`/Game/Blueprints/Components/BPC_EffectManager.EM_RemoveEffect` (`self.EffectManager`) self)
    (`KismetSystemLibrary.PrintString` null "Effect removed on Tick")))

(fn `OnUpdateFunction`
  (params (DeltaTime :type "Float (double-precision)"))
  (if (`self.IsTickEnabled`)
    (`self.OnTick` DeltaTime)))