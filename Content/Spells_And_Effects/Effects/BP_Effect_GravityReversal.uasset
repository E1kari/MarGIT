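; BP_Effect_GravityReversal is a spell effect that changes its owner's gravity for as long as it is applied.
; On apply, it stores the owner's current gravity scale as DefaultGravity, then sends NewGravity to the owner.
; On removal, it restores the stored value, with all reads and changes going through ETI-prefixed calls on the owner.
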(fn `OnEffectApplied`
  (params (EffectOwner :type "/Game/Blueprints/Interfaces/BPI_EffectTargetInterface Interface") (EffectManager :type "/Game/Blueprints/Components/BPC_EffectManager Object Reference"))
  (`parent.OnEffectApplied` EffectOwner EffectManager)
  (bind _gravityscale (`/Game/Blueprints/Interfaces/BPI_EffectTargetInterface.ETI_GetGravityScale` (`self.EffectOwner`)))
  (set `self.DefaultGravity` _gravityscale)
  (`/Game/Blueprints/Interfaces/BPI_EffectTargetInterface.ETI_OnGravityChange` (`self.EffectOwner`) (`self.NewGravity`)))

(fn `OnEffectRemoved`
  (`parent.OnEffectRemoved`)
  (`/Game/Blueprints/Interfaces/BPI_EffectTargetInterface.ETI_OnGravityChange` (`self.EffectOwner`) (`self.DefaultGravity`)))