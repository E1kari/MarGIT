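; BP_Thorns is a spawnable thorns hazard that damages and applies effects to actors within its radius for a limited duration.
; A looping timer applies damage to Characters overlapping DamageCollisionSphere, and a second timer destroys the actor.
; Sphere overlaps send effect add and remove messages when the overlapping actor has authority.
; The construction script sizes the sphere from DamageRadius.
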(event `self.ReceiveBeginPlay`
  (`KismetSystemLibrary.K2_SetTimer` null "DealDamage" (`self.DamageInterval`) true)
  (`KismetSystemLibrary.K2_SetTimerDelegate` (delegate `DestroyThorns`) (`self.Duration`)))

(event `DestroyThorns`
  (`self.K2_DestroyActor`))

(event `self.DamageCollisionSphere.OnComponentBeginOverlap`
  (params (OverlappedComponent :type "PrimitiveComponent Object Reference") (OtherActor :type "Actor Object Reference") (OtherComp :type "PrimitiveComponent Object Reference") (OtherBodyIndex :type Integer) (bFromSweep :type Boolean) (SweepResult :type "HitResult Structure (by ref)"))
  (if (`self.HasAuthority` OtherActor)
    (message `/Game/Blueprints/Interfaces/BPI_EffectTargetInterface.ETI_OnAddEffect` OtherActor (`self.Effect`))))

(event `self.DamageCollisionSphere.OnComponentEndOverlap`
  (params (OverlappedComponent :type "PrimitiveComponent Object Reference") (OtherActor :type "Actor Object Reference") (OtherComp :type "PrimitiveComponent Object Reference") (OtherBodyIndex :type Integer))
  (if (`self.HasAuthority` OtherActor)
    (for _array_element (`self.Effect`)
      (message `/Game/Blueprints/Interfaces/BPI_EffectTargetInterface.ETI_OnRemoveEffect` OtherActor _array_element))))

(fn `DealDamage`
  (for _array_element (`PrimitiveComponent.GetOverlappingActors` (`self.DamageCollisionSphere`) "/Script/Engine.Character")
    (`GameplayStatics.ApplyDamage` _array_element (`self.BaseDamage`) null self (`self.Damage Type Class`))))

(fn `UserConstructionScript`
  (`parent.UserConstructionScript`)
  (`SphereComponent.SetSphereRadius` (`self.DamageCollisionSphere`) (`self.DamageRadius`) true))