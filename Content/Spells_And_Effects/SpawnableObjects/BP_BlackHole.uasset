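; Spawnable black hole spell object that pulls in and damages characters inside its pull sphere until its duration expires and it destroys itself.
; Each Tick forces movement input toward the center through each overlapping actor's Instigator, optionally scaled by an exponential distance falloff.
; A looping timer applies damage that always uses its own exponential distance falloff.
; Both effects skip the spell owner unless IsSpellOwnerAffected is set.
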(event `self.ReceiveBeginPlay`
  (`parent.ReceiveBeginPlay`)
  (`KismetSystemLibrary.K2_SetTimer` null "DealDamage" (`self.DamageTimeInterval`) true)
  (`KismetSystemLibrary.K2_SetTimerDelegate` (delegate `DestroyBlackHole`) (`self.Duration`)))

(event `DestroyBlackHole`
  (`self.K2_DestroyActor`))

(event `self.ReceiveTick`
  (params (DeltaSeconds :type "Float (single-precision)"))
  (for _array_element (`PrimitiveComponent.GetOverlappingActors` (`self.PullZoneSphere`) "/Script/Engine.Character")
    (if (or (!= _array_element (`self.SpellOwner`)) (`self.IsSpellOwnerAffected`))
      (`self.PullTowardsCenter` _array_element))))

(fn `DealDamage`
  (for _array_element (`PrimitiveComponent.GetOverlappingActors` (`self.PullZoneSphere`) "/Script/Engine.Character")
    (if (or (!= _array_element (`self.SpellOwner`)) (`self.IsSpellOwnerAffected`))
      (`GameplayStatics.ApplyDamage` _array_element (* (`self.BaseDamage`) (`KismetMathLibrary.MultiplyMultiply_FloatFloat` (- 1.0 (`KismetMathLibrary.FClamp` (/ (`KismetMathLibrary.Vector_Distance` (`self.K2_GetActorLocation` _array_element) (`SceneComponent.K2_GetComponentLocation` (`self.PullZoneSphere`))) (`self.PullZoneRadius`)))) (`self.ExponentForDamage`))) null self (`self.Damage Type Class`)))))

(fn `PullTowardsCenter`
  (params (OverlappingActor :type "Actor Object Reference"))
  (locals (TempPullStrenght :type "Vector Structure"))
  (bind _returnvalue (`self.K2_GetActorLocation` OverlappingActor))
  (bind _returnvalue_2 (`SceneComponent.K2_GetComponentLocation` (`self.PullZoneSphere`)))
  (bind _returnvalue_3 (* (`KismetMathLibrary.GetDirectionUnitVector` _returnvalue _returnvalue_2) (`self.PullStrenght`)))
  (set `local.TempPullStrenght` _returnvalue_3)
  (if (not (not (`self.IsPullStrenghtExponential`)))
    (set `local.TempPullStrenght` (* _returnvalue_3 (`KismetMathLibrary.MultiplyMultiply_FloatFloat` (- 1.0 (`KismetMathLibrary.FClamp` (/ (`KismetMathLibrary.Vector_Distance` _returnvalue _returnvalue_2) (`self.PullZoneRadius`)))) (`self.ExponentForPullStrenght`)))))
  (`Pawn.AddMovementInput` (`Actor.Instigator` OverlappingActor) (`local.TempPullStrenght`) 1.0 true))

(fn `UserConstructionScript`
  (`parent.UserConstructionScript`)
  (`SphereComponent.SetSphereRadius` (`self.PullZoneSphere`) (`self.PullZoneRadius`) true))