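; A 3D book actor that serves as a menu, showing the main menu on one of its pages.
; The render target of WCMainMenu feeds a dynamic page material, created in the construction script and recreated every Tick.
; OpenFrontCover uses a timeline to swing the front cover 75 degrees in yaw, then a second to turn the book root 90 degrees.
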(event `self.ReceiveTick`
  (params (DeltaSeconds :type "Float (single-precision)"))
  (bind _returnvalue (`KismetMaterialLibrary.CreateDynamicMaterialInstance` "/Game/Mechanics/MenuBook/M_BookPage_Base.M_BookPage_Base"))
  (bind _output_get (set `self.PageMainMenuMat` _returnvalue))
  (`MaterialInstanceDynamic.SetTextureParameterValue` _output_get "PageTexture" (`WidgetComponent.GetRenderTarget` (`self.WC_MainMenu`)))
  (`PrimitiveComponent.SetMaterial` (`self.Mesh_PageMainMenu`) 0 (`self.PageMainMenuMat`)))

(event `OpenFrontCover`
  (bind _output_get (set `self.CurrentRotation` (`SceneComponent.RelativeRotation` (`self.Mesh_CoverFront`))))
  (set `self.TargetRotation` (`KismetMathLibrary.ComposeRotators` _output_get (`KismetMathLibrary.MakeRotator` 0.0 0.0 75.0)))
  (bind (_direction _alpha) (`Timeline|TimelineFrontCover` :!via `PlayFromStart`)
    (:`Update`
      (`SceneComponent.K2_SetRelativeRotation` (`self.Mesh_CoverFront`) (`KismetMathLibrary.RLerp` (`self.CurrentRotation`) (`self.TargetRotation`) _alpha) false false))
    (:`Finished`
      (bind _output_get_2 (set `self.CurrentRotation` (`SceneComponent.RelativeRotation` (`self.Mesh_BookRoot`))))
      (set `self.TargetRotation` (`KismetMathLibrary.ComposeRotators` _output_get_2 (`KismetMathLibrary.MakeRotator` 0.0 0.0 90.0)))
      (bind (_direction_2 _alpha_2) (`Timeline|Timeline` :!via `PlayFromStart`)
        (:`Update`
          (`SceneComponent.K2_SetRelativeRotation` (`self.Mesh_BookRoot`) (`KismetMathLibrary.RLerp` (`self.CurrentRotation`) (`self.TargetRotation`) _alpha_2) false false))))))

(fn `UserConstructionScript`
  (bind _returnvalue (`KismetMaterialLibrary.CreateDynamicMaterialInstance` "/Game/Mechanics/MenuBook/M_BookPage_Base.M_BookPage_Base"))
  (bind _output_get (set `self.PageMainMenuMat` _returnvalue))
  (`MaterialInstanceDynamic.SetTextureParameterValue` _output_get "PageTexture" (`WidgetComponent.GetRenderTarget` (`self.WC_MainMenu`)))
  (`PrimitiveComponent.SetMaterial` (`self.Mesh_PageMainMenu`) 0 (`self.PageMainMenuMat`)))