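; Base actor for instant raycast spells, which resolves a single trace on spawn instead of persisting in the world.
; After the parent BeginPlay, it line-traces from BoxCollision along its forward vector up to MaxDistance on a specific trace channel.
; The result goes to OnRaycastHit, or the endpoint goes to OnNoRaycastHit on a miss; both are empty hooks for child spells.
; The actor destroys itself immediately afterward.
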(event `self.ReceiveBeginPlay`
  (bind _boxcollision (`self.BoxCollision`))
  (bind _returnvalue (`SceneComponent.K2_GetComponentLocation` _boxcollision))
  (bind _returnvalue_2 (+ _returnvalue (* (`KismetMathLibrary.GetForwardVector` (`SceneComponent.K2_GetComponentRotation` _boxcollision)) (`self.MaxDistance`))))
  (`parent.ReceiveBeginPlay`)
  (bind (_outhit _returnvalue_3) (`KismetSystemLibrary.LineTraceSingle` _returnvalue _returnvalue_2 (enumliteral `ETraceTypeQuery` "TraceTypeQuery3")))
  (if _returnvalue_3
    (`self.OnRaycastHit` _outhit)
    (else
      (`self.OnNoRaycastHit` _returnvalue_2)))
  (`self.K2_DestroyActor`))

(fn `OnNoRaycastHit`
  (params (RaycastEndpoint :type "Vector Structure")))

(fn `OnRaycastHit`
  (params (HitResult :type "HitResult Structure")))

(fn `UserConstructionScript`
  (`parent.UserConstructionScript`))