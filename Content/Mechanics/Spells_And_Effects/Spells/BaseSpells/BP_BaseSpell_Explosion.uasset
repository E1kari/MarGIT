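; Base explosion spell that hits everything inside a spherical radius once on spawn, then destroys itself.
; The sphere is sized from ExplosionRadius in the construction script and on BeginPlay, which then queries overlapping actors directly.
; Each actor except SpellOwner is passed to OnExplosion, an empty hook here, before OnExplosionEnd destroys the spell.
; A debug hitbox event toggles the sphere's in-game visibility.
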(event `self.ReceiveBeginPlay`
  (`parent.ReceiveBeginPlay`)
  (`SphereComponent.SetSphereRadius` (`self.ExplosionRadiusSphere`) (`self.ExplosionRadius`) true)
  (`self.OnBeginOverlap`))

(event `/Game/Mechanics/Interfaces/BPI_DebugGizmos.DG_ShowHitbox`
  (`parent.DG_ShowHitbox`)
  (if (`self.ShowHitbox?`)
    (`SceneComponent.SetHiddenInGame` (`self.ExplosionRadiusSphere`) false false)
    (else
      (`SceneComponent.SetHiddenInGame` (`self.ExplosionRadiusSphere`) true false))))

(fn `OnBeginOverlap`
  (for _array_element (`PrimitiveComponent.GetOverlappingActors` (`self.ExplosionRadiusSphere`) null)
    (if (!= _array_element (`self.SpellOwner`))
      (`self.OnExplosion` _array_element)))
  (`self.OnExplosionEnd`))

(fn `OnExplosion`
  (params (OverlappingActor :type "Actor Object Reference")))

(fn `OnExplosionEnd`
  (`self.K2_DestroyActor`))

(fn `UserConstructionScript`
  (`parent.UserConstructionScript`)
  (`SphereComponent.SetSphereRadius` (`self.ExplosionRadiusSphere`) (`self.ExplosionRadius`) true))