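; Base spell Blueprint that spawns a configurable object in front of itself when it begins play.
; GetSpawnTransform offsets the spell actor's location along its forward vector by SpawningDistance, keeping its rotation and scale.
; BeginPlay passes that transform to a server RPC, which spawns SpawnedObject with SpellOwner as instigator and forwards the ShowHitbox setting.
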(event `self.ReceiveBeginPlay`
  (`parent.ReceiveBeginPlay`)
  (bind _transform (`self.GetSpawnTransform`))
  (`self.RPC_Server_SpawnObject` _transform))

(event `RPC_Server_SpawnObject`
  (params (Transform :type "Transform Structure"))
  (`|SpawnActorFromClass` (`self.SpawnedObject`) Transform "Undefined" "MultiplyWithRoot" null (`self.ShowHitbox?`) (`self.SpellOwner`)))

(fn `GetSpawnTransform`
  (returns (Transform :type "Transform Structure"))
  (bind (_returnvalue_location _returnvalue_rotation _returnvalue_scale) (`KismetMathLibrary.BreakTransform` (`self.GetTransform`)))
  (return (`KismetMathLibrary.MakeTransform` (+ (* (`self.GetActorForwardVector`) (`self.SpawningDistance`)) _returnvalue_location) _returnvalue_rotation _returnvalue_scale)))

(fn `UserConstructionScript`
  (`parent.UserConstructionScript`))