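; Push spell actor, a child spell Blueprint that sets up a forward box area and plays a creation sound.
; The construction script sizes the box from BoxScale and offsets the Arrow backward; BeginPlay moves the box forward by its X extent.
; Knockback of overlapping actors away from SpellOwner, self-destruction and a line-of-sight trace exist only as disconnected nodes, so this graph applies no push itself.
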(event `self.ReceiveBeginPlay`
  (bind _boxcollision (`self.BoxCollision`))
  (bind _boxscale_x (`KismetMathLibrary.BreakVector` (`self.BoxScale`)))
  (`parent.ReceiveBeginPlay`)
  (`SceneComponent.K2_SetWorldLocation` _boxcollision (+ (`SceneComponent.K2_GetComponentLocation` _boxcollision) (* (`SceneComponent.GetForwardVector` _boxcollision) _boxscale_x)) false true)
  (`AudioManagerSubsystem.PlaySFXAtLocation` (subsystem `AudioManagerSubsystem`) (`self.CreationSFX`) (`self.K2_GetActorLocation`) null true 1.0))

(fn `UserConstructionScript`
  (bind _boxscale (`self.BoxScale`))
  (`parent.UserConstructionScript`)
  (`BoxComponent.SetBoxExtent` (`self.BoxCollision`) _boxscale true)
  (`SceneComponent.K2_AddLocalOffset` (`self.Arrow`) (`KismetMathLibrary.MakeVector` (* (.x _boxscale) -1.0)) false false))