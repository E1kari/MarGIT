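; Experimental wall spell that places a player-oriented wall where its aim raycast ends without a hit; direct hits do nothing.
; A downward trace finds the height at the endpoint, then box traces check space for a central piece and one to its right.
; If both are clear, it spawns one BP_PartialWall and passes it both transforms as wall instances.
; All traces draw persistent debug shapes.
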(fn `CheckForHeight`
  (params (`LineTrace Location` :type "Vector Structure"))
  (returns (`Ground Location ` :type "Vector Structure"))
  (bind (_half_size_x _half_size_y _half_size_z) (`KismetMathLibrary.BreakVector` (`self.Half Size`)))
  (bind _outhit (`KismetSystemLibrary.LineTraceSingle` :`Start` `LineTrace Location` :`End` (`KismetMathLibrary.MakeVector` (.x `LineTrace Location`) (.y `LineTrace Location`) (* (+ _half_size_z 50.0) -1.0)) :`TraceChannel` "TraceTypeQuery1" :`DrawDebugType` "Persistent"))
  (return (`.Location` (`GameplayStatics.BreakHitResult` _outhit))))

(fn `CheckForSpace`
  (params (CheckLocation :type "Vector Structure"))
  (bind (_half_size_x _half_size_y _half_size_z) (`KismetMathLibrary.BreakVector` (`self.Half Size`)))
  (bind (_centralpieceloaction_x _centralpieceloaction_y _centralpieceloaction_z) (`KismetMathLibrary.BreakVector` (`self.CentralPieceLoaction`)))
  (bind (_half_size_x_2 _half_size_y_2 _half_size_z_2) (`KismetMathLibrary.BreakVector` (`self.Half Size`)))
  (bind (_half_size_x_3 _half_size_y_3 _half_size_z_3) (`KismetMathLibrary.BreakVector` (`self.Half Size`)))
  (bind (_half_size_x_4 _half_size_y_4 _half_size_z_4) (`KismetMathLibrary.BreakVector` (`self.Half Size`)))
  (bind _allrightpiecelocations (`self.AllRightPieceLocations`))
  (bind _returnvalue (`KismetMathLibrary.MakeVector` (.x CheckLocation) (.y CheckLocation) (+ (.z CheckLocation) _half_size_z_2)))
  (bind (_outhit _returnvalue_2) (`KismetSystemLibrary.BoxTraceSingle` :`Start` _returnvalue :`End` _returnvalue :`HalfSize` (`KismetMathLibrary.MakeVector` _half_size_x_4 _half_size_y_4 (/ _half_size_z_4 2.0)) :`Orientation` (`KismetMathLibrary.ComposeRotators` (`self.K2_GetActorRotation` (`GameplayStatics.GetPlayerCharacter` 0)) (struct :`Yaw` 90.0)) :`TraceChannel` "TraceTypeQuery1" :`DrawDebugType` "Persistent"))
  (if (not _returnvalue_2)
    (bind _output_get (set `self.CentralPieceLoaction` CheckLocation))
    (`KismetArrayLibrary.Array_Add` (`self.AllRightPieceLocations`) (`self.CentralPieceLoaction`))
    (bind _returnvalue_3 (+ (`KismetMathLibrary.MakeVector` (.x _output_get) (.y _output_get) _half_size_z_3) (* (`self.GetActorRightVector` (`GameplayStatics.GetPlayerCharacter` 0)) (* _half_size_x_3 2.0))))
    (bind (_outhit_2 _returnvalue_4) (`KismetSystemLibrary.BoxTraceSingle` :`Start` _returnvalue_3 :`End` _returnvalue_3 :`HalfSize` (`KismetMathLibrary.MakeVector` _half_size_x _half_size_y (/ _half_size_z 2.0)) :`Orientation` (`KismetMathLibrary.ComposeRotators` (`self.K2_GetActorRotation` (`GameplayStatics.GetPlayerCharacter` 0)) (struct :`Yaw` 90.0)) :`TraceChannel` "TraceTypeQuery1" :`DrawDebugType` "Persistent"))
    (if (not _returnvalue_4)
      (`KismetArrayLibrary.Array_Add` _allrightpiecelocations (`KismetMathLibrary.MakeVector` (.x _returnvalue_3) (.y _returnvalue_3) _centralpieceloaction_z))
      (for _array_element _allrightpiecelocations
        (`KismetArrayLibrary.Array_Add` (`self.AllPiecesTransforms`) (`KismetMathLibrary.MakeTransform` _array_element (`self.K2_GetActorRotation` (`GameplayStatics.GetPlayerCharacter` 0)))))
      (bind _returnvalue_5 (`|SpawnActorFromClass` "/Game/Mechanics/Spells_And_Effects/SpawnableObjects/BP_PartialWall.BP_PartialWall_C" (`|GetArrayItem` (`self.AllPiecesTransforms`)) "Undefined" "MultiplyWithRoot" null false null))
      (`/Game/Mechanics/Spells_And_Effects/SpawnableObjects/BP_PartialWall.AddWallInstances` _returnvalue_5 (`self.AllPiecesTransforms`)))))

(fn `OnNoRaycastHit`
  (params (RaycastEndpoint :type "Vector Structure"))
  (bind _ground_location_ (`self.CheckForHeight` RaycastEndpoint))
  (`self.CheckForSpace` _ground_location_))

(fn `OnRaycastHit`
  (params (HitResult :type "HitResult Structure")))

(fn `UserConstructionScript`
  (`parent.UserConstructionScript`))