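; BP_Pending_Spell_GravityReverse is a pending spell for gravity reversal that applies its SpellEffect to actors in an area.
; Construction sizes the Sphere from Radius, and BeginPlay runs the parent logic and prints a debug string.
; On a raycast hit, it moves BoxCollision to the hit location, then sends the effect through an add-effect interface message to every actor overlapping the Sphere.
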(event `self.ReceiveBeginPlay`
  (`parent.ReceiveBeginPlay`)
  (`KismetSystemLibrary.PrintString` "GravityReverse"))

(fn `OnRaycastHit`
  (params (HitResult :type "HitResult Structure"))
  (`SceneComponent.K2_SetWorldLocation` (`self.BoxCollision`) (`.Location` (`GameplayStatics.BreakHitResult` HitResult)) false false)
  (for _array_element (`PrimitiveComponent.GetOverlappingActors` (`self.Sphere`) null)
    (message `/Game/Mechanics/Interfaces/BPI_EffectTargetInterface.ETI_OnAddEffect` _array_element (`self.SpellEffect`))))

(fn `UserConstructionScript`
  (`parent.UserConstructionScript`)
  (`SphereComponent.SetSphereRadius` (`self.Sphere`) (`self.Radius`) true))