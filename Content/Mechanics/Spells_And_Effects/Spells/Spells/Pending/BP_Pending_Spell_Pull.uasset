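; Pending pull spell that, on a raycast hit, draws targets toward the trace origin or launches the caster toward static geometry.
; On authority only, it launches the owner along the trace using PushForce for Static components, while Movable hits get a reversed PullForce.
; Characters are pulled with LaunchCharacter, other movable components with a multiplied impulse.
; BeginPlay prints a debug label, and GetImpulse offsets the collision box location along its forward vector.
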(event `self.ReceiveBeginPlay`
  (`parent.ReceiveBeginPlay`)
  (`KismetSystemLibrary.PrintString` "Pull"))

(fn `GetImpulse`
  (params (Force :type "Float (double-precision)"))
  (returns (Impulse :type "Vector Structure"))
  (bind _boxcollision (`self.BoxCollision`))
  (return (+ (`SceneComponent.K2_GetComponentLocation` _boxcollision) (* (`KismetMathLibrary.GetForwardVector` (`SceneComponent.K2_GetComponentRotation` _boxcollision)) Force))))

(fn `OnRaycastHit`
  (params (HitResult :type "HitResult Structure"))
  (bind (_bblockinghit _binitialoverlap _time _distance _location _impactpoint _normal _impactnormal _physmat _hitactor _hitcomponent _hitbonename _bonename _hititem _elementindex _faceindex _tracestart _traceend) (`GameplayStatics.BreakHitResult` HitResult))
  (bind _mobility (`SceneComponent.Mobility` _hitcomponent))
  (bind _returnvalue (* (* (`self.ImpulseVector`) (`self.PullForce`)) -1.0))
  (if (`self.HasAuthority`)
    (set `self.ImpulseVector` (`KismetMathLibrary.GetDirectionUnitVector` _tracestart _traceend))
    (if (`KismetSystemLibrary.IsValid` _hitcomponent)
      (if (`|EnumEquality` _mobility "Static")
        (`Character.LaunchCharacter` (`self.SpellOwner`) (* (`self.ImpulseVector`) (`self.PushForce`)) false false)
        (elif (`|EnumEquality` _mobility "Movable")
          (bind _ascharacter (cast `Character` _hitactor)
            (:`then`
              (`Character.LaunchCharacter` _ascharacter _returnvalue false false))
            (:`CastFailed`
              (`PrimitiveComponent.AddImpulse` _hitcomponent (* _returnvalue (`self.PullForceObjectMultiply`)) "None" false))))))))

(fn `UserConstructionScript`
  (`parent.UserConstructionScript`))