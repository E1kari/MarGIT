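; BP_Pending_Spell_FrostBolt is a frost bolt spell projectile that damages and applies a spell effect to the actor it hits.
; It runs its parent's construction script and supplies its own collision response.
; On collision it applies damage, prints the hit actor's name, passes SpellEffect to that actor through an add-effect message, then destroys itself.
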(fn `OnProjectileCollision`
  (params (OtherActor :type "Actor Object Reference") (Hit :type "HitResult Structure"))
  (`GameplayStatics.ApplyDamage` OtherActor (`self.DamageAmount`) null self (`self.DamageType`))
  (`KismetSystemLibrary.PrintString` (`KismetSystemLibrary.GetDisplayName` OtherActor))
  (message `/Game/Mechanics/Interfaces/BPI_EffectTargetInterface.ETI_OnAddEffect` OtherActor (`self.SpellEffect`))
  (`self.K2_DestroyActor`))

(fn `UserConstructionScript`
  (`parent.UserConstructionScript`))