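; Legacy wall spell that places an object on the surface in front of the caster when it begins play.
; On the authority, it offsets from the spell owner's capsule along its forward vector by the spawning distance and runs a vertical Visibility line trace there.
; A blocking hit triggers the server spawn RPC at the impact location, using the capsule's rotation; without a hit, nothing spawns.
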(event `self.ReceiveBeginPlay`
  (bind _capsulecomponent (`Character.CapsuleComponent` (`self.SpellOwner`)))
  (bind _returnvalue (`SceneComponent.K2_GetComponentRotation` _capsulecomponent))
  (bind _returnvalue_2 (+ (`SceneComponent.K2_GetComponentLocation` _capsulecomponent) (* (`KismetMathLibrary.GetForwardVector` _returnvalue) (`self.SpawningDistance`))))
  (if (`self.HasAuthority`)
    (bind _outhit (`KismetSystemLibrary.LineTraceSingle` (+ _returnvalue_2 (0.0 0.0 200.0)) (- _returnvalue_2 (0.0 0.0 200.0)) "TraceTypeQuery1"))
    (bind (_bblockinghit _binitialoverlap _time _distance _location) (`GameplayStatics.BreakHitResult` _outhit))
    (if _bblockinghit
      (`self.RPC_Server_SpawnObject` (`KismetMathLibrary.MakeTransform` _location _returnvalue)))))

(fn `UserConstructionScript`
  (`parent.UserConstructionScript`))