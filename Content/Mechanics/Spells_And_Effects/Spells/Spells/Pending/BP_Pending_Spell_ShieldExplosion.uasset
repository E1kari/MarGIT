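; BP_Pending_Spell_ShieldExplosion is a pending spell that defines what a shield explosion does to an actor it overlaps.
; OnExplosion applies damage with the spell as causer, then sends a knockback interface message to that actor.
; The knockback points away from the spell owner's location rather than the spell's own, scaled by an impulse strength.
; The construction script only calls its parent.
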(fn `OnExplosion`
  (params (OverlappingActor :type "Actor Object Reference"))
  (`GameplayStatics.ApplyDamage` OverlappingActor (`self.DamageAmount`) null self (`self.Damage Type Class`))
  (message `/Game/Mechanics/Interfaces/BPI_EffectTargetInterface.ETI_OnKnockback` OverlappingActor (* (`KismetMathLibrary.GetDirectionUnitVector` (`self.K2_GetActorLocation` (`self.SpellOwner`)) (`self.K2_GetActorLocation` OverlappingActor)) (`self.ImpluseStrenght`))))

(fn `UserConstructionScript`
  (`parent.UserConstructionScript`))