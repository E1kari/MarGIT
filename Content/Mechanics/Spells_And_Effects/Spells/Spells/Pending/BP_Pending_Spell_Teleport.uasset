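; Pending teleport spell that moves its owner to the point hit by a raycast.
; The construction script runs the parent's, then on authority sets a very large MaxDistance fallback when HasMaxDistance is false.
; OnRaycastHit teleports SpellOwner to the hit location on authority only, keeping the owner's current rotation.
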(fn `OnRaycastHit`
  (params (HitResult :type "HitResult Structure"))
  (bind _spellowner (`self.SpellOwner`))
  (if (`self.HasAuthority`)
    (`self.K2_TeleportTo` _spellowner (`.Location` (`GameplayStatics.BreakHitResult` HitResult)) (`self.K2_GetActorRotation` _spellowner))))

(fn `UserConstructionScript`
  (`parent.UserConstructionScript`)
  (if (`self.HasAuthority`)
    (if (not (`self.HasMaxDistance`))
      (set `self.MaxDistance` 9999.0))))