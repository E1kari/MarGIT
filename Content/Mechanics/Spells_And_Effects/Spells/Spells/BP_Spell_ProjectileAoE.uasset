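; Area-of-effect projectile spell that explodes on collision or on reaching max distance, dealing full radial damage credited to the spell owner's controller.
; On impact it stops movement, swaps the travel effect for explosion FX, plays a destroy sound, spawns a BP_MasterField and destroys itself after a short timer.
; A bool limits the max-distance trigger to one firing, and construction sizes a debug sphere to the damage radius.
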(fn `DestroyActor`
  (`self.K2_DestroyActor`))

(fn `OnMaxDistanceReached`
  (if (not (`self.OnMaxDistanceReachedBool`))
    (set `self.OnMaxDistanceReachedBool` true)
    (`self.OnProjectileCollision` null)))

(fn `OnProjectileCollision`
  (params (OtherActor :type "Actor Object Reference") (Hit :type "HitResult Structure"))
  (`MovementComponent.StopMovementImmediately` (`self.SpellMovement`))
  (`GameplayStatics.ApplyRadialDamage` :`BaseDamage` (`self.DamageAmount`) :`Origin` (`SceneComponent.K2_GetComponentLocation` (`self.BoxCollision`)) :`DamageRadius` (`self.DamageRadius`) :`DamageTypeClass` (`self.Damage Type Class`) :`DamageCauser` self :`InstigatedByController` (`Pawn.GetController` (`self.SpellOwner`)) :`bDoFullDamage` true)
  (`ActorComponent.Activate` (`self.FXExplotion`) false)
  (`SceneComponent.SetVisibility` (`self.FXSystem`) false false)
  (`AudioManagerSubsystem.PlaySFXAtLocation` (subsystem `AudioManagerSubsystem`) (`self.DestroySFX`) (`self.K2_GetActorLocation`) "/Game/Audio/Attenuation/FireballAttenuation.FireballAttenuation" true 1.0 true)
  (`|SpawnActorFromClass` "/Game/Mechanics/Destructables/BP_MasterField.BP_MasterField_C" (`self.GetTransform`) "Undefined" "MultiplyWithRoot" null null)
  (`KismetSystemLibrary.K2_SetTimer` null "DestroyActor" 1.0))

(fn `UserConstructionScript`
  (`parent.UserConstructionScript`)
  (`SphereComponent.SetSphereRadius` (`self.DebugSphere`) (`self.DamageRadius`) true))