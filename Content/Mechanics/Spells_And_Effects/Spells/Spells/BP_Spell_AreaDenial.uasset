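; BP_Spell_AreaDenial is a spell that spawns a BP_IceStorm area effect where its raycast hits.
; When the hit normal's Z is below the NormalZ threshold, as on steep surfaces, it pulls the spawn point back by DamageRadius against the caster's forward vector.
; It passes radius, duration, effect and hitbox visibility to the storm, with the caster as instigator.
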(fn `OnRaycastHit`
  (params (HitResult :type "HitResult Structure"))
  (locals (SpawnTransform :type "Transform Structure"))
  (bind (_bblockinghit _binitialoverlap _time _distance _location _impactpoint _normal _impactnormal) (`GameplayStatics.BreakHitResult` HitResult))
  (if (>= (.z _impactnormal) (`self.NormalZ`))
    (set `local.SpawnTransform` (`KismetMathLibrary.Conv_VectorToTransform` _location))
    (else
      (set `local.SpawnTransform` (`KismetMathLibrary.Conv_VectorToTransform` (+ _location (* (`self.GetActorForwardVector` (`self.SpellOwner`)) (`self.Damage Radius`) -1.0))))))
  (`|SpawnActorFromClass` "/Game/Mechanics/Spells_And_Effects/SpawnableObjects/BP_IceStorm.BP_IceStorm_C" (`local.SpawnTransform`) "Undefined" "MultiplyWithRoot" null (`self.Damage Radius`) (`self.Duration`) (`self.SpellEffect`) 0.0 (`self.ShowHitbox?`) (`self.SpellOwner`)))

(fn `UserConstructionScript`
  (`parent.UserConstructionScript`))