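; BP_Spell_BouncyRaycast is a raycast spell that starts a bouncing lightning effect where the ray hits.
; On hit, it spawns a BP_LightningSphere at the impact point, passing it the target, damage, jump settings and the caster's location as the previous sphere position.
; Character hits start the jump count at zero; other hits set it very high, apparently to prevent further bouncing.
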(fn `OnRaycastHit`
  (params (HitResult :type "HitResult Structure"))
  (bind (_bblockinghit _binitialoverlap _time _distance _location _impactpoint _normal _impactnormal _physmat _hitactor) (`GameplayStatics.BreakHitResult` HitResult))
  (bind _ascharacter (cast `Character` _hitactor)
    (:`then`
      (set `self.Main Target` _ascharacter)
      (set `self.Current Jump Cycle` 0))
    (:`CastFailed`
      (set `self.Main Target` _hitactor)
      (set `self.Current Jump Cycle` 9999)))
  (`|SpawnActorFromClass` "/Game/Mechanics/Spells_And_Effects/SpawnableObjects/BP_LightningSphere.BP_LightningSphere_C" (`KismetMathLibrary.Conv_VectorToTransform` _location) "Undefined" "MultiplyWithRoot" null (`self.Sphere Radius`) (`self.Main Target`) (`self.Base Damage`) (`self.Damage Type Class`) (`self.Damage Reduction`) (`self.Jump Timer`) (`self.Current Jump Cycle`) (`self.Max Jump Cycles`) (`self.Jump Chance`) (`self.K2_GetActorLocation` (`self.SpellOwner`)) 0.0 (`self.ShowHitbox?`) (`self.SpellOwner`)))

(fn `UserConstructionScript`
  (`parent.UserConstructionScript`))