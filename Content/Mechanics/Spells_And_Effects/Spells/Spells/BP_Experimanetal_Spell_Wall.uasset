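; Experimental wall spell that spawns a BP_PartialWall where the spell's raycast hits or ends, sized to fit the available space.
; A downward trace finds the base height, then CheckSides runs stacked traces along the player's right vector to measure clearance on each side.
; Blocked sides shorten the wall and shift its center away from the obstacle before it spawns with the player's rotation.
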(fn `CheckForHeight`
  (params (`LineTrace Location` :type "Vector Structure"))
  (returns (`Ground Location ` :type "Vector Structure"))
  (locals (NewLocalVar :type "Vector Structure" :default (0.0 0.0 0.0)))
  (bind _returnvalue (/ (`self.Height`) 2.0))
  (bind _outhit (`KismetSystemLibrary.LineTraceSingle` (+ `LineTrace Location` (`KismetMathLibrary.MakeVector` 0.0 0.0 _returnvalue)) (`KismetMathLibrary.MakeVector` (.x `LineTrace Location`) (.y `LineTrace Location`) (* (+ _returnvalue 50.0) -1.0)) "TraceTypeQuery1" false (`|MakeArray` (`self.SpellOwner`) :!type "Actor Object Reference")))
  (return (`.Location` (`GameplayStatics.BreakHitResult` _outhit))))

(fn `CheckForSpace`
  (params (CheckLocation :type "Vector Structure"))
  (locals (LeftSideLenght :type "Float (double-precision)" :default 0.0) (RightSideLenght :type "Float (double-precision)" :default 0.0))
  (bind _output_get (set `self.SpawnLocation` CheckLocation))
  (set `self.CenterLowestCheckHeight` (`KismetMathLibrary.MakeVector` (.x _output_get) (.y _output_get) (+ (.z _output_get) (/ (`self.Height`) 4.0))))
  (set `self.PlayerActorRightVector` (`self.GetActorRightVector` (`GameplayStatics.GetPlayerCharacter` 0)))
  (bind _distance (`self.CheckSides` true))
  (set `local.LeftSideLenght` _distance)
  (bind _distance_2 (`self.CheckSides` false))
  (set `local.RightSideLenght` _distance_2)
  (`|SpawnActorFromClass` "/Game/Mechanics/Spells_And_Effects/SpawnableObjects/BP_PartialWall.BP_PartialWall_C" (`KismetMathLibrary.MakeTransform` (+ (`self.SpawnLocation`) (0.0 0.0 1.0)) (`self.K2_GetActorRotation` (`GameplayStatics.GetPlayerCharacter` 0))) "Undefined" "MultiplyWithRoot" null (`self.Thiccness`) (+ (`local.LeftSideLenght`) (`local.RightSideLenght`)) (`self.Height`) (`self.WallMaterial`) (`self.MaxHealth`) false (`self.SpellOwner`)))

(fn `CheckSides`
  (params (`LeftSide?` :type Boolean))
  (returns (Distance :type "Float (double-precision)"))
  (locals (ShortestTrace :type "Float (double-precision)") (SideMultiplier :type "Float (double-precision)"))
  (bind _shortesttrace (`local.ShortestTrace`))
  (if `LeftSide?`
    (set `local.SideMultiplier` -1.0)
    (else
      (set `local.SideMultiplier` 1.0)))
  (set `local.ShortestTrace` (`self.MaxSideDistance`))
  (for _index (range (`self.MaxTraceChecksPerSide`))
    (bind _returnvalue (+ (`self.CenterLowestCheckHeight`) (`KismetMathLibrary.MakeVector` 0.0 0.0 (* (/ (/ (`self.Height`) 2.0) (`self.MaxTraceChecksPerSide`)) _index))))
    (bind (_outhit _returnvalue_2) (`KismetSystemLibrary.LineTraceSingle` _returnvalue (+ _returnvalue (* (`self.PlayerActorRightVector`) (`self.MaxSideDistance`) (`local.SideMultiplier`))) "TraceTypeQuery1" false (`|MakeArray` (`self.SpellOwner`))))
    (if _returnvalue_2
      (bind (_bblockinghit _binitialoverlap _time _distance) (`GameplayStatics.BreakHitResult` _outhit))
      (if (< _distance (`local.ShortestTrace`))
        (set `local.ShortestTrace` _distance))))
  (if (< _shortesttrace (`self.MaxSideDistance`))
    (set `self.SpawnLocation` (+ (`self.SpawnLocation`) (* (`self.PlayerActorRightVector`) (/ (- (`self.MaxSideDistance`) _shortesttrace) 2.0) (* (`local.SideMultiplier`) -1.0)))))
  (return (`local.ShortestTrace`)))

(fn `OnNoRaycastHit`
  (params (RaycastEndpoint :type "Vector Structure"))
  (bind _ground_location_ (`self.CheckForHeight` RaycastEndpoint))
  (`self.CheckForSpace` _ground_location_))

(fn `OnRaycastHit`
  (params (HitResult :type "HitResult Structure"))
  (bind _ground_location_ (`self.CheckForHeight` (`.Location` (`GameplayStatics.BreakHitResult` HitResult))))
  (`self.CheckForSpace` _ground_location_))

(fn `UserConstructionScript`
  (`parent.UserConstructionScript`))