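; Raycast-based spell that spawns a BP_BlackHole at the targeted point, despite its PullProjectile name.
; Both the hit and no-hit raycast callbacks call a server RPC, passing the impact location or the ray's endpoint.
; The RPC passes the spell's pull, damage, radius, timing and owner settings to the black hole, feeding ExponentForDamage into its pull-strength exponent.
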(event `RPC_Server_SpawnBlackHole`
  (params (Position :type "Vector Structure"))
  (bind _spellowner (`self.SpellOwner`))
  (`|SpawnActorFromClass` "/Game/Mechanics/Spells_And_Effects/SpawnableObjects/BP_BlackHole.BP_BlackHole_C" (`KismetMathLibrary.Conv_VectorToTransform` Position) "Undefined" "MultiplyWithRoot" null (`self.Pull Strenght`) (`self.Base Damage`) (`self.Pull Zone Radius`) (`self.Damage Time Interval`) _spellowner (`self.Is Spell Owner Affected`) (`self.Damage Type Class`) (`self.Duration`) (`self.Exponent for Damage`) (`self.Is Damage Exponential`) 0.0 (`self.ShowHitbox?`) _spellowner))

(fn `OnNoRaycastHit`
  (params (RaycastEndpoint :type "Vector Structure"))
  (`self.RPC_Server_SpawnBlackHole` RaycastEndpoint))

(fn `OnRaycastHit`
  (params (HitResult :type "HitResult Structure"))
  (`self.RPC_Server_SpawnBlackHole` (`.Location` (`GameplayStatics.BreakHitResult` HitResult))))

(fn `UserConstructionScript`
  (`parent.UserConstructionScript`))