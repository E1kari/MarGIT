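; Black hole spell object that pulls and damages characters inside a sphere zone, then destroys itself after a set duration.
; Tick pulls overlapping characters inward with forced movement input, while a looping timer applies damage.
; Both effects can scale by an exponential distance falloff and optionally affect the caster.
; Shortly after spawn, enemies in the zone with an AIC_Enemy_02 controller are set to flee from it.
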(event `self.ReceiveBeginPlay`
  (`parent.ReceiveBeginPlay`)
  (`KismetSystemLibrary.K2_SetTimer` null "DealDamage" (`self.DamageTimeInterval`) true)
  (`KismetSystemLibrary.K2_SetTimerDelegate` (delegate `DestroyBlackHole`) (`self.Duration`))
  (`KismetSystemLibrary.Delay` 0.2)
  (for _array_element (`PrimitiveComponent.GetOverlappingActors` (`self.PullZoneSphere`) "/Script/Engine.Character")
    (if (`GameplayStatics.ObjectIsA` _array_element "/Game/Mechanics/Enemy/Blueprints/BP_Enemy_Base.BP_Enemy_Base_C")
      (bind _asaic_enemy_02 (cast `/Game/Mechanics/Enemy/AI/AIC_Enemy_02` (`AIBlueprintHelperLibrary.GetAIController` _array_element)))
      (`/Game/Mechanics/Enemy/AI/AIC_Enemy_02.SetStateAsFleeing` _asaic_enemy_02 self))))

(event `DestroyBlackHole`
  (`self.K2_DestroyActor`))

(event `self.ReceiveTick`
  (params (DeltaSeconds :type "Float (single-precision)"))
  (for _array_element (`PrimitiveComponent.GetOverlappingActors` (`self.PullZoneSphere`) "/Script/Engine.Character")
    (if (or (!= _array_element (`self.SpellOwner`)) (`self.IsSpellOwnerAffected`))
      (`self.PullTowardsCenter` _array_element))))

(event `/Game/Mechanics/Interfaces/BPI_DebugGizmos.DG_ShowHitbox`
  (`parent.DG_ShowHitbox`)
  (if (`self.ShowHitbox?`)
    (`SceneComponent.SetHiddenInGame` (`self.PullZoneSphere`) false false)
    (else
      (`SceneComponent.SetHiddenInGame` (`self.PullZoneSphere`) true false))))

(event `self.Sphere.OnComponentBeginOverlap`
  (params (OverlappedComponent :type "PrimitiveComponent Object Reference") (OtherActor :type "Actor Object Reference") (OtherComp :type "PrimitiveComponent Object Reference") (OtherBodyIndex :type Integer) (bFromSweep :type Boolean) (SweepResult :type "HitResult Structure (by ref)"))
  (if (`GameplayStatics.ObjectIsA` OtherActor "/Script/Engine.Character")
    _))

(fn `DealDamage`
  (for _array_element (`PrimitiveComponent.GetOverlappingActors` (`self.PullZoneSphere`) "/Script/Engine.Character")
    (if (or (!= _array_element (`self.SpellOwner`)) (`self.IsSpellOwnerAffected`))
      (if (not (not (`self.IsDamageExponential`)))
        (set `self.BaseDamage` (* (`self.BaseDamage`) (`KismetMathLibrary.MultiplyMultiply_FloatFloat` (- 1.0 (`KismetMathLibrary.FClamp` (/ (`KismetMathLibrary.Vector_Distance` (`self.K2_GetActorLocation` _array_element) (`SceneComponent.K2_GetComponentLocation` (`self.PullZoneSphere`))) (`self.PullZoneRadius`)))) (`self.ExponentForDamage`)))))
      (`GameplayStatics.ApplyDamage` _array_element (`self.BaseDamage`) (`self.GetInstigatorController`) self (`self.Damage Type Class`)))))

(fn `PullTowardsCenter`
  (params (OverlappingActor :type "Actor Object Reference"))
  (locals (TempPullStrenght :type "Vector Structure"))
  (bind _returnvalue (`SceneComponent.K2_GetComponentLocation` (`self.PullZoneSphere`)))
  (bind _ascharacter (cast `Character` OverlappingActor))
  (bind _returnvalue_2 (`self.K2_GetActorLocation` _ascharacter))
  (bind _returnvalue_3 (* (`KismetMathLibrary.GetDirectionUnitVector` _returnvalue_2 _returnvalue) (`self.PullStrenght`)))
  (set `local.TempPullStrenght` _returnvalue_3)
  (if (not (not (`self.IsPullStrenghtExponential`)))
    (set `local.TempPullStrenght` (* _returnvalue_3 (`KismetMathLibrary.MultiplyMultiply_FloatFloat` (- 1.0 (`KismetMathLibrary.FClamp` (/ (`KismetMathLibrary.Vector_Distance` _returnvalue_2 _returnvalue) (`self.PullZoneRadius`)))) (`self.ExponentForPullStrenght`)))))
  (`Pawn.AddMovementInput` _ascharacter (`local.TempPullStrenght`) 1.0 true))

(fn `UserConstructionScript`
  (`parent.UserConstructionScript`)
  (`SphereComponent.SetSphereRadius` (`self.PullZoneSphere`) (`self.PullZoneRadius`) true)
  (if (`self.ShowHitbox?`)
    (`SceneComponent.SetHiddenInGame` (`self.PullZoneSphere`) false false)))