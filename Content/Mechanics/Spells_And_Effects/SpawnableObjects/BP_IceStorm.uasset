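; Spawnable ice storm spell area that applies its configured effects to actors inside a damage sphere sized by DamageRadius, then destroys itself after Duration.
; On the authority, effects are sent through ETI interface messages on overlap begin and removed on overlap end.
; A one-second looping timer also re-applies them to every overlapping actor.
; A debug toggle shows or hides the hitbox.
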(event `self.ReceiveBeginPlay`
  (bind _returnvalue (`KismetSystemLibrary.K2_SetTimer` null "TryApplyEffects" 1.0 true))
  (`KismetSystemLibrary.K2_SetTimerDelegate` (delegate `DestroyIceStorm`) (`self.Duration`)))

(event `DestroyIceStorm`
  (`KismetSystemLibrary.K2_PauseTimerHandle` (stale `self.ReceiveBeginPlay` _returnvalue))
  (`self.K2_DestroyActor`))

(event `self.DamageCollision.OnComponentBeginOverlap`
  (params (OverlappedComponent :type "PrimitiveComponent Object Reference") (OtherActor :type "Actor Object Reference") (OtherComp :type "PrimitiveComponent Object Reference") (OtherBodyIndex :type Integer) (bFromSweep :type Boolean) (SweepResult :type "HitResult Structure (by ref)"))
  (if (`self.HasAuthority`)
    (message `/Game/Mechanics/Interfaces/BPI_EffectTargetInterface.ETI_OnAddEffect` OtherActor (`self.Effect`))))

(event `self.DamageCollision.OnComponentEndOverlap`
  (params (OverlappedComponent :type "PrimitiveComponent Object Reference") (OtherActor :type "Actor Object Reference") (OtherComp :type "PrimitiveComponent Object Reference") (OtherBodyIndex :type Integer))
  (if (`self.HasAuthority`)
    (for _array_element (`self.Effect`)
      (message `/Game/Mechanics/Interfaces/BPI_EffectTargetInterface.ETI_OnRemoveEffect` OtherActor _array_element))))

(event `/Game/Mechanics/Interfaces/BPI_DebugGizmos.DG_ShowHitbox`
  (`parent.DG_ShowHitbox`)
  (if (`self.ShowHitbox?`)
    (`SceneComponent.SetHiddenInGame` (`self.DamageCollision`) false false)
    (else
      (`SceneComponent.SetHiddenInGame` (`self.DamageCollision`) true false))))

(fn `TryApplyEffects`
  (if (`self.HasAuthority`)
    (for _array_element (`PrimitiveComponent.GetOverlappingActors` (`self.DamageCollision`) "/Script/Engine.Actor")
      (message `/Game/Mechanics/Interfaces/BPI_EffectTargetInterface.ETI_OnAddEffect` _array_element (`self.Effect`)))))

(fn `UserConstructionScript`
  (`parent.UserConstructionScript`)
  (`SphereComponent.SetSphereRadius` (`self.DamageCollision`) (`self.DamageRadius`) true)
  (if (`self.ShowHitbox?`)
    (`SceneComponent.SetHiddenInGame` (`self.DamageCollision`) false false)))