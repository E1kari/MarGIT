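; BP_OLD_Wall is a spawnable spell-system wall that takes damage and is destroyed outright when damaged by a pull projectile.
; Effect damage routes through ApplyDamage into AnyDamage, which calls OnTakeDamage and drives both a health gizmo widget and a dynamic material "crack range" parameter from the health ratio.
; Effect-target getters report zero gravity and speed.
; Gizmo visibility initially copies an enemy's debug gizmo and toggles on the enemy-status debug event.
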(event `self.ReceiveBeginPlay`
  (bind _widget (`self.Widget`))
  (bind _mesh (`self.Mesh`))
  ; For Debug Gizmo
  (bind _returnvalue (`GameplayStatics.GetActorOfClass` "/Game/Mechanics/Enemy/Blueprints/BP_Enemy_Base.BP_Enemy_Base_C"))
  (`/Engine/EditorBlueprintResources/StandardMacros.IsValid` _returnvalue
    (:`Is Valid`
      (`SceneComponent.SetVisibility` _widget (`SceneComponent.bVisible` (`/Game/Mechanics/Enemy/Blueprints/BP_Enemy_Base.DebugGizmo` _returnvalue)) false))
    (:`Is Not Valid`
      _))
  (bind _aswb_wall_gizmo (cast `/Game/Mechanics/Enemy/Gizmos/WB_WallGizmo` (`WidgetComponent.GetWidget` _widget)))
  (set `self.GizmoRef` _aswb_wall_gizmo)
  (bind _returnvalue_2 (`PrimitiveComponent.CreateDynamicMaterialInstance` (`self.Mesh`) 0 (`PrimitiveComponent.GetMaterial` _mesh 0) "None"))
  (bind _output_get (set `self.MatInst` _returnvalue_2))
  (`PrimitiveComponent.SetMaterial` _mesh 0 _output_get)
  (`MaterialInstanceDynamic.SetScalarParameterValue` (`self.MatInst`) "crack range" 1.0))

(event `/Game/Mechanics/Interfaces/BPI_EffectTargetInterface.ETI_OnTakeEffectDamage`
  (params (`Damage Amount` :type "Float (double-precision)") (DamageCauser :type "Actor Object Reference") (DamageType :type "DamageType Class Reference"))
  (`GameplayStatics.ApplyDamage` self `Damage Amount` null DamageCauser DamageType))

(event `self.ReceiveAnyDamage`
  (params (Damage :type "Float (single-precision)") (DamageType :type "DamageType Object Reference") (InstigatedBy :type "Controller Object Reference") (DamageCauser :type "Actor Object Reference"))
  (bind _matinst (`self.MatInst`))
  (bind _returnvalue (/ (`self.CurrentHealth`) (`self.MaxHealth`)))
  (if (`GameplayStatics.ObjectIsA` DamageCauser "/Game/Mechanics/Spells_And_Effects/Spells/Spells/Pending/BP_Pending_Spell_PullProjectile.BP_Pending_Spell_PullProjectile_C")
    (`self.K2_DestroyActor`)
    (else
      (`self.OnTakeDamage` Damage DamageType)
      (bind _gizmoref (`self.GizmoRef`)
        (:`then`
          (`/Game/Mechanics/Enemy/Gizmos/WB_WallGizmo.SetHealthPercent` _gizmoref _returnvalue)
          (`MaterialInstanceDynamic.SetScalarParameterValue` _matinst "crack range" _returnvalue)
          (bind _returnvalue_2 (`MaterialInstanceDynamic.K2_GetScalarParameterValue` _matinst "crack range"))
          (`KismetSystemLibrary.PrintString` (`KismetStringLibrary.Conv_DoubleToString` _returnvalue_2)))
        (:`else`)))))

(event `/Game/Mechanics/Interfaces/BPI_DebugGizmos.DG_ShowHitbox`
  (`parent.DG_ShowHitbox`)
  (if (`self.ShowHitbox?`)
    _))

(event `/Game/Mechanics/Interfaces/BPI_DebugGizmos.DG_ShowEnemyStatus`
  (bind _widget (`self.Widget`))
  (`SceneComponent.SetVisibility` _widget (not (`SceneComponent.bVisible` _widget)) false))

(fn `ETI_GetGravityScale`
  (returns (GravityScale :type "Float (double-precision)"))
  (return 0.0))

(fn `ETI_GetMovementSpeed`
  (returns (MovementSpeed :type "Float (double-precision)"))
  (return 0.0))

(fn `ETI_GetPlayerController`
  (returns (PlayerController :type "PlayerController Object Reference"))
  (return null))

(fn `UserConstructionScript`
  (`parent.UserConstructionScript`)
  (`SceneComponent.SetWorldScale3D` (`self.Mesh`) (`self.Scale`))
  (if (`self.ShowHitbox?`)
    _))