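; BP_Thorns is a timed spawnable thorn area that applies effects to actors inside its collision sphere, destroying itself after Duration.
; Overlapping actors with authority receive the Effect array through an add-effect message, then a remove message per element when they leave.
; Construction sizes the sphere from DamageRadius, and ShowHitbox controls its in-game visibility, also through a DGShowHitbox override that extends the parent.
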(event `self.ReceiveBeginPlay`
  (`KismetSystemLibrary.K2_SetTimerDelegate` (delegate `DestroyThorns`) (`self.Duration`)))

(event `DestroyThorns`
  (`self.K2_DestroyActor`))

(event `self.DamageCollisionSphere.OnComponentBeginOverlap`
  (params (OverlappedComponent :type "PrimitiveComponent Object Reference") (OtherActor :type "Actor Object Reference") (OtherComp :type "PrimitiveComponent Object Reference") (OtherBodyIndex :type Integer) (bFromSweep :type Boolean) (SweepResult :type "HitResult Structure (by ref)"))
  (if (`self.HasAuthority` OtherActor)
    (message `/Game/Mechanics/Interfaces/BPI_EffectTargetInterface.ETI_OnAddEffect` OtherActor (`self.Effect`))))

(event `self.DamageCollisionSphere.OnComponentEndOverlap`
  (params (OverlappedComponent :type "PrimitiveComponent Object Reference") (OtherActor :type "Actor Object Reference") (OtherComp :type "PrimitiveComponent Object Reference") (OtherBodyIndex :type Integer))
  (if (`self.HasAuthority` OtherActor)
    (for _array_element (`self.Effect`)
      (message `/Game/Mechanics/Interfaces/BPI_EffectTargetInterface.ETI_OnRemoveEffect` OtherActor _array_element))))

(event `/Game/Mechanics/Interfaces/BPI_DebugGizmos.DG_ShowHitbox`
  (`parent.DG_ShowHitbox`)
  (if (`self.ShowHitbox?`)
    (`SceneComponent.SetHiddenInGame` (`self.DamageCollisionSphere`) false false)
    (else
      (`SceneComponent.SetHiddenInGame` (`self.DamageCollisionSphere`) true false))))

(fn `UserConstructionScript`
  (`parent.UserConstructionScript`)
  (`SphereComponent.SetSphereRadius` (`self.DamageCollisionSphere`) (`self.DamageRadius`) true)
  (if (`self.ShowHitbox?`)
    (`SceneComponent.SetHiddenInGame` (`self.DamageCollisionSphere`) false false)))