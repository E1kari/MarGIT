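; BP_PartialWall is a damageable spell-system wall with a procedural box mesh and collision, built from its dimensions in the construction script.
; Damage updates health and drives a dynamic material's crack parameter and a health gizmo, while black hole damage destroys it outright.
; It accepts effects through an effect manager, turning effect damage into regular damage.
; The gizmo's initial visibility matches an enemy's debug gizmo and can be toggled.
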(event `self.ReceiveBeginPlay`
  (bind _widget (`self.Widget`))
  (`SceneComponent.K2_SetRelativeLocation` _widget (`KismetMathLibrary.MakeVector` 0.0 0.0 (`self.Dimension Z`)) false false)
  (bind _aswb_wall_gizmo (cast `/Game/Mechanics/Enemy/Gizmos/WB_WallGizmo` (`WidgetComponent.GetWidget` _widget))
    (:`then`
      (set `self.GizmoRef` _aswb_wall_gizmo)
      (bind _returnvalue (`GameplayStatics.GetActorOfClass` "/Game/Mechanics/Enemy/Blueprints/BP_Enemy_Base.BP_Enemy_Base_C"))
      (`/Engine/EditorBlueprintResources/StandardMacros.IsValid` _returnvalue
        (:`Is Valid`
          (`SceneComponent.SetVisibility` (`self.Widget`) (`SceneComponent.bVisible` (`/Game/Mechanics/Enemy/Blueprints/BP_Enemy_Base.DebugGizmo` _returnvalue)) false))))
    (:`CastFailed`
      (`KismetSystemLibrary.PrintString` "Cast to Wall Gizmo failed"))))

(event `self.ReceiveAnyDamage`
  (params (Damage :type "Float (single-precision)") (DamageType :type "DamageType Object Reference") (InstigatedBy :type "Controller Object Reference") (DamageCauser :type "Actor Object Reference"))
  (bind _returnvalue (/ (`self.CurrentHealth`) (`self.MaxHealth`)))
  (if (`GameplayStatics.ObjectIsA` DamageCauser "/Game/Mechanics/Spells_And_Effects/SpawnableObjects/BP_BlackHole.BP_BlackHole_C")
    (`self.K2_DestroyActor`)
    (else
      (`self.OnTakeDamage` Damage DamageType)
      (`MaterialInstanceDynamic.SetScalarParameterValue` (`self.MaterialInstanceRef`) "crack range" _returnvalue)
      (bind _gizmoref (`self.GizmoRef`)
        (:`then`
          (`/Game/Mechanics/Enemy/Gizmos/WB_WallGizmo.SetHealthPercent` _gizmoref _returnvalue))
        (:`else`)))))

(event `/Game/Mechanics/Interfaces/BPI_DebugGizmos.DG_ShowEnemyStatus`
  (bind _widget (`self.Widget`))
  (`SceneComponent.SetVisibility` _widget (not (`SceneComponent.bVisible` _widget)) false))

(event `/Game/Mechanics/Interfaces/BPI_EffectTargetInterface.ETI_OnAddEffect`
  (params (Effects :type "Array of /Game/Mechanics/Spells_And_Effects/Effects/BP_Effect_Base Class Reference (by ref)"))
  (`/Game/Mechanics/Components/BPC_EffectManager.EM_AddEffect` (`self.BPC_EffectManager`) Effects self))

(event `/Game/Mechanics/Interfaces/BPI_EffectTargetInterface.ETI_OnRemoveEffect`
  (params (Effect :type "/Game/Mechanics/Spells_And_Effects/Effects/BP_Effect_Base Class Reference"))
  (`/Game/Mechanics/Components/BPC_EffectManager.EM_ExternalRemoveEffect` (`self.BPC_EffectManager`) Effect))

(event `/Game/Mechanics/Interfaces/BPI_EffectTargetInterface.ETI_OnTakeEffectDamage`
  (params (`Damage Amount` :type "Float (double-precision)") (DamageCauser :type "Actor Object Reference") (DamageType :type "DamageType Class Reference"))
  (`GameplayStatics.ApplyDamage` self `Damage Amount` null DamageCauser DamageType))

(fn `ETI_GetGravityScale`
  (returns (GravityScale :type "Float (double-precision)"))
  (return 0.0))

(fn `ETI_GetMovementSpeed`
  (returns (MovementSpeed :type "Float (double-precision)"))
  (return 0.0))

(fn `ETI_GetPlayerController`
  (returns (PlayerController :type "PlayerController Object Reference"))
  (return null))

(fn `UserConstructionScript`
  (bind _dynamicmesh (`self.DynamicMesh`))
  (`parent.UserConstructionScript`)
  (bind _returnvalue (`BaseDynamicMeshComponent.GetDynamicMesh` (`self.DynamicMesh`)))
  (bind (_simplecollision _returnvalue_2) (`GeometryScriptLibrary_MeshPrimitiveFunctions.AppendBoxWithCollision` _returnvalue (struct) (struct) (`self.Dimension X`) (`self.Dimension Y`) (`self.Dimension Z`) 0 0 0 "Base" null))
  (`GeometryScriptLibrary_CollisionFunctions.SetDynamicMeshCollisionFromMesh` _returnvalue_2 (`self.DynamicMesh`) (struct) null)
  (bind _returnvalue_3 (`PrimitiveComponent.CreateDynamicMaterialInstance` _dynamicmesh 0 (`self.Material`) "None"))
  (bind _output_get (set `self.MaterialInstanceRef` _returnvalue_3))
  (`PrimitiveComponent.SetMaterial` _dynamicmesh 0 _output_get)
  (`MaterialInstanceDynamic.SetScalarParameterValue` _output_get "crack range" 1.0))