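; BP_LightningSphere is one link of a chain lightning effect, damaging its main target when spawned.
; It draws a Niagara beam from the previous sphere, then after a timer rolls a chance for each overlapping effect target to spawn another sphere there, and destroys itself.
; Character targets inherit the chain settings, with cycle-limited jumps and falling damage; other targets receive mostly default settings.
; A line-of-sight trace is present but unconnected.
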(event `self.ReceiveBeginPlay`
  (`parent.ReceiveBeginPlay`)
  (`GameplayStatics.ApplyDamage` (`self.MainTarget`) (- (`self.BaseDamage`) (* (* (`self.BaseDamage`) (/ (`self.DamageReduction`) 100.0)) (`self.CurrentJumpCycle`))) (`Pawn.GetController` (`self.Instigator`)) self (`self.Damage Type Class`))
  (bind _returnvalue (`NiagaraFunctionLibrary.SpawnSystemAtLocation` "/Game/Visuals/VFX/Niagara/NS_Lightning.NS_Lightning" (`self.K2_GetActorLocation`)))
  (bind _output_get (set `self.LightningVFX` _returnvalue))
  (`NiagaraComponent.SetVariableVec3` _output_get "BeamStart" (`KismetMathLibrary.InverseTransformLocation` (`self.GetTransform`) (`self.LocOfSphereBefore`)))
  (`NiagaraComponent.SetVariableVec3` (`self.LightningVFX`) "BeamEnd" (0.0 0.0 0.0))
  (`KismetSystemLibrary.K2_SetTimer` null "OnLightningJump" (`self.JumpTimer`)))

(event `/Game/Mechanics/Interfaces/BPI_DebugGizmos.DG_ShowHitbox`
  (`parent.DG_ShowHitbox`)
  (if (`self.ShowHitbox?`)
    (`SceneComponent.SetHiddenInGame` (`self.SphereCollision`) false false)
    (else
      (`SceneComponent.SetHiddenInGame` (`self.SphereCollision`) true false))))

(fn `OnLightningJump`
  (if (<= (`self.CurrentJumpCycle`) (`self.MaxJumpCycles`))
    (`/Engine/EditorBlueprintResources/StandardMacros.IncrementInt` (`self.CurrentJumpCycle`)
      (:`  `
        (for _array_element (`PrimitiveComponent.GetOverlappingActors` (`self.SphereCollision`) "/Script/Engine.Actor")
          (if (and (!= (`self.MainTarget`) _array_element) (`KismetSystemLibrary.DoesImplementInterface` _array_element "/Game/Mechanics/Interfaces/BPI_EffectTargetInterface.BPI_EffectTargetInterface_C"))
            (if (<= (`KismetMathLibrary.RandomFloatInRange` 0.0 100.0) (`self.JumpChance`))
              (if (`GameplayStatics.ObjectIsA` _array_element "/Script/Engine.Character")
                (`|SpawnActorFromClass` "BP_LightningSphere_C" (`KismetMathLibrary.Conv_VectorToTransform` (`self.K2_GetActorLocation` _array_element)) "Undefined" "MultiplyWithRoot" null 300.0 _array_element (`self.BaseDamage`) (`self.Damage Type Class`) (`self.DamageReduction`) (`self.JumpTimer`) (`self.CurrentJumpCycle`) (`self.MaxJumpCycles`) (`self.JumpChance`) (`self.K2_GetActorLocation`) 0.0 (`self.ShowHitbox?`) (`self.Instigator`))
                (else
                  (`|SpawnActorFromClass` "BP_LightningSphere_C" (`KismetMathLibrary.Conv_VectorToTransform` (`self.K2_GetActorLocation` _array_element)) "Undefined" "MultiplyWithRoot" null 300.0 null 30.0 "/Game/Mechanics/DamageTypes/BP_TestDamageType.BP_TestDamageType_C" 0.2 0.3 0 3 50.0 (`self.K2_GetActorLocation`) 0.0 false (`self.Instigator`))))))))))
  (`ActorComponent.K2_DestroyComponent` (`self.LightningVFX`))
  (`self.K2_DestroyActor`))

(fn `UserConstructionScript`
  (`parent.UserConstructionScript`)
  (`SphereComponent.SetSphereRadius` (`self.SphereCollision`) (`self.SphereRadius`) true)
  (if (`self.ShowHitbox?`)
    (`SceneComponent.SetHiddenInGame` (`self.SphereCollision`) false false)))