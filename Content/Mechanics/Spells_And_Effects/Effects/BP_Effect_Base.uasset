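; BP_Effect_Base is the base class for timed effects applied to an owner.
; OnInit stores the owner and effect manager and sets the duration; while ticking is enabled, the update counts it down and asks the manager to remove the effect at zero.
; Apply and remove events toggle the owner's HUD icon, keyed by the class name after "BP_Effect_".
; OnGetHit returns zero by default.
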(fn `GetEffectName`
  (returns (Name :type String))
  (return (`.RightS` (`KismetStringLibrary.Split` (`KismetSystemLibrary.GetClassDisplayName` (`GameplayStatics.GetObjectClass` self)) "BP_Effect_"))))

(fn `OnEffectApplied`
  (bind _name (`self.GetEffectName`))
  (`/Game/Mechanics/Interfaces/BPI_EffectTargetInterface.ETI_AddEffectIconHUD` (`self.EffectOwner`) _name))

(fn `OnEffectRemoved`
  (bind _name (`self.GetEffectName`))
  (`/Game/Mechanics/Interfaces/BPI_EffectTargetInterface.ETI_RemoveEffectIconHUD` (`self.EffectOwner`) _name))

(fn `OnGetHit`
  (params (DamageAmount :type "Float (double-precision)"))
  (returns (RestDamageAmount :type "Float (double-precision)"))
  (return 0.0))

(fn `OnInit`
  (params (EffectOwner :type "/Game/Mechanics/Interfaces/BPI_EffectTargetInterface Interface") (EffectManager :type "/Game/Mechanics/Components/BPC_EffectManager Object Reference"))
  (set `self.EffectOwner` EffectOwner)
  (set `self.EffectManager` EffectManager)
  (set `self.RemainingDuration` (`self.EffectDuration`)))

(fn `OnTick`
  (params (DeltaTime :type "Float (double-precision)"))
  (bind _output_get (set `self.RemainingDuration` (- (`self.RemainingDuration`) DeltaTime)))
  (if (<= _output_get 0.0)
    (`/Game/Mechanics/Components/BPC_EffectManager.EM_RemoveEffect` (`self.EffectManager`) self)))

(fn `OnUpdateFunction`
  (params (DeltaTime :type "Float (double-precision)"))
  (if (`self.IsTickEnabled`)
    (`self.OnTick` DeltaTime)))