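; Ice Storm damage effect that periodically damages its owner while applied.
; On apply, a looping timer calls DealDamage every damage interval, with a negative start delay cancelling the first wait so damage begins immediately.
; Each tick sends the damage amount and type to the effect owner through ETIOnTakeEffectDamage.
; Removal pauses the timer rather than clearing it, and init only forwards to the parent effect class.
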(fn `DealDamage`
  (`/Game/Mechanics/Interfaces/BPI_EffectTargetInterface.ETI_OnTakeEffectDamage` (`self.EffectOwner`) (`self.DamageAmount`) null (`self.DamageType`)))

(fn `OnEffectApplied`
  (bind _damageinterval (`self.DamageInterval`))
  (`parent.OnEffectApplied`)
  (`KismetSystemLibrary.K2_SetTimer` null "DealDamage" _damageinterval true false (* _damageinterval -1.0)))

(fn `OnEffectRemoved`
  (`parent.OnEffectRemoved`)
  (`KismetSystemLibrary.K2_PauseTimer` null "DealDamage"))

(fn `OnInit`
  (params (EffectOwner :type "/Game/Mechanics/Interfaces/BPI_EffectTargetInterface Interface") (EffectManager :type "/Game/Mechanics/Components/BPC_EffectManager Object Reference"))
  (`parent.OnInit` EffectOwner EffectManager))