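; Trigger actor that shows the tutorial box HUD while the player character overlaps it and grants a rune.
; Begin and end overlap events check for the player character, then toggle the HUD through BP_ThirdPersonCharacter's SwitchTutorialBoxHUD.
; On the first entry only, a DoOnce adds the "Volatility" rune to the character's known runes via its BPCRuneSystem component.
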(event `self.ReceiveActorBeginOverlap`
  (params (OtherActor :type "Actor Object Reference"))
  (bind _returnvalue (`GameplayStatics.GetPlayerCharacter` 0))
  (if (== OtherActor _returnvalue)
    (bind _asbp_third_person_character (cast `/Game/Mechanics/Player/Blueprints/BP_ThirdPersonCharacter` _returnvalue))
    (`/Game/Mechanics/Player/Blueprints/BP_ThirdPersonCharacter.SwitchTutorialBoxHUD` _asbp_third_person_character true)
    (`/Engine/EditorBlueprintResources/StandardMacros.DoOnce` false
      (:`Completed`
        (`/Game/Mechanics/Components/BPC_RuneSystem.AddRuneToKnownRunes` (`/Game/Mechanics/Player/Blueprints/BP_ThirdPersonCharacter.BPC_RuneSystem` _asbp_third_person_character) "Volatility")))))

(event `self.ReceiveActorEndOverlap`
  (params (OtherActor :type "Actor Object Reference"))
  (bind _returnvalue (`GameplayStatics.GetPlayerCharacter` 0))
  (if (== OtherActor _returnvalue)
    (bind _asbp_third_person_character (cast `/Game/Mechanics/Player/Blueprints/BP_ThirdPersonCharacter` _returnvalue))
    (`/Game/Mechanics/Player/Blueprints/BP_ThirdPersonCharacter.SwitchTutorialBoxHUD` _asbp_third_person_character false)))

(fn `UserConstructionScript`)