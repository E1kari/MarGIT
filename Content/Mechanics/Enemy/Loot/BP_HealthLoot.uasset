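; BP_HealthLoot is a health pickup that hovers in place and heals the player character on contact.
; Tick bobs the mesh vertically around its starting relative location with a game-time sine wave driven by hover amplitude and frequency.
; On mesh overlap with BP_ThirdPersonCharacter, it picks a random or maximum heal amount, sends it through the ETIHealByAmount interface message, then destroys itself.
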(event `self.ReceiveBeginPlay`
  (set `self.BaseRelativeLoc` (`SceneComponent.RelativeLocation` (`self.Mesh`))))

(event `self.ReceiveTick`
  (params (DeltaSeconds :type "Float (single-precision)"))
  (`SceneComponent.K2_SetRelativeLocation` (`self.Mesh`) (+ (`self.BaseRelativeLoc`) (`KismetMathLibrary.MakeVector` 0.0 0.0 (* (`KismetMathLibrary.Sin` (* (`KismetSystemLibrary.GetGameTimeInSeconds`) (* (* (`KismetMathLibrary.GetPI`) 2.0) (`self.HoverFrequencyHz`)))) (`self.HoverAmplitude`)))) false false))

(event `self.Mesh.OnComponentBeginOverlap`
  (params (OverlappedComponent :type "PrimitiveComponent Object Reference") (OtherActor :type "Actor Object Reference") (OtherComp :type "PrimitiveComponent Object Reference") (OtherBodyIndex :type Integer) (bFromSweep :type Boolean) (SweepResult :type "HitResult Structure (by ref)"))
  (if (`GameplayStatics.ObjectIsA` OtherActor "/Game/Mechanics/Player/Blueprints/BP_ThirdPersonCharacter.BP_ThirdPersonCharacter_C")
    (if (`self.IsHealthAmountRandom`)
      (set `self.HealthAmount` (`KismetMathLibrary.RandomFloatInRange` (`self.MinHealthAmount`) (`self.MaxHealthAmount`)))
      (else
        (set `self.HealthAmount` (`self.MaxHealthAmount`))))
    (message `/Game/Mechanics/Interfaces/BPI_EffectTargetInterface.ETI_HealByAmount` OtherActor (`self.HealthAmount`))
    (`self.K2_DestroyActor`)))

(fn `UserConstructionScript`)