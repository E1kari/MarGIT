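; BP_Enemy_Cloak is an enemy character that casts spells at a target and detects nearby actors for fleeing.
; A server RPC waits briefly, spawns the EnemySpell aimed from SpellCastPoint at the target, then signals the attack's end.
; A separate multicast event plays the attack montage.
; FleeSphere overlaps are forwarded to AIC_Enemy_Cloak, the AI controller, to check whether the actor is in fleeing range.
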(event `RPC_EC_Server_SpellAttack`
  (params (AttackTarget :type "Actor Object Reference"))
  (`KismetSystemLibrary.Delay` 0.2)
  (bind _spelltransform (`self.GetSpellTransform` AttackTarget))
  (`|SpawnActorFromClass` (`self.EnemySpell`) _spelltransform "Undefined" "MultiplyWithRoot" null self false null)
  (`self.OnSpellAttackEnd`))

(event `RPC_EC_MC_SpellAttack`
  (`|PlayMontage` null))

(event `self.FleeSphere.OnComponentBeginOverlap`
  (params (OverlappedComponent :type "PrimitiveComponent Object Reference") (OtherActor :type "Actor Object Reference") (OtherComp :type "PrimitiveComponent Object Reference") (OtherBodyIndex :type Integer) (bFromSweep :type Boolean) (SweepResult :type "HitResult Structure (by ref)"))
  (bind _asaic_enemy_cloak (cast `/Game/Mechanics/Enemy/AI/AIC_Enemy_Cloak` (`AIBlueprintHelperLibrary.GetAIController` self))
    (:`then`
      (`/Game/Mechanics/Enemy/AI/AIC_Enemy_Cloak.CheckSensedActorInFleeingRange` _asaic_enemy_cloak OtherActor))
    (:`CastFailed`
      (`KismetSystemLibrary.PrintString` "BP_Enemy_Cloak: Cast to AIC_Enemy_Cloak failed"))))

(fn `GetSpellTransform`
  (params (AttackTarget :type "Actor Object Reference"))
  (returns (SpellTransform :type "Transform Structure"))
  (bind _returnvalue (`SceneComponent.K2_GetComponentLocation` (`self.SpellCastPoint`)))
  (return (`KismetMathLibrary.MakeTransform` _returnvalue (`KismetMathLibrary.FindLookAtRotation` _returnvalue (`self.K2_GetActorLocation` AttackTarget)))))

(fn `UserConstructionScript`
  (`parent.UserConstructionScript`))