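; Enemy 03 character, driven by AIC_Enemy_03, with a provisional jump attack standing in until an attack animation exists.
; OnAttack jumps and polls vertical velocity on a looping timer; at zero it plays SFX, damages the controller's target without rechecking range, pauses the timer and signals attack end.
; AttackRangeSphere overlaps with the target toggle the controller's attack-range flag.
; Knockback launches the character at half impulse and spawns VFX.
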(event `OnAttack`
  ; Provizorische Attack Function while no Anim available
  (`self.Jump`)
  (bind _returnvalue (`KismetSystemLibrary.K2_SetTimerDelegate` (delegate `CheckOnJumpEnd`) 0.1 true))
  (set `self.JumpTimer` _returnvalue))

(event `/Game/Mechanics/Interfaces/BPI_EffectTargetInterface.ETI_OnKnockback`
  (params (ImpulseForce :type "Vector Structure") (`Spell Owner` :type "Actor Object Reference"))
  (`self.LaunchCharacter` (/ ImpulseForce 2.0))
  (`self.SpawnKnockbackVFX` ImpulseForce))

(event `CheckOnJumpEnd`
  (bind (_velocity_x _velocity_y _velocity_z) (`KismetMathLibrary.BreakVector` (`MovementComponent.Velocity` (`self.CharacterMovement`))))
  ; Provizorische Attack Function while no Anim available
  (if (== _velocity_z 0.0)
    (`self.PlayAttackSFX`)
    (`GameplayStatics.ApplyDamage` (`/Game/Mechanics/Enemy/AI/AIC_Enemy_Base.AttackTarget` (`self.AIController`)) (`self.BaseDamage`) null self "/Game/Mechanics/DamageTypes/BP_TestDamageType.BP_TestDamageType_C")
    (`KismetSystemLibrary.K2_PauseTimerHandle` (`self.JumpTimer`))
    (`self.OnAttackEnd`)))

(event `self.ReceiveBeginPlay`
  (bind _asaic_enemy_03 (cast `/Game/Mechanics/Enemy/AI/AIC_Enemy_03` (`AIBlueprintHelperLibrary.GetAIController` self)))
  (set `self.AIController` _asaic_enemy_03))

(event `self.AttackRangeSphere.OnComponentBeginOverlap`
  (params (OverlappedComponent :type "PrimitiveComponent Object Reference") (OtherActor :type "Actor Object Reference") (OtherComp :type "PrimitiveComponent Object Reference") (OtherBodyIndex :type Integer) (bFromSweep :type Boolean) (SweepResult :type "HitResult Structure (by ref)"))
  (bind _aicontroller (`self.AIController`)
    (:`then`
      (if (== (`/Game/Mechanics/Enemy/AI/AIC_Enemy_Base.AttackTarget` _aicontroller) OtherActor)
        (`/Game/Mechanics/Enemy/AI/AIC_Enemy_03.SetAttackRange` _aicontroller true)))
    (:`else`)))

(event `self.AttackRangeSphere.OnComponentEndOverlap`
  (params (OverlappedComponent :type "PrimitiveComponent Object Reference") (OtherActor :type "Actor Object Reference") (OtherComp :type "PrimitiveComponent Object Reference") (OtherBodyIndex :type Integer))
  (bind _aicontroller (`self.AIController`)
    (:`then`
      (if (== (`/Game/Mechanics/Enemy/AI/AIC_Enemy_Base.AttackTarget` _aicontroller) OtherActor)
        (`/Game/Mechanics/Enemy/AI/AIC_Enemy_03.SetAttackRange` _aicontroller false)))
    (:`else`)))

(fn `UserConstructionScript`
  (`parent.UserConstructionScript`))