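; Rune spellcasting component that classifies mouse-drawn runes and combines them into spells.
; Mouse points are rendered to a canvas render target (optionally saved as PNG) and fed as grayscale to an ONNX model.
; Known predictions accumulate, then their unique, sorted labels form a "+"-joined key into SpellsMap for server spawning.
; RPC events handle rune VFX and slow-motion drawing with fewer than two players, while GameInstance counts results.
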(event `self.ReceiveBeginPlay`
  (bind _returnvalue (`KismetMathLibrary.FTrunc` (`self.CanvasWH`)))
  (bind _returnvalue_2 (`CanvasRenderTarget2D.CreateCanvasRenderTarget2D` "/Game/Mechanics/RuneAI/Blueprints/BP_RuneDrawCanvas.BP_RuneDrawCanvas_C" _returnvalue _returnvalue))
  (set `self.RuneCanvas` _returnvalue_2)
  (bind _returnvalue_3 (`|SpawnActorFromClass` "/Game/Mechanics/RuneAI/Blueprints/BP_ONNXInferenceActor.BP_ONNXInferenceActor_C" (`KismetMathLibrary.MakeTransform` (0.0 0.0 0.0)) "Undefined" "MultiplyWithRoot" null null))
  (set `self.ONNXModel` _returnvalue_3)
  (bind _asgi_game_instance (cast `/Game/Mechanics/GameInstance/GI_GameInstance` (`GameplayStatics.GetGameInstance`)))
  (set `self.GameInstance` _asgi_game_instance))

(event `RPC_RS_Server_RuneRecognized`
  (params (CurrentRuneEffect :type "NiagaraComponent Object Reference"))
  ; FX Rune (Not) Recognized Calls
  (`self.RPC_RuneRecognized` CurrentRuneEffect))

(event `RPC_RS_Server_RuneNotRecognized`
  (params (CurrentRuneEffect :type "NiagaraComponent Object Reference"))
  ; FX Rune (Not) Recognized Calls
  (`self.RPC_RuneNotRecognized` CurrentRuneEffect))

(event `RPC_RS_Server_StartTimeDelation`
  ; Time Delation
  (`self.StartTimeDelation`))

(event `RPC_RuneRecognized`
  (params (CurrentRuneEffect :type "NiagaraComponent Object Reference"))
  ; FX Rune (Not) Recognized Calls
  (`self.Deactivate` CurrentRuneEffect))

(event `RPC_RuneNotRecognized`
  (params (CurrentRuneEffect :type "NiagaraComponent Object Reference"))
  ; FX Rune (Not) Recognized Calls
  (`NiagaraComponent.SetNiagaraVariableVec3` CurrentRuneEffect "User.GravityForce" (0.0 0.0 -980.0))
  (`NiagaraComponent.SetNiagaraVariableFloat` CurrentRuneEffect "LifeTime" 1.5)
  (`self.K2_DestroyComponent` CurrentRuneEffect))

(event `RPC_RS_Server_StopTimeDelation`
  ; Time Delation
  (`self.StopTimeDelation`))

(event `RPC_RS_Server_DestroyAllRunes`
  ; Destroy all drawn runes
  (`self.RPC_DestroyAllRunes`))

(event `RPC_DestroyAllRunes`
  (bind _allrunevfx (`self.AllRuneVFX`))
  ; Destroy all drawn runes
  (for _array_element _allrunevfx
    (`self.K2_DestroyComponent` _array_element))
  (`KismetArrayLibrary.Array_Clear` _allrunevfx))

(event `RPC_RS_Server_CastSpell`
  (params (SpellBluePrint :type "/Game/Mechanics/Spells_And_Effects/Spells/BaseSpells/BP_BaseSpell Class Reference") (SpellTransform :type "Transform Structure") (SpellOwner :type "Character Object Reference"))
  ; Cast Spell
  ;; To disable Spawning while inEngine RuneDrawinh
  (if (`self.CastSpell`)
    (if (`Actor.HasAuthority` (`GameplayStatics.GetPlayerController` 0))
      (`|SpawnActorFromClass` SpellBluePrint SpellTransform "Undefined" "MultiplyWithRoot" null SpellOwner (`self.ShowHitbox?`) null))))

(fn `AddRuneToKnownRunes`
  (params (RuneName :type String))
  (`KismetArrayLibrary.Array_AddUnique` (`self.KnownRunes`) RuneName))

(fn `CheckToAddResult`
  (params (PredictionResult :type "PredictionResult Structure") (`Current Rune Effect` :type "NiagaraComponent Object Reference"))
  (bind (_predictedlabel _predictedindex _confidence _bsuccess) (break `PredictionResult` PredictionResult))
  (bind (_predictedlabel_2 _predictedindex_2 _confidence_2) (break `PredictionResult` (`self.DebugPredictionResult`)))
  (bind _returnvalue (`KismetStringLibrary.Concat_StrStr` "Debug: Predicted Rune: " _predictedlabel_2 " " "with Confidence: " (`KismetStringLibrary.Conv_DoubleToString` _confidence_2)))
  (if (`KismetArrayLibrary.Array_Contains` (`self.KnownRunes`) _predictedlabel)
    (`KismetArrayLibrary.Array_Add` (`self.RunePredictionResultArray`) PredictionResult)
    (`self.RPC_RS_Server_RuneRecognized` `Current Rune Effect`)
    (bind _output_get (set `self.DebugPredictionResult` PredictionResult))
    (bind (_predictedlabel_3 _predictedindex_3 _confidence_3) (break `PredictionResult` _output_get))
    (`KismetSystemLibrary.PrintString` (`KismetStringLibrary.Concat_StrStr` "Debug: Predicted Rune: " _predictedlabel_3 " " "with Confidence: " (`KismetStringLibrary.Conv_DoubleToString` _confidence_3)) true true (struct :`R` 0.079028 :`G` 1.0 :`B` 0.072917 :`A` 1.0))
    (else
      (if (`KismetStringLibrary.EqualEqual_StrStr` _predictedlabel "Unknown")
        (set `self.DebugPredictionResult` PredictionResult)
        (`KismetSystemLibrary.PrintString` _returnvalue true true (struct :`R` 1.0 :`G` 0.03125 :`B` 0.03125 :`A` 1.0))
        (else
          (set `self.DebugPredictionResult` (make `PredictionResult` "Unknown till now" 2 _confidence _bsuccess))
          (`KismetSystemLibrary.PrintString` _returnvalue true true (struct :`R` 1.0 :`G` 0.970797 :`B` 0.031642 :`A` 1.0))))
      (`self.RPC_RS_Server_RuneNotRecognized` `Current Rune Effect`)))
  (`/Game/Mechanics/GameInstance/GI_GameInstance.AddToRuneCounter` (`self.GameInstance`) (`self.DebugPredictionResult`)))

(fn `ClearRunePredictionResultsArray`
  (`KismetArrayLibrary.Array_Clear` (`self.RunePredictionResultArray`)))

(fn `GetDeprojectScreenToWorld`
  (returns (Pos :type "Vector Structure"))
  (bind _returnvalue (`GameplayStatics.GetPlayerController` 0))
  (bind (_locationx _locationy) (`PlayerController.GetMousePosition` _returnvalue))
  (bind (_worldposition _worlddirection) (`GameplayStatics.DeprojectScreenToWorld` _returnvalue (`KismetMathLibrary.MakeVector2D` _locationx _locationy)))
  (return (+ _worldposition (* _worlddirection (`self.SpawnDistanceToPlayer`)))))

(fn `RS_CastSpell`
  (params (SpellOwner :type "Character Object Reference") (SpellTransform :type "Transform Structure"))
  (locals (RunesNames :type "Array of String") (SpellName :type String))
  (bind _runesnames (`local.RunesNames`))
  (bind _runesnames_2 (`local.RunesNames`))
  (bind _returnvalue (`KismetArrayLibrary.Array_Length` _runesnames))
  (bind (_value _returnvalue_2) (`BlueprintMapLibrary.Map_Find` (`self.SpellsMap`) (`local.SpellName`)))
  (`KismetArrayLibrary.Array_Clear` (`local.RunesNames`))
  (for _array_element (`self.RunePredictionResultArray`)
    (`KismetArrayLibrary.Array_AddUnique` (`local.RunesNames`) (`.PredictedLabel` (break `PredictionResult` _array_element))))
  (`KismetArrayLibrary.SortStringArray` _runesnames)
  (if (> _returnvalue 0)
    (set `local.SpellName` (`|GetArrayItem` _runesnames))
    (if (> _returnvalue 1)
      (for _index (range 1 (+ (`KismetArrayLibrary.Array_LastIndex` _runesnames_2) 1))
        (set `local.SpellName` (`KismetStringLibrary.Concat_StrStr` (`local.SpellName`) "+" (`|GetArrayItem` _runesnames_2 _index)))))
    (if _returnvalue_2
      (`self.RPC_RS_Server_CastSpell` _value SpellTransform SpellOwner)
      (`/Game/Mechanics/GameInstance/GI_GameInstance.AddToSpellCounter` (`self.GameInstance`) (`KismetSystemLibrary.GetClassDisplayName` _value))
      (else
        (`KismetSystemLibrary.PrintString` "Spell not Found")
        (`/Game/Mechanics/GameInstance/GI_GameInstance.AddToSpellCounter` (`self.GameInstance`) "Unknown")))
    (`self.RPC_RS_Server_DestroyAllRunes`)
    (`KismetArrayLibrary.Array_Clear` (`self.RunePredictionResultArray`))))

(fn `RS_OnOngoingDrawing`
  (bind (_returnvalue_x _returnvalue_y) (`KismetMathLibrary.BreakVector2D` (`WidgetLayoutLibrary.GetViewportSize`)))
  (bind _canvaswh (`self.CanvasWH`))
  (bind (_locationx _locationy) (`PlayerController.GetMousePosition` (`GameplayStatics.GetPlayerController` 0)))
  (`KismetArrayLibrary.Array_Add` (`self.RuneDrawingPoints`) (`KismetMathLibrary.MakeVector2D` (* (/ _locationx _returnvalue_x) _canvaswh) (* (/ _locationy _returnvalue_y) _canvaswh))))

(fn `RS_OnStartDrawing`
  (`KismetArrayLibrary.Array_Clear` (`self.RuneDrawingPoints`))
  (`self.RPC_RS_Server_StartTimeDelation`))

(fn `RS_OnStopDrawing`
  (params (CurrentRuneEffect :type "NiagaraComponent Object Reference"))
  (locals (BaseFolderPath :type String :default "DrawnRunes/"))
  (bind _runename (`self.RuneName`))
  (bind _runecanvas (`self.RuneCanvas`))
  (`KismetArrayLibrary.Array_Add` (`self.AllRuneVFX`) CurrentRuneEffect)
  (bind _asbp_rune_draw_canvas (cast `/Game/Mechanics/RuneAI/Blueprints/BP_RuneDrawCanvas` _runecanvas)
    (:`then`
      (set `/Game/Mechanics/RuneAI/Blueprints/BP_RuneDrawCanvas.RunePoints` (`self.RuneDrawingPoints`) _asbp_rune_draw_canvas)
      (`CanvasRenderTarget2D.UpdateResource` _runecanvas)
      (if (`self.SaveDrawnRunes`)
        (`RuneFunctionLibrary.SaveCanvasRenderTargetToPNG` _runecanvas (`KismetStringLibrary.Concat_StrStr` (`local.BaseFolderPath`) _runename) (`KismetStringLibrary.Concat_StrStr` _runename "_" (`KismetStringLibrary.Conv_IntToString` (`self.RuneNameCounter`))))
        (bind _result (`/Engine/EditorBlueprintResources/StandardMacros.IncrementInt` (`self.RuneNameCounter`))
          (:`  `
            (`KismetSystemLibrary.PrintString` (`KismetStringLibrary.Concat_StrStr` (`self.RuneName`) " " (`KismetStringLibrary.Conv_IntToString` _result))))))
      (bind _outdata (`RuneFunctionLibrary.GetCanvasGrayscaleData` _runecanvas))
      (bind _onnxmodel (`self.ONNXModel`)
        (:`then`
          (bind _returnvalue (`ONNXInferenceActor.RunInferenceBP` _onnxmodel _outdata))
          (`self.CheckToAddResult` _returnvalue CurrentRuneEffect)
          (`self.RPC_RS_Server_StopTimeDelation`))
        (:`else`
          (`KismetSystemLibrary.PrintString` "Not Valid"))))
    (:`CastFailed`
      (`KismetSystemLibrary.PrintString` "Cast Failed"))))

(fn `SetLocalMousePos64x64`
  (returns (NewParam :type "Vector2D Structure"))
  (bind (_returnvalue_x _returnvalue_y) (`KismetMathLibrary.BreakVector2D` (`WidgetLayoutLibrary.GetViewportSize`)))
  (bind (_locationx _locationy) (`PlayerController.GetMousePosition` (`GameplayStatics.GetPlayerController` 0)))
  (return (`KismetMathLibrary.MakeVector2D` (* (/ _locationx _returnvalue_x) 64.0) (* (/ _locationy _returnvalue_y) 64.0))))

(fn `StartTimeDelation`
  (if (`self.EnableTimeDelation`)
    (bind _asbp_third_person_game_mode (cast `/Game/Mechanics/Player/GameModes/BP_ThirdPersonGameMode` (`GameplayStatics.GetGameMode`)))
    (bind _returnvalue (`GameModeBase.GetNumPlayers` _asbp_third_person_game_mode))
    (if (< _returnvalue 2)
      (`GameplayStatics.SetGlobalTimeDilation` (`self.SlowedTimeDelation`)))))

(fn `StopTimeDelation`
  (`GameplayStatics.SetGlobalTimeDilation` (`self.BaseTimeDelation`)))