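; BPC_ColorManager is a component that applies one color to an emissive mesh and an optional light source on BeginPlay.
; LightRefresh uses either a local color or a preset read from the MPC_ColorPresets parameter collection, with the enum name as parameter name.
; It writes the color to the mesh's RedChannelLight material parameter and the light, then scales intensity, and point-light attenuation radius, by the mesh's average world scale.
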(event `self.ReceiveBeginPlay`
  (`self.lightRefresh`))

(fn `lightRefresh`
  (bind _returnvalue (/ (+ (.x (`SceneComponent.K2_GetComponentScale` (`self.EmissionMesh`))) (.y (`SceneComponent.K2_GetComponentScale` (`self.EmissionMesh`))) (.z (`SceneComponent.K2_GetComponentScale` (`self.EmissionMesh`)))) 3.0))
  (if (`self.useLocalColor`)
    (set `self.LightColor` (`self.LocalColor`))
    (else
      (bind _returnvalue_2 (`KismetMaterialLibrary.GetVectorParameterValue` "/Game/Visuals/Material/LightSystem/MPC_ColorPresets.MPC_ColorPresets" (`KismetStringLibrary.Conv_StringToName` (`|GetEnumeratorNameAsString` (`self.Preset Color`)))))
      (set `self.LightColor` _returnvalue_2)))
  (`MeshComponent.SetVectorParameterValueOnMaterials` (`self.EmissionMesh`) "RedChannelLight" (`KismetMathLibrary.Conv_LinearColorToVector` (`self.LightColor`)))
  (if (`KismetSystemLibrary.IsValid` (`self.LightSource`))
    (`LightComponent.SetLightColor` (`self.LightSource`) (`self.LightColor`) true)
    (`LightComponent.SetIntensity` (`self.LightSource`) (* 1000.0 _returnvalue))
    (bind _aspoint_light_component (cast `PointLightComponent` (`self.LightSource`)))
    (`LocalLightComponent.SetAttenuationRadius` _aspoint_light_component (* 1000.0 _returnvalue))))