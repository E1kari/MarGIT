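; Temple hub statue actor that rescales itself uniformly based on its distance to the player pawn.
; Each tick it maps that distance from the min/max distance range onto the min/max scale, updating only while the player is inside that range.
; The construction script assigns a GUID when the ID is empty.
; Save functions add this ID and current scale to the level save data and restore the scale from statue save data.
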(event `self.ReceiveBeginPlay`)

(event `self.ReceiveTick`
  (params (DeltaSeconds :type "Float (single-precision)"))
  (bind _returnvalue (`KismetMathLibrary.MapRangeClamped` (`self.Distance`) (`self.MinDistance`) (`self.MaxDistance`) (`self.MinScale`) (`self.MaxScale`)))
  (bind _playercharacterref (`self.PlayerCharacterRef`)
    (:`then`
      (set `self.Distance` (`KismetMathLibrary.Vector_Distance` (`self.K2_GetActorLocation`) (`self.K2_GetActorLocation` _playercharacterref)))
      (if (and (< (`self.Distance`) (`self.MaxDistance`)) (> (`self.Distance`) (`self.MinDistance`)))
        (`self.SetActorScale3D` (`KismetMathLibrary.MakeVector` _returnvalue _returnvalue _returnvalue))))
    (:`else`
      (set `self.PlayerCharacterRef` (`GameplayStatics.GetPlayerPawn` 0)))))

(fn `GetActorSaveData`
  (params (CurrentLevelSaveData :type "/Game/Mechanics/SaveGameSystem/SaveGameStructs/S_LevelSaveData Structure"))
  (returns (FilledLevelSaveData :type "/Game/Mechanics/SaveGameSystem/SaveGameStructs/S_LevelSaveData Structure"))
  (locals (LevelSaveData :type "/Game/Mechanics/SaveGameSystem/SaveGameStructs/S_LevelSaveData Structure"))
  (bind _output_get (set `local.LevelSaveData` CurrentLevelSaveData))
  (bind _statuesavedata (`self.GetStatueSaveData`))
  (`KismetArrayLibrary.Array_Add` (`.AllStatues_16_D6623FAA4847E1F539D56FACBD7E977F` (break `/Game/Mechanics/SaveGameSystem/SaveGameStructs/S_LevelSaveData` _output_get)) _statuesavedata)
  (return (`local.LevelSaveData`)))

(fn `GetActorUniqueID`
  (returns (UniqueID :type String))
  (return (`self.UniqueID`)))

(fn `GetStatueSaveData`
  (returns (StatueSaveData :type "/Game/Mechanics/SaveGameSystem/SaveGameStructs/S_StatueSaveData Structure"))
  (return (make `/Game/Mechanics/SaveGameSystem/SaveGameStructs/S_StatueSaveData` (`self.UniqueID`) (`self.GetActorScale3D`))))

(fn `UserConstructionScript`
  (if (`KismetStringLibrary.IsEmpty` (`self.UniqueID`))
    (set `self.UniqueID` (`KismetGuidLibrary.Conv_GuidToString` (`KismetGuidLibrary.NewGuid`)))
    (`self.SetActorTickEnabled` (`self.TickEnabled`))))

(fn `UseStatueSaveData`
  (params (StatueSaveData :type "/Game/Mechanics/SaveGameSystem/SaveGameStructs/S_StatueSaveData Structure"))
  (`self.SetActorScale3D` StatueSaveData_CurrentScale_7_01D9AE9446BCF826CD513E838100BF27))