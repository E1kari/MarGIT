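; Base class for crystal switches that toggle between active and inactive whenever they take damage, playing a sound on activation.
; The IsActive RepNotify swaps the crystal's material and calls empty OnActivate/OnDeactivate hooks; the multicast RPC equivalents appear to be leftovers.
; Construction applies the start state, generates a GUID if needed and refreshes the color manager's emission lighting.
; Save functions store state, ID and class in level save data and restore the active state.
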(event `self.ReceiveAnyDamage`
  (params (Damage :type "Float (single-precision)") (DamageType :type "DamageType Object Reference") (InstigatedBy :type "Controller Object Reference") (DamageCauser :type "Actor Object Reference"))
  (bind _output_get (set `self.IsActive` (not (`self.IsActive`))))
  (if _output_get
    (`self.PlayActivateSFX`)))

(event `RPC_MC_OnActivate`
  (`self.OnActivate`))

(event `RPC_MC_OnDeactivate`
  (`self.OnDeactivate`))

(event `/Game/Mechanics/Interfaces/BPI_DebugGizmos.DG_ShowHitbox`
  (`parent.DG_ShowHitbox`)
  (if (`self.ShowHitbox?`)
    (`SceneComponent.SetHiddenInGame` (`self.Capsule`) false false)
    (else
      (`SceneComponent.SetHiddenInGame` (`self.Capsule`) true false))))

(fn `GetActorSaveData`
  (params (CurrentLevelSaveData :type "/Game/Mechanics/SaveGameSystem/SaveGameStructs/S_LevelSaveData Structure"))
  (returns (FilledLevelSaveData :type "/Game/Mechanics/SaveGameSystem/SaveGameStructs/S_LevelSaveData Structure"))
  (locals (LevelSaveData :type "/Game/Mechanics/SaveGameSystem/SaveGameStructs/S_LevelSaveData Structure"))
  (bind _output_get (set `local.LevelSaveData` CurrentLevelSaveData))
  (bind _crystalsavedata (`self.GetCrystalSaveData`))
  (`KismetArrayLibrary.Array_Add` (`.AllCrystals_6_0831D2FB493E6618B7017184EE3C1AC3` (break `/Game/Mechanics/SaveGameSystem/SaveGameStructs/S_LevelSaveData` _output_get)) _crystalsavedata)
  (return (`local.LevelSaveData`)))

(fn `GetActorUniqueID`
  (returns (UniqueID :type String))
  (return (`self.UniqueID`)))

(fn `GetCrystalSaveData`
  (returns (CrystalSaveData :type "/Game/Mechanics/SaveGameSystem/SaveGameStructs/S_CrystalSaveData Structure"))
  (return (make `/Game/Mechanics/SaveGameSystem/SaveGameStructs/S_CrystalSaveData` (`self.UniqueID`) (`self.IsActive`) (`GameplayStatics.GetObjectClass` self))))

(fn `OnActivate`)

(fn `OnDeactivate`)

(fn `OnRep_IsActive`
  (if (`self.IsActive`)
    (`PrimitiveComponent.SetMaterial` (`self.crystal_switch`) 0 (`self.Material_Active`))
    (`self.OnActivate`)
    (else
      (`PrimitiveComponent.SetMaterial` (`self.crystal_switch`) 0 (`self.Material_Deactive`))
      (`self.OnDeactivate`))))

(fn `PlayActivateSFX`
  (`AudioManagerSubsystem.PlaySFXAtLocation` (subsystem `AudioManagerSubsystem`) (`self.ActivationSFX`) (`self.K2_GetActorLocation`) null false 1.0 true))

(fn `UseCrystalSaveData`
  (params (CrystalSaveData :type "/Game/Mechanics/SaveGameSystem/SaveGameStructs/S_CrystalSaveData Structure"))
  (set `self.IsActive` CrystalSaveData_IsActive_1_9F8FBC5541BE16C91F22409B2FBFD495))

(fn `UserConstructionScript`
  (bind _bpc_colormanager (`self.BPC_ColorManager`))
  (set `self.IsActive` (`self.StartAsActive`))
  (if (`KismetStringLibrary.IsEmpty` (`self.UniqueID`))
    (set `self.UniqueID` (`KismetGuidLibrary.Conv_GuidToString` (`KismetGuidLibrary.NewGuid`))))
  (set `/Game/Mechanics/Components/BPC_ColorManager.EmissionMesh` (`self.crystal_switch`) _bpc_colormanager)
  (`/Game/Mechanics/Components/BPC_ColorManager.lightRefresh` _bpc_colormanager))