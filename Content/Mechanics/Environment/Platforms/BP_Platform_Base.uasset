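; BP_Platform_Base is a base Blueprint for environment platforms, providing shared activation, timing, light color and save-data helpers.
; The construction script applies LightColor to the cube's materials and assigns a GUID-based UniqueID when empty.
; Save functions package ID, transform and class, and restore only the transform.
; Helpers scale timeline play rate by TimeToComplete and optionally activate on begin; the debug hitbox toggle is left unwired.
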(event `/Game/Mechanics/Interfaces/BPI_DebugGizmos.DG_ShowHitbox`
  (`parent.DG_ShowHitbox`)
  (if (`self.ShowHitbox?`)
    _))

(fn `GetPlatformSaveData`
  (returns (PlatformSaveData :type "/Game/Mechanics/SaveGameSystem/SaveGameStructs/S_PlatformSaveData Structure"))
  (return (make `/Game/Mechanics/SaveGameSystem/SaveGameStructs/S_PlatformSaveData` (`self.UniqueID`) (`self.GetTransform`) (`GameplayStatics.GetObjectClass` self))))

(fn `LightRefresh`
  (`MeshComponent.SetVectorParameterValueOnMaterials` (`self.Cube`) "RedChannelLight" (`KismetMathLibrary.Conv_LinearColorToVector` (`self.Light Color`))))

(fn `SetPlayRate`
  (params (Timeline :type "TimelineComponent Object Reference"))
  (`TimelineComponent.SetPlayRate` Timeline (/ 1.0 (`self.TimeToComplete`))))

(fn `StartOnBegin`
  (if (`self.StartAsActive`)
    (`/Game/Mechanics/Interfaces/BPI_EnvironmentInterface.EI_OnActivate`)))

(fn `UsePlatfromSaveData`
  (params (PlatformSaveData :type "/Game/Mechanics/SaveGameSystem/SaveGameStructs/S_PlatformSaveData Structure"))
  (`self.K2_SetActorTransform` PlatformSaveData_Transform_2_DD842C2549C2BFB15B44419C0C0A7A23))

(fn `UserConstructionScript`
  (`self.LightRefresh`)
  (if (`KismetStringLibrary.IsEmpty` (`self.UniqueID`))
    (set `self.UniqueID` (`KismetGuidLibrary.Conv_GuidToString` (`KismetGuidLibrary.NewGuid`)))))