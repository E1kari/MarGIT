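; BP_Plattform_Standard is a platform that moves along a referenced spline when activated.
; Activate plays MovementTimeline and deactivate reverses it, with the play rate set on BeginPlay before StartOnBegin is called.
; Each timeline update maps the MoveTrack alpha to a distance along the spline and sets the actor's world location there without sweeping.
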(event `self.ReceiveBeginPlay`
  (`self.SetPlayRate` (`self.MovementTimeline`))
  (`self.StartOnBegin`))

(event `/Game/Mechanics/Interfaces/BPI_EnvironmentInterface.EI_OnActivate`
  (bind _spline (`/Game/Mechanics/Environment/SplinePath/BP_SplinePath.Spline` (`self.SplineReference`)))
  (bind (_direction _movetrack) (`Timeline|MovementTimeline` :!label _label)
    (:`Update`
      (`self.K2_SetActorLocation` (`SplineComponent.GetLocationAtDistanceAlongSpline` _spline (`KismetMathLibrary.Lerp` 0.0 (`SplineComponent.GetSplineLength` _spline) _movetrack) "World")))))

(event `/Game/Mechanics/Interfaces/BPI_EnvironmentInterface.EI_OnDeactivate`
  (goto _label :!via `Reverse`))

(fn `UserConstructionScript`
  (`parent.UserConstructionScript`))