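; BP_Plattform_Base is a base Blueprint for environment platforms, providing shared helpers for timing, activation and hitbox debugging.
; SetPlayRate scales a given timeline by the inverse of TimeToComplete, so that value controls its duration.
; StartOnBegin calls EIOnActivate when StartAsActive is set.
; The DGShowHitbox event calls its parent, then shows or hides BoxCollision in game according to ShowHitbox.
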(event `/Game/Mechanics/Interfaces/BPI_DebugGizmos.DG_ShowHitbox`
  (`parent.DG_ShowHitbox`)
  (if (`self.ShowHitbox?`)
    (`SceneComponent.SetHiddenInGame` (`self.BoxCollision`) false false)
    (else
      (`SceneComponent.SetHiddenInGame` (`self.BoxCollision`) true false))))

(fn `SetPlayRate`
  (params (Timeline :type "TimelineComponent Object Reference"))
  (`TimelineComponent.SetPlayRate` Timeline (/ 1.0 (`self.TimeToComplete`))))

(fn `StartOnBegin`
  (if (`self.StartAsActive`)
    (`/Game/Mechanics/Interfaces/BPI_EnvironmentInterface.EI_OnActivate`)))

(fn `UserConstructionScript`)