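; Base Blueprint for an environmental shield that switches on and off through Ion activate and deactivate events.
; Activation shows the static mesh, enables query and physics collision, and plays a sound at the actor's location through the audio manager subsystem.
; Deactivation hides the mesh and disables collision silently, as its sound call is unconnected.
; When flagged Standalone, the shield activates itself from the construction script.
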(event `/Game/Mechanics/Interfaces/BPI_EnvironmentInterface.EI_OnDeactivate`
  (`self.OnDeactivate`))

(event `/Game/Mechanics/Interfaces/BPI_EnvironmentInterface.EI_OnActivate`
  (`self.OnActivate`))

(fn `OnActivate`
  (bind _staticmesh (`self.StaticMesh`))
  (`SceneComponent.SetHiddenInGame` _staticmesh false true)
  (`PrimitiveComponent.SetCollisionEnabled` _staticmesh "QueryAndPhysics")
  (`AudioManagerSubsystem.PlaySFXAtLocation` (subsystem `AudioManagerSubsystem`) (`self.ActivateSFX`) (`self.K2_GetActorLocation`) null false 1.0 true))

(fn `OnDeactivate`
  (bind _staticmesh (`self.StaticMesh`))
  (`SceneComponent.SetHiddenInGame` _staticmesh true true)
  (`PrimitiveComponent.SetCollisionEnabled` _staticmesh "NoCollision"))

(fn `UserConstructionScript`
  (`parent.UserConstructionScript`)
  (if (`self.Standalone?`)
    (`self.OnActivate`)))