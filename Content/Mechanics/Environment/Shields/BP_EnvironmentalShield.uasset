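; BP_EnvironmentalShield is an environmental shield that switches between an active, solid state and an inactive, hidden one.
; Interface-style activate and deactivate events call functions that toggle the static mesh's in-game visibility, including children, and its collision between query-and-physics and none.
; The construction script runs the parent's script, then applies the initial state from StartAsActive.
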(event `/Game/Mechanics/Interfaces/BPI_EnvironmentInterface.EI_OnDeactivate`
  (`self.OnDeactivate`))

(event `/Game/Mechanics/Interfaces/BPI_EnvironmentInterface.EI_OnActivate`
  (`self.OnActivate`))

(fn `OnActivate`
  (bind _staticmesh (`self.StaticMesh`))
  (`SceneComponent.SetHiddenInGame` _staticmesh false true)
  (`PrimitiveComponent.SetCollisionEnabled` _staticmesh "QueryAndPhysics"))

(fn `OnDeactivate`
  (bind _staticmesh (`self.StaticMesh`))
  (`SceneComponent.SetHiddenInGame` _staticmesh true true)
  (`PrimitiveComponent.SetCollisionEnabled` _staticmesh "NoCollision"))

(fn `UserConstructionScript`
  (`parent.UserConstructionScript`)
  (if (`self.StartAsActive`)
    (`self.OnActivate`)
    (else
      (`self.OnDeactivate`))))