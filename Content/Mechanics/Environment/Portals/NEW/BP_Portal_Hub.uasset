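; BP_Portal_Hub is the hub-side portal that links to a start portal inside a streamed sublevel.
; On load, it streams its linked sublevel by soft reference, then finds the BP_Portal_Sublevel_Start whose own level matches that world asset.
; It registers itself with that portal by its index in AllHubPortals, then sets up the linked render target and deactivates the other portal's frame mesh.
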(event `self.OnLoadOtherLevel`
  (`GameplayStatics.LoadStreamLevelBySoftObjectPtr` (`.WorldAsset` (break `SoftWorldReference` (`self.LinkedSubLevel`))) true)
  (`self.OnOtherLevelLoaded`)
  (bind _outactors (`GameplayStatics.GetAllActorsOfClass` "/Game/Mechanics/Environment/Portals/NEW/BP_Portal_Sublevel_Start.BP_Portal_Sublevel_Start_C"))
  (for _array_element _outactors
    (if (== (`.WorldAsset` (break `SoftWorldReference` (`/Game/Mechanics/Environment/Portals/NEW/BP_Portal.OwnLevel` _array_element))) (`.WorldAsset` (break `SoftWorldReference` (`self.LinkedSubLevel`))))
      (set `self.LinkedPortal` _array_element)))
  (bind _linkedportal (`self.LinkedPortal`)
    (:`then`
      (`self.AddLinkedPortal` _linkedportal (`KismetArrayLibrary.Array_Find` (`self.AllHubPortals`) self) self)
      (`self.SetLinkedPortalRenderTarget`)
      (`self.DeactivateOtherPortalFrameMesh`))
    (:`else`)))

(fn `AddLinkedPortal`
  (params (Index :type Integer) (LinkedPortalRef :type "/Game/Mechanics/Environment/Portals/NEW/BP_Portal Object Reference"))
  (set `self.LinkedPortal` LinkedPortalRef))

(fn `UserConstructionScript`
  (`parent.UserConstructionScript`))