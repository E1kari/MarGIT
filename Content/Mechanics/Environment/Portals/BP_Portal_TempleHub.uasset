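; Temple hub portal that streams in its linked level and pairs itself with the matching temple section portal.
; When the third-person character enters the preload volume, it loads the level without blocking and finds the section portal whose OwnLevel matches.
; It registers itself there by its index among all hub portals, sets previews both ways and activates the section portal.
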(event `self.OnPreloadBeginOverlap`
  (params (OtherActor :type "Actor Object Reference"))
  (bind _linkedportal (`self.LinkedPortal`))
  (bind _linkedportal_2 (`self.LinkedPortal`))
  (if (`GameplayStatics.ObjectIsA` OtherActor "/Game/Mechanics/Player/Blueprints/BP_ThirdPersonCharacter.BP_ThirdPersonCharacter_C")
    (`GameplayStatics.LoadStreamLevelBySoftObjectPtr` (`self.LinkedLevel`) true)
    (bind _outactors (`GameplayStatics.GetAllActorsOfClass` "/Game/Mechanics/Environment/Portals/BP_Portal_TempleSections.BP_Portal_TempleSections_C"))
    (for _array_element _outactors
      (if (== (`/Game/Mechanics/Environment/Portals/BP_Portal_Base.OwnLevel` _array_element) (`self.LinkedLevel`))
        (set `self.LinkedPortal` _array_element)))
    (`/Engine/EditorBlueprintResources/StandardMacros.IsValid` _linkedportal_2
      (:`Is Valid`
        (`/Game/Mechanics/Environment/Portals/BP_Portal_TempleSections.AddLinkedPortal` _linkedportal_2 (`KismetArrayLibrary.Array_Find` (`self.AllTempleHubPortals`) self) self)
        (`self.SetPortalPreview` _linkedportal)
        (`self.SetPortalPreview` _linkedportal self)
        (`self.SetPortalActive` _linkedportal true)))))

(fn `AddLinkedPortal`
  (params (Index :type Integer) (LinkedPortal :type "/Game/Mechanics/Environment/Portals/BP_Portal_Base Object Reference"))
  (set `self.LinkedPortal` LinkedPortal))

(fn `UserConstructionScript`
  (`parent.UserConstructionScript`))