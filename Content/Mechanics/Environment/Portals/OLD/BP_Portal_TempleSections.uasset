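; Portal for temple sections that streams in its linked level and pairs itself with a temple hub portal, extending a parent portal Blueprint.
; When the third-person character enters the preload overlap, it loads the level non-blocking and activates the linked portal.
; If no valid link exists, it refreshes the GameInstance portal list, picks the hub portal by index, and cross-links both portals and their previews before activation.
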(event `self.OnPreloadBeginOverlap`
  (params (OtherActor :type "Actor Object Reference"))
  (bind _linkedportal (`self.LinkedPortal`))
  (if (`GameplayStatics.ObjectIsA` OtherActor "/Game/Mechanics/Player/Blueprints/BP_ThirdPersonCharacter.BP_ThirdPersonCharacter_C")
    (`GameplayStatics.LoadStreamLevelBySoftObjectPtr` (`self.LinkedLevel`) true)
    (`/Engine/EditorBlueprintResources/StandardMacros.IsValid` _linkedportal
      (:`Is Valid`
        (`self.SetPortalActive` _linkedportal true))
      (:`Is Not Valid`
        (bind _asgi_game_instance (cast `/Game/Mechanics/GameInstance/GI_GameInstance` (`GameplayStatics.GetGameInstance`)))
        (`/Game/Mechanics/GameInstance/GI_GameInstance.AddAllPortals` _asgi_game_instance)
        (bind _output_get (set `self.LinkedPortal` (`|GetArrayItem` (`/Game/Mechanics/GameInstance/GI_GameInstance.AllTempleHubPortals` _asgi_game_instance) (`self.Linked Portal Index`))))
        (`self.SetPortalPreview` _output_get)
        (`self.SetPortalPreview` _output_get self)
        (`self.AddLinkedPortal` _output_get 0 self)
        (`self.SetPortalActive` _output_get true)))))

(fn `AddLinkedPortal`
  (params (Index :type Integer) (LinkedPortal :type "/Game/Mechanics/Environment/Portals/OLD/BP_Portal_Base Object Reference"))
  (set `self.Linked Portal Index` Index)
  (set `self.LinkedPortal` LinkedPortal))

(fn `UserConstructionScript`
  (`parent.UserConstructionScript`))