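; Base portal actor that shows a render-target preview through a linked portal and teleports the third-person character to it.
; While active, its scene capture mirrors the player camera's offset from the linked portal, feeding a dynamic material for previews.
; Teleporting preserves relative location and control rotation, temporarily disabling the destination to prevent bounce-back.
; Leaving the preload sphere deactivates the linked portal and unloads its level; preload entry is an empty hook.
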(event `/Game/Mechanics/Interfaces/BPI_DebugGizmos.DG_ShowHitbox`
  (`parent.DG_ShowHitbox`)
  (if (`self.ShowHitbox?`)
    (`SceneComponent.SetHiddenInGame` (`self.TeleportVolume`) false false)
    (`SceneComponent.SetHiddenInGame` (`self.PreloadVolume`) false false)
    (else
      (`SceneComponent.SetHiddenInGame` (`self.TeleportVolume`) true false)
      (`SceneComponent.SetHiddenInGame` (`self.PreloadVolume`) true false))))

(event `self.ReceiveBeginPlay`
  (bind (_previewtexturesize_x _previewtexturesize_y) (`KismetMathLibrary.BreakVector2D` (`self.PreviewTextureSize`)))
  (bind _returnvalue (`KismetRenderingLibrary.CreateRenderTarget2D` (`KismetMathLibrary.FTrunc` _previewtexturesize_x) (`KismetMathLibrary.FTrunc` _previewtexturesize_y)))
  (bind _output_get (set `SceneCaptureComponent2D.TextureTarget` _returnvalue (`self.PortalCapture`)))
  (bind _returnvalue_2 (`KismetMaterialLibrary.CreateDynamicMaterialInstance` "/Game/Mechanics/Environment/Portals/OLD/M_PortalPreview.M_PortalPreview"))
  (bind _output_get_2 (set `self.OwnPortalMID` _returnvalue_2))
  (`MaterialInstanceDynamic.SetTextureParameterValue` _output_get_2 "PortalTexture" _output_get)
  (`ActorComponent.Deactivate` (`self.PortalCapture`)))

(event `self.ReceiveTick`
  (params (DeltaSeconds :type "Float (single-precision)"))
  (if (`self.PortalActive`)
    (bind (_relativloc _relativrot) (`self.GetPlayerRelativeLocation` (`self.LinkedPortal`)))
    (`SceneComponent.K2_SetRelativeLocationAndRotation` (`self.PortalCapture`) _relativloc (`KismetMathLibrary.ComposeRotators` (`KismetMathLibrary.MakeRotator` 270.0) _relativrot) false false)))

(event `self.PreloadVolume.OnComponentBeginOverlap`
  (params (OverlappedComponent :type "PrimitiveComponent Object Reference") (OtherActor :type "Actor Object Reference") (OtherComp :type "PrimitiveComponent Object Reference") (OtherBodyIndex :type Integer) (bFromSweep :type Boolean) (SweepResult :type "HitResult Structure (by ref)"))
  (`self.OnPreloadBeginOverlap` OtherActor))

(event `OnPreloadBeginOverlap`
  (params (OtherActor :type "Actor Object Reference")))

(event `self.PreloadVolume.OnComponentEndOverlap`
  (params (OverlappedComponent :type "PrimitiveComponent Object Reference") (OtherActor :type "Actor Object Reference") (OtherComp :type "PrimitiveComponent Object Reference") (OtherBodyIndex :type Integer))
  (`self.OnPreloadVolumeEndOverlap` OtherActor))

(event `OnPreloadVolumeEndOverlap`
  (params (OtherActor :type "Actor Object Reference"))
  (if (and (`GameplayStatics.ObjectIsA` OtherActor "/Game/Mechanics/Player/Blueprints/BP_ThirdPersonCharacter.BP_ThirdPersonCharacter_C") (not (`self.PlayerJustTeleported`)))
    (`self.SetPortalActive` (`self.LinkedPortal`) false)
    (`self.ResetRelativeSphereLocation`)
    (`GameplayStatics.UnloadStreamLevelBySoftObjectPtr` (`self.LinkedLevel`))))

(event `self.TeleportVolume.OnComponentBeginOverlap`
  (params (OverlappedComponent :type "PrimitiveComponent Object Reference") (OtherActor :type "Actor Object Reference") (OtherComp :type "PrimitiveComponent Object Reference") (OtherBodyIndex :type Integer) (bFromSweep :type Boolean) (SweepResult :type "HitResult Structure (by ref)"))
  (`self.OnTeleportBeginOverlap` OtherActor))

(event `OnTeleportBeginOverlap`
  (params (OtherActor :type "Actor Object Reference"))
  (bind _linkedportal (`self.LinkedPortal`))
  (bind _linkedportal_2 (`self.LinkedPortal`))
  (if (and (`GameplayStatics.ObjectIsA` OtherActor "/Game/Mechanics/Player/Blueprints/BP_ThirdPersonCharacter.BP_ThirdPersonCharacter_C") (`self.IsTeleportEnabled`))
    (`/Engine/EditorBlueprintResources/StandardMacros.IsValid` _linkedportal
      (:`Is Valid`
        (`self.DisableTeleport` _linkedportal)
        (`PrimitiveComponent.SetCollisionEnabled` (`/Game/Mechanics/Environment/Portals/OLD/BP_Portal_Base.PortalMesh` _linkedportal) "NoCollision")
        (set `self.PlayerJustTeleported` true)
        (bind _playercontroller (message `/Game/Mechanics/Interfaces/BPI_EffectTargetInterface.ETI_GetPlayerController` OtherActor))
        (bind (_returnvalue_roll _returnvalue_pitch _returnvalue_yaw) (`KismetMathLibrary.BreakRotator` (`KismetMathLibrary.ComposeRotators` (`self.K2_GetActorRotation` _linkedportal_2) (`KismetMathLibrary.NormalizedDeltaRotator` (`Controller.GetControlRotation` _playercontroller) (`self.K2_GetActorRotation`)))))
        (`Controller.SetControlRotation` _playercontroller (`KismetMathLibrary.MakeRotator` 0.0 _returnvalue_pitch _returnvalue_yaw))
        (`self.K2_SetActorLocation` OtherActor (`KismetMathLibrary.TransformLocation` (`self.GetTransform` _linkedportal_2) (`KismetMathLibrary.InverseTransformLocation` (`self.GetTransform`) (`self.K2_GetActorLocation` OtherActor))) false false)
        (if (`self.IsTeleportEnabled`)
          (`self.SetPortalActive` (`self.LinkedPortal`) false))))))

(event `self.TeleportVolume.OnComponentEndOverlap`
  (params (OverlappedComponent :type "PrimitiveComponent Object Reference") (OtherActor :type "Actor Object Reference") (OtherComp :type "PrimitiveComponent Object Reference") (OtherBodyIndex :type Integer))
  (`self.OnTeleportEndOverlap` OtherActor))

(event `DisableTeleport`
  (set `self.IsTeleportEnabled` false))

(event `OnTeleportEndOverlap`
  (params (OtherActor :type "Actor Object Reference"))
  (if (`GameplayStatics.ObjectIsA` OtherActor "/Game/Mechanics/Player/Blueprints/BP_ThirdPersonCharacter.BP_ThirdPersonCharacter_C")
    (`KismetSystemLibrary.Delay` 0.5)
    (set `self.IsTeleportEnabled` true)
    (set `self.PlayerJustTeleported` false)
    (`PrimitiveComponent.SetCollisionEnabled` (`self.PortalMesh`) "QueryAndPhysics")))

(event `AddAllTempleHubPortals`
  (params (Input :type "Array of /Game/Mechanics/Environment/Portals/OLD/BP_Portal_TempleHub Object Reference"))
  (set `self.AllTempleHubPortals` Input))

(fn `ActivateLinkedPortalCapture`
  (params (NewParam :type "/Game/Mechanics/Environment/Portals/OLD/BP_Portal_Base Object Reference"))
  (`ActorComponent.Activate` (`/Game/Mechanics/Environment/Portals/OLD/BP_Portal_Base.PortalCapture` NewParam) false))

(fn `AddLinkedPortal`
  (params (Index :type Integer) (LinkedPortal :type "/Game/Mechanics/Environment/Portals/OLD/BP_Portal_Base Object Reference")))

(fn `GetPlayerRelativeLocation`
  (returns (RelativLoc :type "Vector Structure") (RelativRot :type "Rotator Structure"))
  (bind _returnvalue (`GameplayStatics.GetPlayerCameraManager` 0))
  (bind _relativesphere (`self.RelativeSphere`))
  (`SceneComponent.K2_SetWorldLocationAndRotation` _relativesphere (`PlayerCameraManager.GetCameraLocation` _returnvalue) (`PlayerCameraManager.GetCameraRotation` _returnvalue) false false)
  (return (`SceneComponent.RelativeLocation` _relativesphere) (`SceneComponent.RelativeRotation` _relativesphere)))

(fn `ResetRelativeSphereLocation`
  (`SceneComponent.K2_SetRelativeLocation` (`self.RelativeSphere`) (0.0 0.0 0.0) false false))

(fn `SetPortalActive`
  (params (`Active?` :type Boolean))
  (bind _portalcapture (`self.PortalCapture`))
  (bind _output_get (set `self.PortalActive` `Active?`))
  (`SceneComponent.SetHiddenInGame` (`self.PortalMesh`) _output_get true)
  (`|ExecutionSequence`
    (:`then_0`
      (if (not _output_get)
        (`SceneComponent.K2_SetRelativeLocation` (`self.PortalCapture`) (0.0 0.0 89.0) false false)))
    (:`then_1`
      (if _output_get
        (`ActorComponent.Activate` _portalcapture false)
        (else
          (`ActorComponent.Deactivate` _portalcapture))))))

(fn `SetPortalPreview`
  (params (LinkedPortal :type "/Game/Mechanics/Environment/Portals/OLD/BP_Portal_Base Object Reference"))
  (bind _ownportalmid (`/Game/Mechanics/Environment/Portals/OLD/BP_Portal_Base.OwnPortalMID` LinkedPortal))
  (`/Engine/EditorBlueprintResources/StandardMacros.IsValid` _ownportalmid
    (:`Is Valid`
      (`PrimitiveComponent.SetMaterial` (`self.PortalPreview`) 0 _ownportalmid))
    (:`Is Not Valid`
      (`KismetSystemLibrary.PrintString` "NotValid"))))

(fn `UserConstructionScript`
  (set `self.BaseRotation` (`SceneComponent.RelativeRotation` (`self.PortalCapture`)))
  (`SphereComponent.SetSphereRadius` (`self.PreloadVolume`) (`self.PreloadVolumeRadius`) true))